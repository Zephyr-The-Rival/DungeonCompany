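; BP_RockGenerator is a trigger-driven falling-rock and sand VFX actor with sound, built on the RockMaster Niagara component.
; When a PlayerCharacter enters the sphere, the server rolls TriggerChance and calls the multicast SpawnRocks.
; SetParameters feeds size and rate variables to Niagara, both there and in the construction script, which also sizes the sphere.
; Non-looping rocks and sand stop emitting after their own delays.
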(event `self.ReceiveBeginPlay`)

(event `self.Sphere.OnComponentBeginOverlap`
  (params (OverlappedComponent :type "PrimitiveComponent Object Reference") (OtherActor :type "Actor Object Reference") (OtherComp :type "PrimitiveComponent Object Reference") (OtherBodyIndex :type Integer) (bFromSweep :type Boolean) (SweepResult :type "HitResult Structure (by ref)"))
  (cast `PlayerCharacter` OtherActor)
  (`/Engine/EditorBlueprintResources/ActorMacros.Switch Has Authority`
    (:`Authority`
      (if (< (`KismetMathLibrary.RandomFloatInRange` 0.0 100.0) (`self.TriggerChance`))
        (`self.SpawnRocks`)))))

(event `SpawnRocks`
  (bind _rockmaster (`self.RockMaster`))
  (bind _rockmaster_2 (`self.RockMaster`))
  ;[1 0.2957 0.9346] Mulitcast
  (`ActorComponent.SetActive` _rockmaster_2 true false)
  (`self.SetParameters` _rockmaster_2)
  (`|ExecutionSequence`
    (:`then_0`
      (`GameplayStatics.SpawnSoundAtLocation` "/Game/_DungeonCompanyContent/Audio/Environment/rock/rocks_Cue.rocks_Cue" (`SceneComponent.K2_GetComponentLocation` (`self.DefaultSceneRoot`)) (struct) 1.0 1.0 0.0 null null))
    (:`then_1`
      (if (not (`self.Lopping`))
        (`KismetSystemLibrary.Delay` (`self.Duration`))
        (`NiagaraComponent.SetVariableFloat` _rockmaster "Generating speed" 0.0)))
    (:`then_2`
      (if (not (`self.Lopping_sand`))
        (`KismetSystemLibrary.Delay` (`self.Duration_sand`))
        (`NiagaraComponent.SetVariableFloat` _rockmaster "SpawnRate" 0.0)))
    (:`then_3`
      (`KismetSystemLibrary.Delay` (`self.Duration`))
      (if (and (not (`self.Lopping`)) (not (`self.Lopping_sand`)))
        (`ActorComponent.SetActive` (`self.RockMaster`) false false)))))

(fn `SetParameters`
  (params (Niagara :type "NiagaraComponent Object Reference"))
  (`|ExecutionSequence`
    (:`then_0`
      (if (`self.IsActive`)
        (set `self.Generating|Rocks` 1.0)
        (else
          (set `self.Generating|Rocks` 0.0))))
    (:`then_1`
      (if (`self.IsActive_sand`)
        (set `self.Generating|sand` 1.0)
        (else
          (set `self.Generating|sand` 0.0))))
    (:`then_2`
      (`NiagaraComponent.SetVariableFloat` Niagara "Generating region size" (`self.Generating region size`)))
    (:`then_3`
      (`NiagaraComponent.SetVariableFloat` Niagara "Generating speed" (* (`self.Generating speed`) (`self.Generating|Rocks`))))
    (:`then_4`
      (`NiagaraComponent.SetVariableFloat` Niagara "Rock size" (`self.RockSize`)))
    (:`then_5`
      (`NiagaraComponent.SetVariableFloat` Niagara "SpawnRegionSize" (`self.Generating region size_sand`)))
    (:`then_6`
      (`NiagaraComponent.SetVariableFloat` Niagara "SpawnRate" (* (`self.Generating speed_sand`) (`self.Generating|sand`))))))

(fn `UserConstructionScript`
  (`self.SetParameters` (`self.RockMaster`))
  (`SphereComponent.SetSphereRadius` (`self.Sphere`) (`self.collisionRadius`) true))