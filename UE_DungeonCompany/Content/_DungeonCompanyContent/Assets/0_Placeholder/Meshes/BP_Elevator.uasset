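; Elevator actor that moves its mesh along timelines, with rumble audio during travel and a bell rope button to call it.
; BeginPlay runs an initial move and binds to the rope's BP_BasicButton child actor press event.
; ElavatorCalled animates the rope, rings the bell and moves the elevator, then runs a second move after a delay.
; TeleportIn and TeleportOut are empty stubs, and the ElevatorUp timeline is unconnected.
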(event `self.ReceiveBeginPlay`
  (bind _asbp_basic_button (cast `/Game/_DungeonCompanyContent/Code/WorldActors/BP_BasicButton` (`ChildActorComponent.ChildActor` (`self.BellRope`))))
  (add `BasicButton.OnButtonPressed` _asbp_basic_button (`|CreateDelegate` :!event `ElavatorCalled`))
  (`AudioComponent.Play` (`self.ElevatorRumble`) 5.0)
  (bind (_direction _newtrack_0) (`Timeline|Timeline_2`)
    (:`Update`
      (`SceneComponent.K2_SetRelativeLocation` (`self.SM_Elevator`) _newtrack_0 false false))
    (:`Finished`
      (`AudioComponent.Stop` (`self.ElevatorRumble`)))))

(event `TeleportIn`)

(event `TeleportOut`)

(event `ElavatorCalled`
  (params (InteractingPawn :type "Pawn Object Reference"))
  (bind (_rope_original_pos_x _rope_original_pos_y _rope_original_pos_z) (`KismetMathLibrary.BreakVector` (`self.rope original pos`)))
  (`|ExecutionSequence`
    (:`then_0`
      (set `self.rope original pos` (`SceneComponent.K2_GetComponentLocation` (`self.BellRope`)))
      (bind (_direction _newtrack_0) (`Timeline|Timeline_0` :!via `PlayFromStart`)
        (:`Update`
          (`SceneComponent.K2_SetWorldLocation` (`self.BellRope`) (`KismetMathLibrary.MakeVector` _rope_original_pos_x _rope_original_pos_y (+ (.z _newtrack_0) _rope_original_pos_z)) false false))))
    (:`then_1`
      (`AudioComponent.Play` (`self.BellSound`) 0.0)
      (`AudioComponent.Play` (`self.ElevatorRumble`) 5.0)
      (bind (_direction_2 _newtrack_0_2) (`Timeline|Timeline`)
        (:`Update`
          (`SceneComponent.K2_SetRelativeLocation` (`self.SM_Elevator`) _newtrack_0_2 false false))
        (:`Finished`
          (`AudioComponent.Stop` (`self.ElevatorRumble`))
          (`KismetSystemLibrary.Delay` 10.0)
          (`AudioComponent.Play` (`self.ElevatorRumble`) 5.0)
          (bind (_direction_3 _newtrack_0_3) (`Timeline|Timeline_1`)
            (:`Update`
              (`SceneComponent.K2_SetRelativeLocation` (`self.SM_Elevator`) _newtrack_0_3 false false))
            (:`Finished`
              (`AudioComponent.Stop` (`self.ElevatorRumble`)))))))))

(fn `UserConstructionScript`)