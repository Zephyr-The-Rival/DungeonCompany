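; Test Spurchin enemy that computes procedural foot placement for walking over uneven ground.
; BeginPlay traces under each toe bone to store its offset from the actor.
; Each tick, unplanted legs follow yaw-rotated offsets traced to the ground, lifted by a cubic falloff of distance travelled.
; Beyond MaxStep, all legs retrace and generally toggle Planted, with misses tracing toward the ground point under the body as fallback.
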(event `self.ReceiveBeginPlay`
  ;[1 1 1] Raycast Leg
  (for (_array_element _array_index) (`self.Legs`)
    (bind _returnvalue_location (`KismetMathLibrary.BreakTransform` (`SkinnedMeshComponent.GetBoneTransform` (`self.Mesh`) (`.ToeName_15_E4BF452742788D6B9A82848356C47169` (break `/Game/_DungeonCompanyContent/Assets/Enemies/Spurchin/S_SpurchinLegs` _array_element)) "RTS_World")))
    (bind (_raystart _rayend) (`self.GetVerticalRay` _returnvalue_location 100.0 -100.0))
    (bind _location (`self.CastRay` _raystart _rayend 30.0)
      (:`Hit`
        (setmembers `/Game/_DungeonCompanyContent/Assets/Enemies/Spurchin/S_SpurchinLegs` :`StructRef` (`|GetArrayItem` (`self.Legs`) _array_index) :`Location` _location :`InitialOffSet` (- _location (`self.K2_GetActorLocation`))))))
  (set `self.PrevLocation` (`self.K2_GetActorLocation`))
  (set `self.Ready` true))

(event `self.ReceiveTick`
  (params (DeltaSeconds :type "Float (single-precision)"))
  (bind (_returnvalue_roll _returnvalue_pitch _returnvalue_yaw) (`KismetMathLibrary.BreakRotator` (`self.K2_GetActorRotation`)))
  (bind (_returnvalue_roll_2 _returnvalue_pitch_2 _returnvalue_yaw_2) (`KismetMathLibrary.BreakRotator` (`self.K2_GetActorRotation`)))
  (bind (_returnvalue_x _returnvalue_y _returnvalue_z) (`KismetMathLibrary.BreakVector` (`self.K2_GetActorLocation`)))
  (bind _returnvalue (`KismetMathLibrary.Vector_Distance2D` (`self.K2_GetActorLocation`) (`self.PrevLocation`)))
  (bind (_raystart _rayend) (`self.GetVerticalRay` (`self.K2_GetActorLocation`) 150.0 -150.0))
  (bind (_relativelocation_x _relativelocation_y _relativelocation_z) (`KismetMathLibrary.BreakVector` (`SceneComponent.RelativeLocation` (`self.Mesh`))))
  (`|ExecutionSequence`
    (:`then_0`
      ;[1 1 1] Racast root
      (bind _location (`self.CastRay` _raystart _rayend)
        (:`Hit`
          (set `self.Center` _location))
        (:`NoHit`
          (set `self.Center` (`KismetMathLibrary.MakeVector` _returnvalue_x _returnvalue_y (+ _returnvalue_z _relativelocation_z))))))
    (:`then_1`
      (for (_array_element _array_index) (`self.Legs`)
        (if (not (`.Planted_12_EA2BC3C24193A96196CDD7A8254D9689` (break `/Game/_DungeonCompanyContent/Assets/Enemies/Spurchin/S_SpurchinLegs` _array_element)))
          (bind (_raystart_2 _rayend_2) (`self.GetVerticalRay` (+ (`KismetMathLibrary.GreaterGreater_VectorRotator` (`.InitialOffSet_11_654236D84EDFF13C739DD4A6850575C7` (break `/Game/_DungeonCompanyContent/Assets/Enemies/Spurchin/S_SpurchinLegs` _array_element)) (`KismetMathLibrary.MakeRotator` 0.0 0.0 _returnvalue_yaw_2)) (`self.K2_GetActorLocation`)) 100.0 -100.0))
          (bind _location_2 (`self.CastRay` _raystart_2 _rayend_2 30.0)
            (:`Hit`
              (setmembers `/Game/_DungeonCompanyContent/Assets/Enemies/Spurchin/S_SpurchinLegs` :`StructRef` (`|GetArrayItem` (`self.Legs`) _array_index) :`Location` (`KismetMathLibrary.MakeVector` (.x _location_2) (.y _location_2) (+ (.z _location_2) (`self.GetLegHeight` _returnvalue))))))))
      (if (> _returnvalue (`self.MaxStep`))
        (for (_array_element_2 _array_index_2) (`self.Legs`)
          (bind (_raystart_3 _rayend_3) (`self.GetVerticalRay` (+ (`KismetMathLibrary.GreaterGreater_VectorRotator` (`.InitialOffSet_11_654236D84EDFF13C739DD4A6850575C7` (break `/Game/_DungeonCompanyContent/Assets/Enemies/Spurchin/S_SpurchinLegs` _array_element_2)) (`KismetMathLibrary.MakeRotator` 0.0 0.0 _returnvalue_yaw)) (`self.K2_GetActorLocation`)) 100.0 -100.0))
          (bind (_location_3 _out_hit_trace_end) (`self.CastRay` _raystart_3 _rayend_3 30.0)
            (:`Hit`
              (bind _output (`|GetArrayItem` (`self.Legs`) _array_index_2))
              (bind _returnvalue_2 (not (`.Planted_12_EA2BC3C24193A96196CDD7A8254D9689` (break `/Game/_DungeonCompanyContent/Assets/Enemies/Spurchin/S_SpurchinLegs` _array_element_2))))
              (setmembers `/Game/_DungeonCompanyContent/Assets/Enemies/Spurchin/S_SpurchinLegs` :`StructRef` _output :`Location` (`KismetMathLibrary.MakeVector` (.x _location_3) (.y _location_3) (+ (.z _location_3) (`self.GetLegHeight` (`KismetMathLibrary.Vector_Distance2D` (`self.K2_GetActorLocation`) (`self.PrevLocation`))))) :`Planted` _returnvalue_2))
            (:`NoHit`
              (bind _location_4 (`self.CastRay` _out_hit_trace_end (`self.Center`) 30.0)
                (:`Hit`
                  (setmembers `/Game/_DungeonCompanyContent/Assets/Enemies/Spurchin/S_SpurchinLegs` :`StructRef` _output :`Location` _location_4))
                (:`NoHit`
                  (setmembers `/Game/_DungeonCompanyContent/Assets/Enemies/Spurchin/S_SpurchinLegs` :`StructRef` _output :`Planted` _returnvalue_2))))))
        (set `self.PrevLocation` (`self.K2_GetActorLocation`))))))

(fn `GetLegHeight`
  (params (Distance :type "Float (double-precision)"))
  (returns (Z :type "Float (double-precision)"))
  (return (* (- 1.0 (`KismetMathLibrary.MultiplyMultiply_FloatFloat` (`KismetMathLibrary.FClamp` (/ Distance (`self.MaxStep`))) 3.0)) (`self.StepHeight`))))

(fn `GetVerticalRay`
  (params (Location :type "Vector Structure") (Upper :type "Float (double-precision)") (Lower :type "Float (double-precision)"))
  (returns (RayStart :type "Vector Structure") (RayEnd :type "Vector Structure"))
  (return (`KismetMathLibrary.MakeVector` Location_X Location_Y (+ Location_Z Upper)) (`KismetMathLibrary.MakeVector` Location_X Location_Y (+ Location_Z Lower))))

(fn `UserConstructionScript`)