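; Impaired-vision debuff that gradually blurs the view of a given camera through post-processing.
; SmoothApply finds M_Blur among the camera's post-process materials, replaces it with a dynamic material instance at full weight, and turns on a tick-driven ramp.
; Tick raises the instance's "Strenght" parameter at the Speed rate until it reaches its cap, then stops ramping.
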(event `self.SmoothApply`
  (params (Camera :type "CameraComponent Object Reference"))
  (bind _array (break `WeightedBlendables` (`.WeightedBlendables` (break `PostProcessSettings` (`CameraComponent.PostProcessSettings` Camera)))))
  (for (_array_element _array_index) _array
    (bind _asmaterial (cast `Material` (`.Object` (break `WeightedBlendable` _array_element))))
    (if (== _asmaterial "/Game/_DungeonCompanyContent/Assets/PostProcess/M_Blur.M_Blur")
      (bind _returnvalue (`KismetMaterialLibrary.CreateDynamicMaterialInstance` _asmaterial))
      (bind _output_get (set `self.DynamicMaterial` _returnvalue))
      (`KismetArrayLibrary.Array_Set` _array _array_index (make `WeightedBlendable` 1.0 _output_get))))
  (set `self.ApplyOverTick` true))

(event `self.ReceiveTick`
  (params (DeltaSeconds :type "Float (single-precision)"))
  (if (`self.ApplyOverTick`)
    (if (< (`self.StrenghtValue`) 5.0)
      (set `self.StrenghtValue` (+ (`self.StrenghtValue`) (* DeltaSeconds (`self.Speed`))))
      (`MaterialInstanceDynamic.SetScalarParameterValue` (`self.DynamicMaterial`) "Strenght" (`self.StrenghtValue`))
      (else
        (`MaterialInstanceDynamic.SetScalarParameterValue` (`self.DynamicMaterial`) "Strenght" 5.0)
        (set `self.ApplyOverTick` false)))))