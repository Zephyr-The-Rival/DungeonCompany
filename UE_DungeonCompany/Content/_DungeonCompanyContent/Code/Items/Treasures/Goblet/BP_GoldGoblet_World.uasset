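; BP_GoldGoblet_World is the world actor for a gold goblet treasure item that players can hold in hand.
; When held, it turns off gravity, physics simulation and collision on its mesh and box.
; For the locally controlled holder, it also activates an on-top material on the mesh and disables shadow casting.
; Begin play and the primary action only forward to the parent class.
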(event `self.ReceiveBeginPlay`
  (`parent.ReceiveBeginPlay`))

(event `self.OnHoldingInHand`
  (params (LocallyControlled :type Boolean))
  (bind _mesh (`self.Mesh`))
  (bind _mesh_2 (`self.Mesh`))
  ;[1 1 1] On holding in hand
  (`|ExecutionSequence`
    (:`then_0`
      (`PrimitiveComponent.SetEnableGravity` _mesh false)
      (`PrimitiveComponent.SetSimulatePhysics` _mesh false)
      (`PrimitiveComponent.SetCollisionEnabled` (`self.Mesh`) "NoCollision")
      (`PrimitiveComponent.SetCollisionEnabled` _mesh "NoCollision")
      (`PrimitiveComponent.SetCollisionEnabled` (`self.Box`) "NoCollision"))
    (:`then_1`
      (if LocallyControlled
        (`self.ActivateMaterialOnTop` _mesh_2)
        (`PrimitiveComponent.SetCastShadow` _mesh_2 false)))))

(event `self.TriggerPrimaryAction`
  (params (User :type "PlayerCharacter Object Reference"))
  ;[1 1 1] PrimaryAction
  (`parent.TriggerPrimaryAction` User))

(fn `UserConstructionScript`)