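; BP_Nugget_World is the world actor for a gold nugget treasure item that can be held in hand.
; On BeginPlay the authority picks one of three nugget meshes at random, relying on mesh replication to share it with clients.
; When held, it disables physics, gravity and collision on the mesh and EasyInteract.
; For the local holder it also applies an on-top material and turns off shadow casting.
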(event `self.ReceiveBeginPlay`
  (bind _mesh (`self.Mesh`))
  (`parent.ReceiveBeginPlay`)
  (`/Engine/EditorBlueprintResources/ActorMacros.Switch Has Authority`
    (:`Authority`
      (switch `int` (`KismetMathLibrary.RandomIntegerInRange` 0 2) ; mesh is replicated and therefore the static mesh field as well
        (:`0`
          (`StaticMeshComponent.SetStaticMesh` _mesh "/Game/_DungeonCompanyContent/Assets/Meshes/Items/GoldenNugget1.GoldenNugget1"))
        (:`1`
          (`StaticMeshComponent.SetStaticMesh` _mesh "/Game/_DungeonCompanyContent/Assets/Meshes/Items/GoldenNugget2.GoldenNugget2"))
        (:`2`
          (`StaticMeshComponent.SetStaticMesh` _mesh "/Game/_DungeonCompanyContent/Assets/Meshes/Items/GoldenNugget3.GoldenNugget3"))))))

(event `self.OnHoldingInHand`
  (params (locallyControlled :type Boolean))
  (bind _mesh (`self.Mesh`))
  (bind _mesh_2 (`self.Mesh`))
  ;[1 1 1] On holding in hand
  (`|ExecutionSequence`
    (:`then_0`
      (`PrimitiveComponent.SetEnableGravity` _mesh false)
      (`PrimitiveComponent.SetSimulatePhysics` _mesh false)
      (`PrimitiveComponent.SetCollisionEnabled` (`self.Mesh`) "NoCollision")
      (`PrimitiveComponent.SetCollisionEnabled` _mesh "NoCollision")
      (`PrimitiveComponent.SetCollisionEnabled` (`self.EasyInteract`) "NoCollision"))
    (:`then_1`
      (if locallyControlled
        (`self.ActivateMaterialOnTop` _mesh_2)
        (`PrimitiveComponent.SetCastShadow` _mesh_2 false)))))

(event `self.TriggerPrimaryAction`
  (params (User :type "PlayerCharacter Object Reference"))
  ;[1 1 1] PrimaryAction
  (`parent.TriggerPrimaryAction` User))

(fn `UserConstructionScript`)