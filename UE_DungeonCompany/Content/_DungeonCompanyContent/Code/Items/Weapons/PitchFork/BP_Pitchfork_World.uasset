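; BP_Pitchfork_World is the in-world pitchfork weapon item, overriding behavior for being held in hand and for dealing hits.
; When held, it turns off gravity, physics and collision on the mesh and pickup collision, then activates an on-top material on the mesh.
; DealHits passes the weapon collision and two mesh socket locations, marking a weakspot trace start and end, to the parent's hit logic.
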(event `self.ReceiveBeginPlay`)

(event `self.OnHoldingInHand`
  (bind _mesh (`self.Mesh`))
  (`PrimitiveComponent.SetEnableGravity` _mesh false)
  (`PrimitiveComponent.SetSimulatePhysics` _mesh false)
  (`PrimitiveComponent.SetCollisionEnabled` (`self.EasyPickupCollision`) "NoCollision")
  (`PrimitiveComponent.SetCollisionEnabled` _mesh "NoCollision")
  (`self.ActivateMaterialOnTop` (`self.Mesh`)))

(event `self.DealHits`
  (params (WeaponCollision :type "PrimitiveComponent Object Reference") (traceStart :type "Vector Structure") (TraceEnd :type "Vector Structure"))
  (bind _mesh (`self.Mesh`))
  (`parent.DealHits` (`self.WeaponCollision`) (`SceneComponent.GetSocketLocation` _mesh "WeakspotTraceStart") (`SceneComponent.GetSocketLocation` _mesh "WeakspotTraceEnd")))

(fn `UserConstructionScript`)