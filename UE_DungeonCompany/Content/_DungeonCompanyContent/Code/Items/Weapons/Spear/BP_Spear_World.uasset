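; BP_Spear_World is the world actor for the spear weapon item, covering its in-hand setup and trace data.
; When held in hand, it turns off gravity and physics on the mesh, and collision on both the mesh and the easy-pickup volume.
; For the locally controlled holder, it also activates an on-top material and disables shadow casting.
; GetWeaponInfo supplies weapon trace start and end points from two mesh sockets.
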(event `self.ReceiveBeginPlay`
  (`parent.ReceiveBeginPlay`))

(event `self.OnHoldingInHand`
  (params (LocallyControlled :type Boolean))
  (bind _mesh (`self.Mesh`))
  (bind _mesh_2 (`self.Mesh`))
  (`|ExecutionSequence`
    (:`then_0`
      (`PrimitiveComponent.SetEnableGravity` _mesh_2 false)
      (`PrimitiveComponent.SetSimulatePhysics` _mesh_2 false)
      (`PrimitiveComponent.SetCollisionEnabled` (`self.EasyPickupCollision`) "NoCollision")
      (`PrimitiveComponent.SetCollisionEnabled` _mesh_2 "NoCollision"))
    (:`then_1`
      (if LocallyControlled
        (`self.ActivateMaterialOnTop` _mesh)
        (`PrimitiveComponent.SetCastShadow` _mesh false)))))

(fn `GetWeaponInfo`
  (returns (ReturnValue :type "WeaponInfo Structure"))
  (bind _mesh (`self.Mesh`))
  (return (make `WeaponInfo` (`|MakeArray` (`SceneComponent.GetSocketLocation` _mesh "TraceStart")) (`|MakeArray` (`SceneComponent.GetSocketLocation` _mesh "TraceEnd_0")))))

(fn `UserConstructionScript`)