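; BP_Sword_World is the world actor for the sword weapon item, including its behavior while held in hand.
; When held, it turns off gravity, physics and collision on the mesh and pickup collider.
; For the locally controlled holder it also applies an on-top material to the mesh and disables its shadow.
; GetWeaponInfo supplies weapon trace lines from mesh sockets, fanning from one shared start to three end points.
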(event `self.ReceiveBeginPlay`
  (`parent.ReceiveBeginPlay`))

(event `self.OnHoldingInHand`
  (params (LocallyControlled :type Boolean))
  (bind _mesh (`self.Mesh`))
  (bind _mesh_2 (`self.Mesh`))
  (`|ExecutionSequence`
    (:`then_0`
      (`PrimitiveComponent.SetEnableGravity` _mesh_2 false)
      (`PrimitiveComponent.SetSimulatePhysics` _mesh_2 false)
      (`PrimitiveComponent.SetCollisionEnabled` (`self.EasyPickupCollision`) "NoCollision")
      (`PrimitiveComponent.SetCollisionEnabled` _mesh_2 "NoCollision"))
    (:`then_1`
      (if LocallyControlled
        (`self.ActivateMaterialOnTop` _mesh)
        (`PrimitiveComponent.SetCastShadow` _mesh false)))))

(fn `GetWeaponInfo`
  (returns (ReturnValue :type "WeaponInfo Structure"))
  (bind _mesh (`self.Mesh`))
  (bind _returnvalue (`SceneComponent.GetSocketLocation` _mesh "TraceStart"))
  (return (make `WeaponInfo` (`|MakeArray` _returnvalue _returnvalue _returnvalue) (`|MakeArray` (`SceneComponent.GetSocketLocation` _mesh "TraceEnd_0") (`SceneComponent.GetSocketLocation` _mesh "TraceEnd_1") (`SceneComponent.GetSocketLocation` _mesh "TraceEnd_2")))))

(fn `UserConstructionScript`)