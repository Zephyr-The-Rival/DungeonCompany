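; World actor for the Sending Stone item, which relays a directional signal to every Sending Stone in the world by lighting crystals.
; The server-side ServerSendSignal calls the multicast LightUp on all instances, which lights the child crystal actor matching Up, Down, Left or Right.
; Construction gives each crystal mesh slot its own dynamic material and hands it to that child actor.
; When held, physics and collision turn off, and the local holder gets an on-top, shadowless mesh.
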(event `self.ReceiveBeginPlay`
  (`parent.ReceiveBeginPlay`))

(event `self.OnHoldingInHand`
  (params (LocallyControlled :type Boolean))
  (bind _mesh (`self.Mesh`))
  (bind _mesh_2 (`self.Mesh`))
  (`|ExecutionSequence`
    (:`then_0`
      (`PrimitiveComponent.SetEnableGravity` _mesh_2 false)
      (`PrimitiveComponent.SetSimulatePhysics` _mesh_2 false)
      (`PrimitiveComponent.SetCollisionEnabled` (`self.EasyPickupCollision`) "NoCollision")
      (`PrimitiveComponent.SetCollisionEnabled` _mesh_2 "NoCollision"))
    (:`then_1`
      (if LocallyControlled
        (`self.ActivateMaterialOnTop` _mesh)
        (`PrimitiveComponent.SetCastShadow` _mesh false)))))

(event `self.Server_SendSignal`
  (params (Signal :type "ESendingStoneAnimatoinState Enum" :default "Neutral"))
  ;[1 0.8378 0] On Server
  (bind _outactors (`GameplayStatics.GetAllActorsOfClass` "BP_SendingStone_World_C"))
  (for _array_element _outactors
    (`self.LightUp` _array_element Signal)))

(event `LightUp`
  (params (Signal :type "ESendingStoneAnimatoinState Enum" :default "Neutral"))
  ;[1 0.02628 0.9263] Multicast
  (switch `ESendingStoneAnimatoinState` Signal
    (:`Up`
      (bind _asbp_sending_stone_crystal_light_up_actor (cast `/Game/_DungeonCompanyContent/Code/Items/SendingStone/BP_SendingStoneCrystalLightUpActor` (`ChildActorComponent.ChildActor` (`self.CrystalUp`))))
      (`/Game/_DungeonCompanyContent/Code/Items/SendingStone/BP_SendingStoneCrystalLightUpActor.LightUp` _asbp_sending_stone_crystal_light_up_actor))
    (:`Down`
      (bind _asbp_sending_stone_crystal_light_up_actor_2 (cast `/Game/_DungeonCompanyContent/Code/Items/SendingStone/BP_SendingStoneCrystalLightUpActor` (`ChildActorComponent.ChildActor` (`self.CrystalDown`))))
      (`/Game/_DungeonCompanyContent/Code/Items/SendingStone/BP_SendingStoneCrystalLightUpActor.LightUp` _asbp_sending_stone_crystal_light_up_actor_2))
    (:`Left`
      (bind _asbp_sending_stone_crystal_light_up_actor_3 (cast `/Game/_DungeonCompanyContent/Code/Items/SendingStone/BP_SendingStoneCrystalLightUpActor` (`ChildActorComponent.ChildActor` (`self.CrystalLeft`))))
      (`/Game/_DungeonCompanyContent/Code/Items/SendingStone/BP_SendingStoneCrystalLightUpActor.LightUp` _asbp_sending_stone_crystal_light_up_actor_3))
    (:`Right`
      (bind _asbp_sending_stone_crystal_light_up_actor_4 (cast `/Game/_DungeonCompanyContent/Code/Items/SendingStone/BP_SendingStoneCrystalLightUpActor` (`ChildActorComponent.ChildActor` (`self.CrystalRight`))))
      (`/Game/_DungeonCompanyContent/Code/Items/SendingStone/BP_SendingStoneCrystalLightUpActor.LightUp` _asbp_sending_stone_crystal_light_up_actor_4))))

(fn `UserConstructionScript`
  (`parent.UserConstructionScript`)
  (`|ExecutionSequence`
    (:`then_0`
      (bind _returnvalue (`KismetMaterialLibrary.CreateDynamicMaterialInstance` "/Game/_DungeonCompanyContent/Assets/Items/SendingStone/M_SendingStoneCrystal.M_SendingStoneCrystal"))
      (`PrimitiveComponent.SetMaterial` (`self.Mesh`) 2 _returnvalue)
      (bind _asbp_sending_stone_crystal_light_up_actor (cast `/Game/_DungeonCompanyContent/Code/Items/SendingStone/BP_SendingStoneCrystalLightUpActor` (`ChildActorComponent.ChildActor` (`self.CrystalUp`))))
      (set `/Game/_DungeonCompanyContent/Code/Items/SendingStone/BP_SendingStoneCrystalLightUpActor.MyMaterial` _returnvalue _asbp_sending_stone_crystal_light_up_actor))
    (:`then_1`
      (bind _returnvalue_2 (`KismetMaterialLibrary.CreateDynamicMaterialInstance` "/Game/_DungeonCompanyContent/Assets/Items/SendingStone/M_SendingStoneCrystal.M_SendingStoneCrystal"))
      (`PrimitiveComponent.SetMaterial` (`self.Mesh`) 3 _returnvalue_2)
      (bind _asbp_sending_stone_crystal_light_up_actor_2 (cast `/Game/_DungeonCompanyContent/Code/Items/SendingStone/BP_SendingStoneCrystalLightUpActor` (`ChildActorComponent.ChildActor` (`self.CrystalRight`))))
      (set `/Game/_DungeonCompanyContent/Code/Items/SendingStone/BP_SendingStoneCrystalLightUpActor.MyMaterial` _returnvalue_2 _asbp_sending_stone_crystal_light_up_actor_2))
    (:`then_2`
      (bind _returnvalue_3 (`KismetMaterialLibrary.CreateDynamicMaterialInstance` "/Game/_DungeonCompanyContent/Assets/Items/SendingStone/M_SendingStoneCrystal.M_SendingStoneCrystal"))
      (`PrimitiveComponent.SetMaterial` (`self.Mesh`) 4 _returnvalue_3)
      (bind _asbp_sending_stone_crystal_light_up_actor_3 (cast `/Game/_DungeonCompanyContent/Code/Items/SendingStone/BP_SendingStoneCrystalLightUpActor` (`ChildActorComponent.ChildActor` (`self.CrystalDown`))))
      (set `/Game/_DungeonCompanyContent/Code/Items/SendingStone/BP_SendingStoneCrystalLightUpActor.MyMaterial` _returnvalue_3 _asbp_sending_stone_crystal_light_up_actor_3))
    (:`then_3`
      (bind _returnvalue_4 (`KismetMaterialLibrary.CreateDynamicMaterialInstance` "/Game/_DungeonCompanyContent/Assets/Items/SendingStone/M_SendingStoneCrystal.M_SendingStoneCrystal"))
      (`PrimitiveComponent.SetMaterial` (`self.Mesh`) 0 _returnvalue_4)
      (bind _asbp_sending_stone_crystal_light_up_actor_4 (cast `/Game/_DungeonCompanyContent/Code/Items/SendingStone/BP_SendingStoneCrystalLightUpActor` (`ChildActorComponent.ChildActor` (`self.CrystalLeft`))))
      (set `/Game/_DungeonCompanyContent/Code/Items/SendingStone/BP_SendingStoneCrystalLightUpActor.MyMaterial` _returnvalue_4 _asbp_sending_stone_crystal_light_up_actor_4))))