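; Actor for a Sending Stone crystal that briefly drives its glow and plays a sound when lit up.
; LightUp restarts a timeline, unless it is already playing, that scales the material's Brightness parameter, then plays the light-up sound at the actor's location.
; MyMaterial is not created or assigned in these graphs.
; The pressed sound and short delay nodes are disconnected and never run.
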(event `LightUp`
  (if (not (`TimelineComponent.IsPlaying` (`self.CrystalLightUp`)))
    (`|ExecutionSequence`
      (:`then_0`
        (bind (_direction _0_1_0) (`Timeline|CrystalLightUp` :!via `PlayFromStart`)
          (:`Update`
            (`MaterialInstanceDynamic.SetScalarParameterValue` (`self.MyMaterial`) "Brightness" (* _0_1_0 30.0)))))
      (:`then_1`
        (`GameplayStatics.PlaySoundAtLocation` "/Game/_DungeonCompanyContent/Audio/SendingStoneSounds/CrystalLightUpSound.CrystalLightUpSound" (`self.K2_GetActorLocation`) (struct) 1.0 1.0 0.0 null null null null)))))

(fn `UserConstructionScript`)