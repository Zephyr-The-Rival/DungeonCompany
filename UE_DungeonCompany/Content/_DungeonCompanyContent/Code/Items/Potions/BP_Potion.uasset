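; BP_Potion is a potion item Blueprint with a mesh, a collision box and a cork.
; When held in hand, it turns off gravity, physics and collision on the mesh and box.
; For the locally controlled holder, it also applies an on-top material to the mesh and any valid cork and stops the mesh casting shadows.
; A separate event hides the cork.
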(event `self.OnHoldingInHand`
  (params (LocallyControlled :type Boolean))
  (bind _mesh (`self.Mesh`))
  (bind _mesh_2 (`self.Mesh`))
  (bind _potion_cork (`self.Potion_cork`))
  ;[1 1 1] On holding in hand
  (`|ExecutionSequence`
    (:`then_0`
      (`PrimitiveComponent.SetEnableGravity` _mesh false)
      (`PrimitiveComponent.SetSimulatePhysics` _mesh false)
      (`PrimitiveComponent.SetCollisionEnabled` (`self.Mesh`) "NoCollision")
      (`PrimitiveComponent.SetCollisionEnabled` _mesh "NoCollision")
      (`PrimitiveComponent.SetCollisionEnabled` (`self.Box`) "NoCollision"))
    (:`then_1`
      (if LocallyControlled
        (`self.ActivateMaterialOnTop` _mesh_2)
        (`PrimitiveComponent.SetCastShadow` _mesh_2 false)
        (`/Engine/EditorBlueprintResources/StandardMacros.IsValid` _potion_cork
          (:`Is Valid`
            (`self.ActivateMaterialOnTop` _potion_cork)))))))

(event `HIdeCork`
  (`SceneComponent.SetVisibility` (`self.Potion_cork`) false false))

(fn `UserConstructionScript`)