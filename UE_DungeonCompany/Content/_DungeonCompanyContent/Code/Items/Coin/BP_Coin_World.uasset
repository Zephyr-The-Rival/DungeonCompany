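; BP_Coin_World is the world coin item, adding a lens-flare glint that shows when a lit torch is nearby.
; Each tick it orients the flare plane by the player camera's up vector and nudges it from the mesh toward the camera.
; Within torch range, camera distance is fed as time into a Timeline, used as a curve for the dynamic material's Alpha.
; Out of range, a DoOnce zeroes Alpha.
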(event `self.ReceiveBeginPlay`
  (`parent.ReceiveBeginPlay`)
  (bind _returnvalue (`KismetMaterialLibrary.CreateDynamicMaterialInstance` (`PrimitiveComponent.GetMaterial` (`self.Plane`) 0)))
  (set `self.LensFlareMaterial` _returnvalue)
  (`PrimitiveComponent.SetMaterial` (`self.Plane`) 0 _returnvalue))

(event `self.ReceiveTick`
  (params (DeltaSeconds :type "Float (single-precision)"))
  (bind _returnvalue (`SceneComponent.K2_GetComponentLocation` (`self.StaticMesh`)))
  (`|ExecutionSequence`
    (:`then_0`
      (`SceneComponent.K2_SetWorldRotation` (`self.Plane`) (`KismetMathLibrary.Conv_VectorToRotator` (`SceneComponent.GetUpVector` (`PlayerCharacter.FirstPersonCamera` (cast `/Game/_DungeonCompanyContent/Code/PlayerCharacter/BP_PlayerCharacter` (`Controller.K2_GetPawn` (`GameplayStatics.GetPlayerController` 0)) :!pure true)))) false false))
    (:`then_1`
      (`SceneComponent.K2_SetWorldLocation` (`self.Plane`) (+ _returnvalue (* (`KismetMathLibrary.Normal` (- (`SceneComponent.K2_GetComponentLocation` (`PlayerCharacter.FirstPersonCamera` (cast `/Game/_DungeonCompanyContent/Code/PlayerCharacter/BP_PlayerCharacter` (`Controller.K2_GetPawn` (`GameplayStatics.GetPlayerController` 0)) :!pure true))) _returnvalue)) (10.0 10.0 10.0)) (0.0 0.0 2.0)) false false))
    (:`then_3`
      (if (< (`self.ClosestActiveTorch`) 2000.0)
        (`|ExecutionSequence`
          (:`then_0`
            (bind (_direction _visibility) (`Timeline|Timeline` :`NewTime` (`KismetMathLibrary.VSize` (- (`SceneComponent.K2_GetComponentLocation` (`PlayerCharacter.FirstPersonCamera` (cast `/Game/_DungeonCompanyContent/Code/PlayerCharacter/BP_PlayerCharacter` (`Controller.K2_GetPawn` (`GameplayStatics.GetPlayerController` 0)) :!pure true))) (`SceneComponent.K2_GetComponentLocation` (`self.StaticMesh`)))) :!via `SetNewTime`)
              (:`Update`
                (`MaterialInstanceDynamic.SetScalarParameterValue` (`self.LensFlareMaterial`) "Alpha" _visibility))))
          (:`then_1`
            (goto _label :!via `Reset`)))
        (else
          (`/Engine/EditorBlueprintResources/StandardMacros.DoOnce` false :!label _label
            (:`Completed`
              (`MaterialInstanceDynamic.SetScalarParameterValue` (`self.LensFlareMaterial`) "Alpha" 0.0))))))))

(fn `ClosestActiveTorch`
  (returns (SmallestDistance :type "Float (double-precision)"))
  (locals (Tmp :type "Float (double-precision)" :default 0.0) (Min :type "Float (double-precision)" :default 100000.0))
  (bind _outactors (`GameplayStatics.GetAllActorsOfClass` "/Game/_DungeonCompanyContent/Code/Items/Torch/BP_Torch_World.BP_Torch_World_C"))
  (for _array_element _outactors
    (set `local.Tmp` (`KismetMathLibrary.Vector_Distance` (`SceneComponent.K2_GetComponentLocation` (`self.StaticMesh`)) (`SceneComponent.K2_GetComponentLocation` (`/Game/_DungeonCompanyContent/Code/Items/Torch/BP_Torch_World.Mesh` _array_element))))
    (if (and (`/Game/_DungeonCompanyContent/Code/Items/Torch/BP_Torch_Data.On` (cast `/Game/_DungeonCompanyContent/Code/Items/Torch/BP_Torch_Data` (`WorldItem.MyData` _array_element) :!pure true)) (< (`local.Tmp`) (`local.Min`)))
      (set `local.Min` (`local.Tmp`))))
  (return (`local.Min`)))

(fn `UserConstructionScript`)