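; World actor for the torch item, which the primary action lights or puts out while fuel remains.
; RepOn's OnRep syncs state to BP_Torch_Data and drives fire, sounds and a timeline light fade; Tick adds random flicker.
; Fuel drains while light intensity is nonzero, closing a fade-out spam exploit, and the authority extinguishes it when empty.
; When held, physics and collision turn off, and the local player sees it rendered on top.
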(event `self.ReceiveBeginPlay`
  (bind _pointlight (`self.PointLight`))
  (bind _on (`/Game/_DungeonCompanyContent/Code/Items/Torch/BP_Torch_Data.On` (cast `/Game/_DungeonCompanyContent/Code/Items/Torch/BP_Torch_Data` (`self.MyData`) :!pure true)))
  (`parent.ReceiveBeginPlay`)
  (`|ExecutionSequence`
    (:`then_0`
      (set `self.OriginalLightLocation` (`SceneComponent.RelativeLocation` _pointlight))
      (set `self.OriginalLightIntensity` (`LightComponentBase.Intensity` _pointlight)))
    (:`then_1`
      (set `self.RepOn` _on)
      (`ActorComponent.SetActive` (`self.Fire`) _on false)
      (if _on
        (`LightComponent.SetIntensity` (`self.PointLight`) (`self.OriginalLightIntensity`))
        (set `self.Flicker` true)
        (bind _returnvalue (`GameplayStatics.SpawnSoundAttached` "/Game/_DungeonCompanyContent/Assets/Sound/SFX/Torch_Crackling_SeamlessLoop.Torch_Crackling_SeamlessLoop" (`self.Fire`) "None" (0.0 0.0 0.0) (struct) "KeepRelativeOffset" false 0.5 1.0 0.0 "/Game/_DungeonCompanyContent/Audio/Player/Steps/StepsSA.StepsSA" null))
        (set `self.FireLoopSound` _returnvalue)
        (else
          (`LightComponent.SetIntensity` (`self.PointLight`) 0.0)
          (set `self.Flicker` false))))))

(event `self.OnHoldingInHand`
  (params (locallyControlled :type Boolean))
  (bind _mesh (`self.Mesh`))
  (bind _mesh_2 (`self.Mesh`))
  ;[1 1 1] On holding in hand
  (`|ExecutionSequence`
    (:`then_0`
      (`PrimitiveComponent.SetEnableGravity` _mesh false)
      (`PrimitiveComponent.SetSimulatePhysics` _mesh false)
      (`PrimitiveComponent.SetCollisionEnabled` (`self.Mesh`) "NoCollision")
      (`PrimitiveComponent.SetCollisionEnabled` _mesh "NoCollision")
      (`PrimitiveComponent.SetCollisionEnabled` (`self.EasyInteractCollision`) "NoCollision")
      (`PrimitiveComponent.SetCollisionEnabled` (`self.EasyInteractCollision`) "NoCollision"))
    (:`then_1`
      (if locallyControlled
        (`self.ActivateMaterialOnTop` _mesh_2)
        (`FXSystemComponent.SetFloatParameter` (`self.Fire`) "User.OnTopActive" 1.0)
        (`PrimitiveComponent.SetCastShadow` _mesh_2 false)))))

(event `self.TriggerPrimaryAction`
  (params (User :type "PlayerCharacter Object Reference"))
  ;[1 1 1] PrimaryAction
  (`parent.TriggerPrimaryAction` User)
  (if (> (`/Game/_DungeonCompanyContent/Code/Items/Torch/BP_Torch_Data.Fuel` (cast `/Game/_DungeonCompanyContent/Code/Items/Torch/BP_Torch_Data` (`self.MyData`) :!pure true)) 0.0)
    (set `self.RepOn` (not (`self.RepOn`)))))

(event `ToggleLight`
  (params (on :type Boolean))
  (bind _fireloopsound (`self.FireLoopSound`))
  ;[1 1 1] PrimaryAction
  (set `/Game/_DungeonCompanyContent/Code/Items/Torch/BP_Torch_Data.On` on (cast `/Game/_DungeonCompanyContent/Code/Items/Torch/BP_Torch_Data` (`self.MyData`) :!pure true))
  (`ActorComponent.SetActive` (`self.Fire`) on false)
  (if on
    (`GameplayStatics.SpawnSoundAttached` "/Game/_DungeonCompanyContent/Assets/Sound/SFX/Torch_Enlight.Torch_Enlight" (`self.Fire`) "None" (0.0 0.0 0.0) (struct) "KeepRelativeOffset" false 0.3 1.0 0.0 null null)
    (bind (_direction _0_to_1) (`Timeline|Light on/off` :!via `PlayFromStart` :!label _label)
      (:`Update`
        (`LightComponent.SetIntensity` (`self.PointLight`) (* (`self.OriginalLightIntensity`) _0_to_1)))
      (:`Finished`
        (if on
          (set `self.Flicker` true)
          (bind _returnvalue (`GameplayStatics.SpawnSoundAttached` "/Game/_DungeonCompanyContent/Assets/Sound/SFX/Torch_Crackling_SeamlessLoop.Torch_Crackling_SeamlessLoop" (`self.Fire`) "None" (0.0 0.0 0.0) (struct) "KeepRelativeOffset" false 0.5 1.0 0.0 null null))
          (set `self.FireLoopSound` _returnvalue))))
    (else
      (set `self.Flicker` false)
      (`|ExecutionSequence`
        (:`then_0`
          (goto _label :!via `ReverseFromEnd`))
        (:`then_1`
          (`/Engine/EditorBlueprintResources/StandardMacros.IsValid` _fireloopsound
            (:`Is Valid`
              (`AudioComponent.FadeOut` _fireloopsound 0.5 0.0 "Linear"))))))))

(event `self.ReceiveTick`
  (params (DeltaSeconds :type "Float (single-precision)"))
  (bind _returnvalue (`KismetMathLibrary.RandomFloatInRange` -0.5 0.5))
  (bind _pointlight (`self.PointLight`))
  (bind _originallightintensity (`self.OriginalLightIntensity`))
  (bind _asbp_torch_data (cast `/Game/_DungeonCompanyContent/Code/Items/Torch/BP_Torch_Data` (`self.MyData`) :!pure true))
  (`|ExecutionSequence`
    (:`then_0`
      ;[1 1 1] Flicker
      (if (`self.Flicker`)
        (`KismetSystemLibrary.Delay` (`KismetMathLibrary.RandomFloatInRange` 0.01 0.1))
        (`SceneComponent.K2_SetRelativeLocation` _pointlight (+ (`self.OriginalLightLocation`) (`KismetMathLibrary.MakeVector` _returnvalue _returnvalue)) false false)
        (`LightComponent.SetIntensity` _pointlight (+ _originallightintensity (`KismetMathLibrary.RandomFloatInRange` (* _originallightintensity -0.2) (* _originallightintensity 0.2))))))
    (:`then_1`
      ;[1 1 1] FuelConsumption
      (if (and (!= (`LightComponentBase.Intensity` (`self.PointLight`)) 0.0) (> (`/Game/_DungeonCompanyContent/Code/Items/Torch/BP_Torch_Data.Fuel` (cast `/Game/_DungeonCompanyContent/Code/Items/Torch/BP_Torch_Data` (`self.MyData`) :!pure true)) 0.0))
        (set `/Game/_DungeonCompanyContent/Code/Items/Torch/BP_Torch_Data.Fuel` (- (`/Game/_DungeonCompanyContent/Code/Items/Torch/BP_Torch_Data.Fuel` _asbp_torch_data) (`GameplayStatics.GetWorldDeltaSeconds`)) _asbp_torch_data)
        (if (<= (`/Game/_DungeonCompanyContent/Code/Items/Torch/BP_Torch_Data.Fuel` (cast `/Game/_DungeonCompanyContent/Code/Items/Torch/BP_Torch_Data` (`self.MyData`) :!pure true)) 0.0)
          (`/Engine/EditorBlueprintResources/ActorMacros.Switch Has Authority`
            (:`Authority`
              (set `self.RepOn` false))))))))

(event `self.ReceiveDestroyed`
  (bind _fireloopsound (`self.FireLoopSound`))
  (`/Engine/EditorBlueprintResources/StandardMacros.IsValid` _fireloopsound
    (:`Is Valid`
      (`AudioComponent.Stop` _fireloopsound))))

(fn `OnRep_RepOn`
  (bind _mydata (`self.MyData`))
  (`/Engine/EditorBlueprintResources/StandardMacros.IsValid` _mydata
    (:`Is Valid`
      (if (!= (`/Game/_DungeonCompanyContent/Code/Items/Torch/BP_Torch_Data.On` (cast `/Game/_DungeonCompanyContent/Code/Items/Torch/BP_Torch_Data` _mydata :!pure true)) (`self.RepOn`))
        (`self.ToggleLight` (`self.RepOn`))))))

(fn `UserConstructionScript`)