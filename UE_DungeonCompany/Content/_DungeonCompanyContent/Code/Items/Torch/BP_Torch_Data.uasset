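; BP_Torch_Data is the torch item's data object, holding its fuel level and lit state.
; It serializes both values into a semicolon-separated string and restores them by splitting that string on deserialization.
; Fuel doubles as the item's durability, with the maximum taken from the class defaults.
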(event `self.DeserializeMyData`
  (params (StringData :type String))
  (bind _returnvalue (`self.SeperateStringData` StringData))
  (`|ExecutionSequence`
    (:`then_0`
      (set `self.Fuel` (`KismetStringLibrary.Conv_StringToDouble` (`|GetArrayItem` _returnvalue))))
    (:`then_1`
      (set `self.bOn` (`KismetStringLibrary.EqualEqual_StrStr` (`|GetArrayItem` _returnvalue 1) "true")))))

(fn `GetDurabiltiy`
  (returns (Durability :type "Float (double-precision)") (MaxDurability :type "Float (double-precision)"))
  (return (`self.Fuel`) (defaults `/Game/_DungeonCompanyContent/Code/Items/Torch/BP_Torch_Data` "BP_Torch_Data_C")))

(fn `SerializeMyData`
  (returns (ReturnValue :type String))
  (return (`KismetStringLibrary.Concat_StrStr` (`KismetStringLibrary.Conv_DoubleToString` (`self.Fuel`)) ";" (`KismetStringLibrary.Conv_BoolToString` (`self.bOn`)))))