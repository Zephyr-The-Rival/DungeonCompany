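; Coal world item that lets the player holding it spray decals while primary action is held.
; Being held disables physics and collision, and for the local player renders the mesh on top without shadows.
; The hold input toggles a flag that makes Tick call the character's CoalSpawnDecal every frame.
; BeginPlay destroys the actor immediately, and selection wheel calls remain unconnected.
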(event `self.OnHoldingInHand`
  (params (LocallyControlled :type Boolean))
  (bind _staticmesh (`self.StaticMesh`))
  (bind _staticmesh_2 (`self.StaticMesh`))
  ;[1 1 1] On holding in hand
  (`|ExecutionSequence`
    (:`then_0`
      (`PrimitiveComponent.SetEnableGravity` _staticmesh false)
      (`PrimitiveComponent.SetSimulatePhysics` _staticmesh false)
      (`PrimitiveComponent.SetCollisionEnabled` (`self.StaticMesh`) "NoCollision")
      (`PrimitiveComponent.SetCollisionEnabled` _staticmesh "NoCollision")
      (`PrimitiveComponent.SetCollisionEnabled` (`self.Sphere`) "NoCollision"))
    (:`then_1`
      (if LocallyControlled
        (`self.ActivateMaterialOnTop` _staticmesh_2)
        (`PrimitiveComponent.SetCastShadow` _staticmesh_2 false)))))

(event `self.TriggerLocalPrimaryActionHold`
  (params (User :type "PlayerCharacter Object Reference"))
  (bind _asbp_player_character (cast `/Game/_DungeonCompanyContent/Code/PlayerCharacter/BP_PlayerCharacter` User))
  (set `self.MyCharacter` _asbp_player_character)
  (set `self.Spray` true))

(event `self.EndLocalPrimaryActionHold`
  (params (User :type "PlayerCharacter Object Reference"))
  (cast `/Game/_DungeonCompanyContent/Code/PlayerCharacter/BP_PlayerCharacter` User)
  (set `self.Spray` false))

(event `self.ReceiveTick`
  (params (DeltaSeconds :type "Float (single-precision)"))
  (if (`self.Spray`)
    (`/Game/_DungeonCompanyContent/Code/PlayerCharacter/BP_PlayerCharacter.CoalSpawnDecal` (`self.MyCharacter`))))

(event `self.ReceiveBeginPlay`
  (`self.K2_DestroyActor`))

(fn `UserConstructionScript`)