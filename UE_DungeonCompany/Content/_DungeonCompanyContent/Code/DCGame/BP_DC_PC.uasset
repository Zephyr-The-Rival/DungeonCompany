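; Player controller Blueprint for Dungeon Company that opens and closes the in-game options menu.
; ToggleOptionsMenu creates a new WBP_GameMenuStack on each open, switches to Game and UI input with a visible cursor, and reverses this on close.
; It also hides or restores the HUD of the possessed PlayerCharacter; other pawns, such as a spectator, get no HUD handling.
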(event `self.ToggleOptionsMenu`
  (params (On :type Boolean))
  ;[1 1 1] Options
  (if On
    (`|ExecutionSequence`
      (:`then_0`
        (`WidgetBlueprintLibrary.SetInputMode_GameAndUIEx` self null "DoNotLock" false true)
        (set `self.bShowMouseCursor` true)
        (bind _returnvalue (`|CreateWidget` "/Game/_DungeonCompanyContent/Code/UI/GameMenu/WBP_GameMenuStack.WBP_GameMenuStack_C"))
        (bind _output_get (set `self.CurrentOptionsMenu` _returnvalue))
        (`UserWidget.AddToViewport` _output_get 0))
      (:`then_1`
        (bind _asplayer_character (cast `PlayerCharacter` (`self.K2_GetPawn`))) ; maybe also for the spectator pawn
        (`Widget.SetVisibility` (`PlayerCharacter.GetMyHud` _asplayer_character) "Hidden")))
    (else
      (`|ExecutionSequence`
        (:`then_0`
          (`WidgetBlueprintLibrary.SetInputMode_GameOnly` self)
          (set `self.bShowMouseCursor` false)
          (`Widget.RemoveFromParent` (`self.CurrentOptionsMenu`)))
        (:`then_1`
          (bind _asplayer_character_2 (cast `PlayerCharacter` (`self.K2_GetPawn`))) ; maybe also for the spectator pawn
          (`Widget.SetVisibility` (`PlayerCharacter.GetMyHud` _asplayer_character_2) "Visible"))))))

(fn `UserConstructionScript`)