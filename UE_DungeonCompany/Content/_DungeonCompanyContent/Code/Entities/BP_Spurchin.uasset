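; Spurchin enemy creature with procedurally animated legs and timeline-driven body motion for idle, attack and hit reactions.
; Sphere traces place each leg target on surfaces, toggling planted state after a step length of travel and arcing step height by distance moved.
; A vertical trace sets the body center and lowers it under low ceilings.
; Attacks drive body and pincer transforms; death zeroes body and leg offsets.
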(event `self.ReceiveBeginPlay`
  (set `self.Center` (`self.K2_GetActorLocation`))
  ;[1 1 1] RayCast Legs
  (for (_array_element _array_index) (`self.Legs`)
    (bind _returnvalue_location (`KismetMathLibrary.BreakTransform` (`SkinnedMeshComponent.GetBoneTransform` (`self.Mesh`) (`.ToeName_15_E4BF452742788D6B9A82848356C47169` (break `/Game/_DungeonCompanyContent/Assets/Enemies/Spurchin/S_SpurchinLegs` _array_element)) "RTS_World")))
    (bind (_raystart _rayend) (`self.GetVerticalRay` _returnvalue_location (`self.LegUpperRay`) (`self.LegLowerRay`)))
    (bind (_location _hittraceend) (`self.CastRay` _raystart _rayend)
      (:`Hit`
        (setmembers `/Game/_DungeonCompanyContent/Assets/Enemies/Spurchin/S_SpurchinLegs` :`StructRef` (`|GetArrayItem` (`self.Legs`) _array_index) :`Location` _location :`InitialOffSet` (- _hittraceend (`self.K2_GetActorLocation`))))))
  (set `self.PrevLocation` (`self.K2_GetActorLocation`))
  (set `self.Ready` true)
  (set `self.PincerRotation` (struct)))

(event `self.ReceiveTick`
  (params (DeltaSeconds :type "Float (single-precision)"))
  (bind (_returnvalue_x _returnvalue_y _returnvalue_z) (`KismetMathLibrary.BreakVector` (`self.K2_GetActorLocation`)))
  (bind (_returnvalue_roll _returnvalue_pitch _returnvalue_yaw) (`KismetMathLibrary.BreakRotator` (`self.K2_GetActorRotation`)))
  (bind _returnvalue (`self.K2_GetActorLocation`))
  (bind (_returnvalue_roll_2 _returnvalue_pitch_2 _returnvalue_yaw_2) (`KismetMathLibrary.BreakRotator` (`self.K2_GetActorRotation`)))
  (bind _legs (`self.Legs`))
  (bind _legrotation_roll (`KismetMathLibrary.BreakRotator` (`self.LegRotation`)))
  (bind _legrotation_roll_2 (`KismetMathLibrary.BreakRotator` (`self.LegRotation`)))
  (bind (_ceilingcheck_x _ceilingcheck_y _ceilingcheck_z) (`KismetMathLibrary.BreakVector` (`self.CeilingCheck`)))
  (bind (_bodylocation_x _bodylocation_y _bodylocation_z) (`KismetMathLibrary.BreakVector` (`self.BodyLocation`)))
  (bind (_ceilingcheck_x_2 _ceilingcheck_y_2 _ceilingcheck_z_2) (`KismetMathLibrary.BreakVector` (`self.CeilingCheck`)))
  (bind _returnvalue_2 (`KismetMathLibrary.Vector_Distance2D` (`self.K2_GetActorLocation`) (`self.PrevLocation`)))
  (bind (_raystart _rayend) (`self.GetVerticalRay` _returnvalue (`self.CaveHeight`) -100.0))
  (bind (_relativelocation_x _relativelocation_y _relativelocation_z) (`KismetMathLibrary.BreakVector` (`SceneComponent.RelativeLocation` (`self.Mesh`))))
  (`parent.ReceiveTick` DeltaSeconds)
  (`|ExecutionSequence`
    (:`then_0`
      (`|ExecutionSequence`
        (:`then_0`
          ;[1 1 1] Set Root Location
          (set `self.Center` _returnvalue)
          (bind (_location _hittraceend _outhit_impactnormal _outhit_tracestart) (`self.CastRay` _raystart _rayend 50.0)
            (:`Hit`
              (bind _output_get (set `self.Center` _location))
              (set `self.CeilingCheck` (- _outhit_tracestart _output_get)))
            (:`NoHit`
              ;;[1 0.9046 0.3931] If Nothing is hit, set to world location
              (set `self.Center` (`KismetMathLibrary.MakeVector` _returnvalue_x _returnvalue_y (+ _returnvalue_z _relativelocation_z))))))
        (:`then_1`
          ;[1 1 1] Push body down when ceiling is low
          (if (> (`self.CaveHeight`) _ceilingcheck_z)
            (`/Engine/EditorBlueprintResources/StandardMacros.DoOnce` false :!label _label
              (:`Completed`
                (set `self.BodyLocation` (`KismetMathLibrary.MakeVector` 0.0 0.0 (- _bodylocation_z (* (`KismetMathLibrary.Abs` _ceilingcheck_z_2) 0.3))))
                (goto _label_2 :!via `Reset`)))
            (else
              (`/Engine/EditorBlueprintResources/StandardMacros.DoOnce` false :!label _label_2
                (:`Completed`
                  (set `self.BodyLocation` (0.0 0.0 0.0))
                  (goto _label :!via `Reset`))))))
        (:`then_2`
          ;[1 1 1] Move Leg
          (for (_array_element _array_index) (`self.Legs`) :!label _label_3
            (bind _returnvalue_3 (not (`.Planted_12_EA2BC3C24193A96196CDD7A8254D9689` (break `/Game/_DungeonCompanyContent/Assets/Enemies/Spurchin/S_SpurchinLegs` _array_element))))
            (if _returnvalue_3
              (bind (_raystart_2 _rayend_2) (`self.GetVerticalRay` (+ (`KismetMathLibrary.GreaterGreater_VectorRotator` (`.InitialOffSet_11_654236D84EDFF13C739DD4A6850575C7` (break `/Game/_DungeonCompanyContent/Assets/Enemies/Spurchin/S_SpurchinLegs` _array_element)) (`KismetMathLibrary.MakeRotator` _legrotation_roll_2 0.0 _returnvalue_yaw_2)) (`self.K2_GetActorLocation`)) (`self.LegUpperRay`) (`self.LegLowerRay`)))
              (bind (_location_2 _hittraceend_2) (`self.CastRay` _raystart_2 _rayend_2 (`self.LegRadius`))
                (:`Hit`
                  (bind _output (`|GetArrayItem` (`self.Legs`) _array_index))
                  (setmembers `/Game/_DungeonCompanyContent/Assets/Enemies/Spurchin/S_SpurchinLegs` :`StructRef` _output :`Location` (`KismetMathLibrary.MakeVector` (.x _location_2) (.y _location_2) (+ (.z _location_2) (`self.GetLegHeight` _returnvalue_2)))))
                (:`NoHit`
                  (bind _location_3 (`self.CastRay` _hittraceend_2 (`self.Center`) (`self.LegRadius`))
                    (:`Hit`
                      (setmembers `/Game/_DungeonCompanyContent/Assets/Enemies/Spurchin/S_SpurchinLegs` :`StructRef` _output :`Location` _location_3))
                    (:`NoHit`
                      (setmembers `/Game/_DungeonCompanyContent/Assets/Enemies/Spurchin/S_SpurchinLegs` :`StructRef` _output :`Planted` _returnvalue_3)))))))
          ;[1 1 1] Swap Legs
          (if (> _returnvalue_2 (`self.StepLength`))
            (for (_array_element_2 _array_index_2) _legs
              (bind (_raystart_3 _rayend_3) (`self.GetVerticalRay` (+ (`KismetMathLibrary.GreaterGreater_VectorRotator` (`.InitialOffSet_11_654236D84EDFF13C739DD4A6850575C7` (break `/Game/_DungeonCompanyContent/Assets/Enemies/Spurchin/S_SpurchinLegs` _array_element_2)) (`KismetMathLibrary.MakeRotator` _legrotation_roll 0.0 _returnvalue_yaw)) (`self.K2_GetActorLocation`)) (`self.LegUpperRay`) (`self.LegLowerRay`)))
              (bind _location_4 (`self.CastRay` _raystart_3 _rayend_3 (`self.LegRadius`))
                (:`Hit`
                  (bind _output_2 (`|GetArrayItem` _legs _array_index_2))
                  (bind _returnvalue_4 (not (`.Planted_12_EA2BC3C24193A96196CDD7A8254D9689` (break `/Game/_DungeonCompanyContent/Assets/Enemies/Spurchin/S_SpurchinLegs` _array_element_2))))
                  (setmembers `/Game/_DungeonCompanyContent/Assets/Enemies/Spurchin/S_SpurchinLegs` :`StructRef` _output_2 :`Location` (`KismetMathLibrary.MakeVector` (.x _location_4) (.y _location_4) (+ (.z _location_4) (`self.GetLegHeight` (`KismetMathLibrary.Vector_Distance2D` (`self.K2_GetActorLocation`) (`self.PrevLocation`))))) :`Planted` _returnvalue_4))
                (:`NoHit`
                  (bind _location_5 (`self.CastRay` (0.0 0.0 0.0) (`self.Center`) (`self.LegRadius`))
                    (:`Hit`
                      (setmembers `/Game/_DungeonCompanyContent/Assets/Enemies/Spurchin/S_SpurchinLegs` :`StructRef` _output_2 :`Location` _location_5))
                    (:`NoHit`
                      (setmembers `/Game/_DungeonCompanyContent/Assets/Enemies/Spurchin/S_SpurchinLegs` :`StructRef` _output_2 :`Planted` _returnvalue_4))))))
            (set `self.PrevLocation` (`self.K2_GetActorLocation`))))
        (:`then_3`
          ;[0.5176 1 0.3804] Idle
          (bind _output_get_2 (set `self.Velocity` (`self.GetVelocity`)))
          (if (and (`KismetMathLibrary.NearlyEqual_FloatFloat` (`KismetMathLibrary.VSize` _output_get_2) 0.0 0.003) (not (`self.BeingHit`)) (not (`self.Attacking`)))
            (bind (_direction _lerp) (`Timeline|Idle` :`NewTime` 5.0 :!label _label_4)
              (:`Update`
                (set `self.BodyLocation` (`KismetMathLibrary.VLerp` (0.0 0.0 0.0) (0.0 0.0 -10.0) _lerp))))
            (else
              (goto _label_4 :!via `Stop`))))
        (:`then_5`
          (goto _label_3))))
    (:`then_1`
      (`KismetSystemLibrary.Delay` 0.1)
      (`self.CheckSpace`))))

(event `self.OnAttackingPlayer`
  (params (PlayerAttacking :type "PlayerCharacter Object Reference")))

(event `self.OnExecuteAttack`
  (params (Direction :type "Vector Structure"))
  (bind _returnvalue (`self.K2_GetActorRotation`))
  (bind _returnvalue_2 (`self.K2_GetActorRotation`))
  (bind (_returnvalue_x _returnvalue_y _returnvalue_z) (`KismetMathLibrary.BreakVector` (`self.GetActorForwardVector`)))
  ;[0.5176 1 0.3804] Attack
  (if (not (`self.BeingHit`))
    (set `self.PincerRotation` _returnvalue_2)
    (set `self.BodyRotation` _returnvalue_2)
    (set `self.Attacking` true)
    (bind (_direction _rotlerp _pincerrotlerp _zloclerp _xloclerp) (`Timeline|Attack` :!via `PlayFromStart` :!label _label_5)
      (:`Update`
        (set `self.BodyRotation` (`KismetMathLibrary.RLerp` (struct :`Roll` -70.0) (struct :`Roll` 30.0) _rotlerp))
        (set `self.BodyLocation` (`KismetMathLibrary.MakeVector` (+ _returnvalue_x (`KismetMathLibrary.Lerp` -30.0 30.0 _xloclerp)) _returnvalue_y (+ _returnvalue_z (`KismetMathLibrary.Lerp` -80.0 15.0 _zloclerp))))
        (bind _returnvalue_roll (`KismetMathLibrary.BreakRotator` (`KismetMathLibrary.RLerp` (struct :`Yaw` -100.0) (struct :`Yaw` 100.0) _pincerrotlerp)))
        (set `self.PincerRotation` (`KismetMathLibrary.MakeRotator` _returnvalue_roll)))
      (:`Finished`
        (set `self.Attacking` false)
        (set `self.BodyRotation` _returnvalue)
        (set `self.PincerRotation` _returnvalue)))
    (else
      (goto _label_5 :!via `Stop`))))

(event `self.OnTookDamage`
  ;[0.5176 1 0.3804] Hit
  (set `self.BeingHit` true)
  (bind (_direction _lerp) (`Timeline|Hit` :`NewTime` 5.0 :!via `PlayFromStart`)
    (:`Update`
      (set `self.BodyLocation` (`KismetMathLibrary.VLerp` (0.0 0.0 -40.0) (0.0 0.0 10.0) _lerp)))
    (:`Finished`
      (set `self.BeingHit` false))))

(event `self.OnDeath`
  (bind _legs (`self.Legs`))
  ;[0.5176 1 0.3804] Death
  (`KismetSystemLibrary.LogString` "Died")
  (set `self.BodyLocation` (0.0 0.0 0.0))
  (for (_ _array_index) _legs
    (setmembers `/Game/_DungeonCompanyContent/Assets/Enemies/Spurchin/S_SpurchinLegs` :`StructRef` (`|GetArrayItem` _legs _array_index) :`Location` (0.0 0.0 0.0) :`InitialOffSet` (0.0 0.0 0.0))))

(fn `GetHorizontalRay`
  (params (Location :type "Vector Structure") (Positive :type "Float (double-precision)") (Negative :type "Float (double-precision)"))
  (returns (RayStart :type "Vector Structure") (RayEnd :type "Vector Structure"))
  (return (`KismetMathLibrary.MakeVector` (+ Location_X Positive) Location_Y Location_Z) (`KismetMathLibrary.MakeVector` (+ Location_X Negative) Location_Y Location_Z)))

(fn `GetLegHeight`
  (params (Distance :type "Float (double-precision)"))
  (returns (Z :type "Float (double-precision)"))
  (return (* (- 1.0 (`KismetMathLibrary.MultiplyMultiply_FloatFloat` (`KismetMathLibrary.FClamp` (/ Distance (`self.StepLength`))) 2.0)) (`self.StepHeight`))))

(fn `GetVerticalRay`
  (params (Location :type "Vector Structure") (Upper :type "Float (double-precision)") (Lower :type "Float (double-precision)"))
  (returns (RayStart :type "Vector Structure") (RayEnd :type "Vector Structure"))
  (return (`KismetMathLibrary.MakeVector` Location_X Location_Y (+ Location_Z Upper)) (`KismetMathLibrary.MakeVector` Location_X Location_Y (+ Location_Z Lower))))

(fn `UserConstructionScript`)