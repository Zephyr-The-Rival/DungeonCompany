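; BP_FunGuy is an entity with a pulsing point light and an idle breath sound.
; Tick drives the light intensity with a sine of game time, using a random offset set on BeginPlay so instances pulse out of sync.
; BeginPlay also calls RandomBreath, which plays FunGuyIdle at the actor's location once after a random delay, with no re-trigger.
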(event `self.ReceiveBeginPlay`
  (`parent.ReceiveBeginPlay`)
  (set `self.TimeOffset` (`KismetMathLibrary.RandomFloatInRange` 0.0 3.0))
  (`self.RandomBreath`))

(event `self.ReceiveTick`
  (params (DeltaSeconds :type "Float (single-precision)"))
  (`LightComponent.SetIntensity` (`self.PointLight`) (* (`self.Intensity`) (`KismetMathLibrary.Sin` (+ (`KismetSystemLibrary.GetGameTimeInSeconds`) (`self.TimeOffset`))))))

(event `RandomBreath`
  (`KismetSystemLibrary.Delay` (`KismetMathLibrary.RandomFloatInRange` 10.0 40.0))
  (`GameplayStatics.PlaySoundAtLocation` "/Game/_DungeonCompanyContent/Audio/FunGuyIdle.FunGuyIdle" (`self.K2_GetActorLocation`) (struct) 1.0 1.0 0.0 null null null null))

(fn `UserConstructionScript`)