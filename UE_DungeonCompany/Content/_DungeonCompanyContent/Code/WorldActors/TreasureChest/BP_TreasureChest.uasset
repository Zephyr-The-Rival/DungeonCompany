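; Treasure chest actor that, on server interaction, plays its opening animation, marks itself used and launches loot after a short delay.
; Opening disables the box collision and drives a brief shine through a timeline on a dynamic material and point light.
; Loot spawning recursively steps through the loot table with delays, rolling each item's probability and impulsing spawns along the shoot vector with random spread.
; Clients finding it already used at BeginPlay show it statically open.
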(event `self.ReceiveBeginPlay`
  (if (and (`self.Used`) (not (`self.HasAuthority`)))
    (`self.DeactivateOnStart`)))

(event `self.OnInteractedOnServer`
  (`self.Open`)
  (set `self.Used` true)
  (`KismetSystemLibrary.Delay` 1.0)
  (`self.SpawnLoot`))

(event `Open`
  (`SkeletalMeshComponent.PlayAnimation` (`self.SK_treasureChest`) "/Game/_DungeonCompanyContent/Assets/WorldActors/TreasureChest/SK_treasureChest_Open_Anim.SK_treasureChest_Open_Anim" false)
  (`self.ShineUp`))

(event `ShineUp`
  (`PrimitiveComponent.SetCollisionEnabled` (`self.Box`) "NoCollision")
  (`KismetSystemLibrary.Delay` 0.5)
  (`SceneComponent.SetVisibility` (`self.TreasureChestShine`) true false)
  (`SceneComponent.SetVisibility` (`self.PointLight`) true false)
  (bind _returnvalue (`KismetMaterialLibrary.CreateDynamicMaterialInstance` "/Game/_DungeonCompanyContent/Assets/WorldActors/TreasureChest/Shine/M_TreasureShine.M_TreasureShine"))
  (`PrimitiveComponent.SetMaterial` (`self.TreasureChestShine`) 0 _returnvalue)
  (bind (_direction _010) (`Timeline|Timeline` :!via `PlayFromStart`)
    (:`Update`
      (`MaterialInstanceDynamic.SetScalarParameterValue` _returnvalue "Brightness" _010)
      (`LightComponent.SetIntensity` (`self.PointLight`) (* _010 5000.0)))
    (:`Finished`
      (`SceneComponent.SetVisibility` (`self.TreasureChestShine`) false false)
      (`SceneComponent.SetVisibility` (`self.PointLight`) false false))))

(event `SpawnLoot`
  (bind (_itemtospawn _spawnprobability) (break `/Game/_DungeonCompanyContent/Code/WorldActors/TreasureChest/LootTableEntry` (`|GetArrayItem` (`self.LootTable`) (`self.LootIterator`))))
  (if (< (`self.LootIterator`) (`KismetArrayLibrary.Array_Length` (`self.LootTable`)))
    (`|ExecutionSequence`
      (:`then_0`
        (if (>= _spawnprobability (`KismetMathLibrary.RandomFloatInRange` 0.0 100.0))
          (bind _returnvalue (`|SpawnActorFromClass` _itemtospawn (`KismetMathLibrary.MakeTransform` (+ (`SceneComponent.K2_GetComponentLocation` (`self.DefaultSceneRoot`)) (0.0 0.0 40.0))) "Undefined" "MultiplyWithRoot" null null))
          (bind _asmesh_component (cast `MeshComponent` (`Actor.RootComponent` _returnvalue)))
          (`PrimitiveComponent.AddImpulse` _asmesh_component (* (+ (* (`KismetMathLibrary.MakeVector` (`KismetMathLibrary.RandomFloatInRange` -1.0 1.0) (`KismetMathLibrary.RandomFloatInRange` -1.0 1.0) 1.0) (0.1 0.1 0.1)) (`SceneComponent.GetForwardVector` (`self.ShootVector`))) (`self.Shoot strenght`)) "None" true)))
      (:`then_1`
        (`KismetSystemLibrary.Delay` 0.2)
        (`/Engine/EditorBlueprintResources/StandardMacros.IncrementInt` (`self.LootIterator`)
          (:`  `
            (`self.SpawnLoot`)))))))

(event `DeactivateOnStart`
  (`ActorComponent.K2_DestroyComponent` (`self.TreasureChestShine`))
  (`ActorComponent.K2_DestroyComponent` (`self.PointLight`))
  (`ActorComponent.K2_DestroyComponent` (`self.Box`))
  (`SkeletalMeshComponent.PlayAnimation` (`self.SK_treasureChest`) "/Game/_DungeonCompanyContent/Assets/WorldActors/TreasureChest/SK_treasureChest_StaticOpen.SK_treasureChest_StaticOpen" false))

(fn `UserConstructionScript`)