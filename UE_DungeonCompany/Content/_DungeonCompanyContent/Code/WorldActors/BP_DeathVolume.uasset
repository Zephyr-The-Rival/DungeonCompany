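; BP_DeathVolume is a world trigger box that kills entities and removes world items that overlap it.
; On overlap, it calls OnDeath on any DC_Entity that is not already dead.
; Overlapping WorldItems are, on authority only, passed to the level's BP_LostIemsCollection and then destroyed, even if no collection is found.
; The entity death call has no authority check in this Blueprint.
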(event `self.Box.OnComponentBeginOverlap`
  (params (OverlappedComponent :type "PrimitiveComponent Object Reference") (OtherActor :type "Actor Object Reference") (OtherComp :type "PrimitiveComponent Object Reference") (OtherBodyIndex :type Integer) (bFromSweep :type Boolean) (SweepResult :type "HitResult Structure (by ref)"))
  (`|ExecutionSequence`
    (:`then_0`
      (bind _asdc_entity (cast `DC_Entity` OtherActor))
      (if (not (`DC_Entity.IsDead` _asdc_entity))
        (`DC_Entity.OnDeath` _asdc_entity)))
    (:`then_1`
      (bind _asworld_item (cast `WorldItem` OtherActor))
      (`self.AddToLostItems` _asworld_item))))

(event `AddToLostItems`
  (params (WorldItem :type "WorldItem Object Reference"))
  (`/Engine/EditorBlueprintResources/ActorMacros.Switch Has Authority`
    (:`Authority`
      (`|ExecutionSequence`
        (:`then_0`
          (bind _returnvalue (`GameplayStatics.GetActorOfClass` "/Game/_DungeonCompanyContent/Code/WorldActors/LostItemsManager/BP_LostIemsCollection.BP_LostIemsCollection_C"))
          (`/Engine/EditorBlueprintResources/StandardMacros.IsValid` _returnvalue
            (:`Is Valid`
              (`/Game/_DungeonCompanyContent/Code/WorldActors/LostItemsManager/BP_LostIemsCollection.AddToLostItems` _returnvalue WorldItem))
            (:`Is Not Valid`
              (`KismetSystemLibrary.PrintString` "No lost items collection found"))))
        (:`then_1`
          (`self.K2_DestroyActor` WorldItem))))))

(fn `UserConstructionScript`)