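; BP_KathisDecal is a world actor whose mesh glow toggles as lever feedback.
; The construction script creates a dynamic material on the StaticMesh and applies a default EmissiveAmount.
; LeverFeedback flips DidSwitch to alternate between default and fixed emissive values, with an older rotation toggle left unconnected.
; LeverSet separately flips and returns IsPressed, printing On or Off.
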(fn `Lever Feedback`
  (locals (NewLocalVar :type "Array of Float (single-precision)"))
  (bind _dynamicmat (`self.DynamicMat`))
  (if (`self.DidSwitch`)
    (`MaterialInstanceDynamic.SetScalarParameterValue` _dynamicmat "EmissiveAmount" (`self.DefaultEmissiveAmount`))
    (set `self.DidSwitch` false)
    (else
      (`MaterialInstanceDynamic.SetScalarParameterValue` _dynamicmat "EmissiveAmount" 2.0)
      (set `self.DidSwitch` true))))

(fn `LeverSet`
  (returns (IsPressed :type Boolean))
  (if (`self.isPressed`)
    (`KismetSystemLibrary.PrintString` "Off")
    (bind _output_get (set `self.isPressed` false))
    (return _output_get)
    (else
      (`KismetSystemLibrary.PrintString` "On")
      (bind _output_get_2 (set `self.isPressed` true))
      (return _output_get_2))))

(fn `UserConstructionScript`
  (bind _staticmesh (`self.StaticMesh`))
  (bind _returnvalue (`PrimitiveComponent.CreateDynamicMaterialInstance` _staticmesh 0 (`PrimitiveComponent.GetMaterial` _staticmesh 0) "None"))
  (bind _output_get (set `self.DynamicMat` _returnvalue))
  (`MaterialInstanceDynamic.SetScalarParameterValue` _output_get "EmissiveAmount" (`self.DefaultEmissiveAmount`)))