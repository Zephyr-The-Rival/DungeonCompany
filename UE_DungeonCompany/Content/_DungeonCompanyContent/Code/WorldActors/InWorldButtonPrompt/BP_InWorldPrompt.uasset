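; World-space button prompt actor that shows an input action's icon on a plane alongside a text label.
; Gets gamepad and keyboard/mouse textures from PromptTexturesSupplier once loading finishes, then swaps them on a dynamic material when the input device changes.
; Tick optionally turns it toward the first-person camera, fades icon and text by player distance, and hides it while the player is dead, using DoOnce gates to avoid repeated updates.
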(event `self.ReceiveBeginPlay`
  (bind _returnvalue (`KismetMaterialLibrary.CreateDynamicMaterialInstance` "/Game/_DungeonCompanyContent/Assets/Materials/M_InWorldPrompt.M_InWorldPrompt"))
  (set `self.PlaneMaterial` _returnvalue)
  (`PrimitiveComponent.SetMaterial` (`self.Plane`) 0 _returnvalue)
  (bind _returnvalue_2 (`GameplayStatics.GetActorOfClass` "/Game/_DungeonCompanyContent/Code/WorldActors/InWorldButtonPrompt/PromptTexturesSupplier.PromptTexturesSupplier_C"))
  (`/Engine/EditorBlueprintResources/StandardMacros.IsValid` _returnvalue_2
    (:`Is Valid`
      (add `/Game/_DungeonCompanyContent/Code/WorldActors/InWorldButtonPrompt/PromptTexturesSupplier.PromptTextureLoadingFinished` _returnvalue_2 (delegate `LoadTextures`)))
    (:`Is Not Valid`
      (`KismetSystemLibrary.PrintString` "No prompt texture supplier found"))))

(event `LoadTextures`
  (bind _returnvalue (`GameplayStatics.GetActorOfClass` "/Game/_DungeonCompanyContent/Code/WorldActors/InWorldButtonPrompt/PromptTexturesSupplier.PromptTexturesSupplier_C"))
  (bind (_controllertexture _maktexture) (`/Game/_DungeonCompanyContent/Code/WorldActors/InWorldButtonPrompt/PromptTexturesSupplier.Get Prompt Textures` _returnvalue (`self.Input Action`) "/Game/_DungeonCompanyContent/Input/CharacterIMC.CharacterIMC" false null))
  (set `self.Controller Texture` _controllertexture)
  (set `self.Mak Texture` _maktexture)
  (bind _asbp_dc_pc (cast `/Game/_DungeonCompanyContent/Code/DCGame/BP_DC_PC` (`GameplayStatics.GetPlayerController` 0)))
  (add `DC_PC.OnInputDeviceChanged` _asbp_dc_pc (delegate `Update`))
  (`self.Update` (`DC_PC.IsUsingGamepad` _asbp_dc_pc)))

(event `Update`
  (params (IsUsingGamepad :type Boolean))
  (if IsUsingGamepad
    (`MaterialInstanceDynamic.SetTextureParameterValue` (`self.PlaneMaterial`) "Texture" (`self.Controller Texture`))
    (else
      (`MaterialInstanceDynamic.SetTextureParameterValue` (`self.PlaneMaterial`) "Texture" (`self.Mak Texture`)))))

(event `self.ReceiveTick`
  (params (DeltaSeconds :type "Float (single-precision)"))
  (bind _fadedistancestart (`self.FadeDistanceStart`))
  (bind _defaultsceneroot (`self.DefaultSceneRoot`))
  (bind _asplayer_character (cast `PlayerCharacter` (`Controller.K2_GetPawn` (`GameplayStatics.GetPlayerController` 0))))
  (if (not (`DC_Entity.IsDead` _asplayer_character))
    (`|ExecutionSequence`
      (:`then_0`
        (`|ExecutionSequence`
          (:`then_0`
            (`/Engine/EditorBlueprintResources/StandardMacros.DoOnce` false :!label _label
              (:`Completed`
                (`SceneComponent.SetHiddenInGame` (`self.DefaultSceneRoot`) false true))))
          (:`then_1`
            ;[1 1 1] TurnToPlayer
            (if (`self.TurnTowardsPlayer`)
              (`SceneComponent.K2_SetWorldRotation` _defaultsceneroot (`KismetMathLibrary.Conv_VectorToRotator` (- (`SceneComponent.K2_GetComponentLocation` (`PlayerCharacter.FirstPersonCamera` _asplayer_character)) (`SceneComponent.K2_GetComponentLocation` _defaultsceneroot))) false false)))
          (:`then_2`
            ;[1 1 1] FadeByDistance
            (bind _output_get (set `self.DistanceToPlayer` (`KismetMathLibrary.Vector_Distance` (`self.K2_GetActorLocation`) (`self.K2_GetActorLocation` _asplayer_character))))
            (if (< _output_get (`self.FadeDistanceStart`))
              (`|ExecutionSequence`
                (:`then_0`
                  (if (> (`self.DistanceToPlayer`) (`self.FadeDistanceEnd`))
                    (`|ExecutionSequence`
                      (:`then_0`
                        (`self.SetAlpha` (/ (- _fadedistancestart (`self.DistanceToPlayer`)) (- _fadedistancestart (`self.FadeDistanceEnd`)))))
                      (:`then_1`
                        (goto _label_2 :!via `Reset`)))
                    (else
                      (`/Engine/EditorBlueprintResources/StandardMacros.DoOnce` false :!label _label_2
                        (:`Completed`
                          (`self.SetAlpha` 1.0))))))
                (:`then_1`
                  (goto _label_3 :!via `Reset`)))
              (else
                (`/Engine/EditorBlueprintResources/StandardMacros.DoOnce` false :!label _label_3
                  (:`Completed`
                    (`self.SetAlpha` 0.0))))))))
      (:`then_1`
        (goto _label_4 :!via `Reset`)))
    (else
      (`/Engine/EditorBlueprintResources/StandardMacros.DoOnce` false :!label _label_4
        (:`Completed`
          (`|ExecutionSequence`
            (:`then_0`
              (goto _label :!via `Reset`))
            (:`then_1`
              (`SceneComponent.SetHiddenInGame` (`self.DefaultSceneRoot`) true true))))))))

(event `SetAlpha`
  (params (NewAlpha :type "Float (double-precision)"))
  (bind _textrender (`self.TextRender`))
  (bind (_textrendercolor_b _textrendercolor_g _textrendercolor_r) (break `Color` (`TextRenderComponent.TextRenderColor` _textrender)))
  ;[1 1 1] FadeByDistance
  (`MaterialInstanceDynamic.SetScalarParameterValue` (`self.PlaneMaterial`) "Alpha" NewAlpha)
  (`TextRenderComponent.SetTextRenderColor` _textrender (make `Color` _textrendercolor_b _textrendercolor_g _textrendercolor_r (`KismetMathLibrary.Conv_Int64ToByte` (`KismetMathLibrary.Round64` (* NewAlpha 255.0))))))

(fn `UpdateButtonPrompt`
  (params (IsUsingGamepad1 :type Boolean)))

(fn `UserConstructionScript`
  (`TextRenderComponent.K2_SetText` (`self.TextRender`) (`self.Text`)))