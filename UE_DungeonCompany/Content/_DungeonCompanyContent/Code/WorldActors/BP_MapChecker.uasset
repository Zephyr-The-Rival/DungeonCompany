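; BP_MapChecker is a level-validation actor that verifies required singleton actors are placed correctly in a map.
; On BeginPlay or the ConductMapCheck event, only on the authority, it loops through the ActorsToExistOnlyOnce class list.
; For each class it counts instances in the world and prints a color-coded on-screen message: green for exactly one, red for missing or duplicated.
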(event `self.ReceiveBeginPlay`
  (`/Engine/EditorBlueprintResources/ActorMacros.Switch Has Authority` :!label _label
    (:`Authority`
      (`|ExecutionSequence`
        (:`then_0`
          (`KismetSystemLibrary.PrintString` " \n \n \nRunning Map Check..." true true (struct :`R` 1.0 :`G` 0.494074 :`A` 1.0) (`self.DisplayTime`))
          (for _array_element (`self.Actors to exist only once`)
            (`self.Check If there is only one` _array_element)))))))

(event `ConductMapCheck`
  (goto _label))

(fn `Check If there is only one`
  (params (ActorClass :type "Actor Class Reference"))
  (bind _displaytime (`self.DisplayTime`))
  (bind _outactors (`GameplayStatics.GetAllActorsOfClass` ActorClass))
  (bind _returnvalue (`KismetArrayLibrary.Array_Length` _outactors))
  (switch `int` _returnvalue
    (:`Default`
      (`KismetSystemLibrary.PrintString` (`KismetStringLibrary.Concat_StrStr` (`KismetSystemLibrary.GetClassDisplayName` ActorClass) " exists more then once: " (`KismetStringLibrary.Conv_IntToString` _returnvalue) " times") true true (struct :`R` 1.0 :`A` 1.0) _displaytime))
    (:`0`
      (`KismetSystemLibrary.PrintString` (`KismetStringLibrary.Concat_StrStr` (`KismetSystemLibrary.GetClassDisplayName` ActorClass) " is missing") true true (struct :`R` 1.0 :`A` 1.0) _displaytime))
    (:`1`
      (`KismetSystemLibrary.PrintString` (`KismetStringLibrary.Concat_StrStr` (`KismetSystemLibrary.GetClassDisplayName` ActorClass) " exists") true true (struct :`G` 1.0 :`A` 1.0) _displaytime))))

(fn `UserConstructionScript`)