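; Manager actor that resets the dungeon, with the reset accepted only on the server.
; ResetDungeon multicasts a local reset message to every BP_Resettable actor, then requests respawns for spectating players.
; It then saves through BP_SaveManager, in that order because saving assumes all players are alive, and finally flips the RespawnCrystals flag.
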(event `self.BP_ResetDungeon`
  ;[1 0.5688 0.02292] On Server
  ; Reset
  (`/Engine/EditorBlueprintResources/ActorMacros.Switch Has Authority`
    (:`Authority`
      (`|ExecutionSequence`
        (:`then_0`
          (`self.MulticastReset`))
        (:`then_1`
          (`self.RespawnAllPlayers`))
        (:`then_2`
          (bind _returnvalue (`GameplayStatics.GetActorOfClass` "/Game/_DungeonCompanyContent/Code/WorldActors/SaveManager/BP_SaveManager.BP_SaveManager_C")) ; order is important\nsaving assumes all players are alive
          (`/Game/_DungeonCompanyContent/Code/WorldActors/SaveManager/BP_SaveManager.SaveGame` _returnvalue))
        (:`then_3`
          (set `self.RespawnCrystals` (not (`self.RespawnCrystals`))))))
    (:`Remote`
      (`KismetSystemLibrary.PrintString` "Reset Needs To Be Called From Server"))))

(event `MulticastReset`
  ;[1 0 0.7316] Multicast
  ; Reset
  (bind _outactors (`GameplayStatics.GetAllActorsWithInterface` "/Game/_DungeonCompanyContent/Code/WorldActors/DungeonReset/BP_Resettable.BP_Resettable_C"))
  (for _array_element _outactors
    (message `/Game/_DungeonCompanyContent/Code/WorldActors/DungeonReset/BP_Resettable.LocalReset` _array_element)))

(fn `RespawnAllPlayers`
  (bind _outactors (`GameplayStatics.GetAllActorsOfClass` "/Game/_DungeonCompanyContent/Code/DCGame/BP_DC_PC.BP_DC_PC_C"))
  (for _array_element _outactors
    (if (`|EnumEquality` (`DC_PC.PawnType` _array_element) "Spectator")
      (`DC_PC.Server_RequestRespawn` _array_element))))

(fn `UserConstructionScript`)