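; BP_KathisTorch is a world actor for a torch that can be switched on and off.
; Despite its name, TurnTorchOn is a toggle that uses the DidSwitch flag to activate or deactivate the Audio and Fire components and show or hide TorchLightStatic.
; The event graph and construction script are empty, and nothing in the file calls the toggle.
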(fn `Turn Torch On`
  (locals (NewLocalVar :type "Array of Float (single-precision)"))
  (if (`self.DidSwitch`)
    (`ActorComponent.Deactivate` (`self.Audio`))
    (`ActorComponent.Deactivate` (`self.Fire`))
    (`SceneComponent.SetVisibility` (`self.TorchLightStatic`) false false)
    (set `self.DidSwitch` false)
    (else
      (`ActorComponent.Activate` (`self.Audio`) false)
      (`ActorComponent.Activate` (`self.Fire`) false)
      (`SceneComponent.SetVisibility` (`self.TorchLightStatic`) true false)
      (set `self.DidSwitch` true))))

(fn `UserConstructionScript`)