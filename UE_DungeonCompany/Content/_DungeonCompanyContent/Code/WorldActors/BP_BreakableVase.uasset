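; Breakable vase world actor that shatters and drops loot when its Hit event receives the pitchfork weapon class.
; Hit calls Shatter, then spawns every class in ItemPool just above the actor's root.
; Shatter swaps the intact mesh for pre-placed shard and lid components, enabling physics and applying the scaled hit impulse.
; The debris components are destroyed after a short delay, while the actor itself is not destroyed.
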(event `self.ReceiveTick`
  (params (DeltaSeconds :type "Float (single-precision)")))

(event `self.ReceiveBeginPlay`)

(event `self.Hit`
  (params (ImpulseDirection :type "Vector Structure") (WeaponClass :type "Weapon Class Reference"))
  (if (== WeaponClass "/Game/_DungeonCompanyContent/Code/Items/Weapons/PitchFork/BP_Pitchfork_World.BP_Pitchfork_World_C")
    (`self.Shatter` ImpulseDirection)
    (for _array_element (`self.ItemPool`)
      (`|SpawnActorFromClass` _array_element (`KismetMathLibrary.MakeTransform` (+ (`SceneComponent.K2_GetComponentLocation` (`self.DefaultSceneRoot`)) (0.0 0.0 20.0))) "Undefined" "MultiplyWithRoot" null null))))

(event `Shatter`
  (params (Impulse :type "Vector Structure"))
  (bind _shatteredvase_4 (`self.ShatteredVase_4`))
  (`|ExecutionSequence`
    (:`then_0`
      (`|ExecutionSequence`
        (:`then_0`
          (`ActorComponent.K2_DestroyComponent` (`self.vase_LP`)))
        (:`then_1`
          (`SceneComponent.SetVisibility` (`self.ShatteredVase_1`) true false)
          (`SceneComponent.SetVisibility` _shatteredvase_4 true false)
          (`SceneComponent.SetVisibility` (`self.ShatteredVase_2`) true false)
          (`SceneComponent.SetVisibility` (`self.vase_LP_Lid`) true false)
          (`SceneComponent.SetVisibility` (`self.ShatteredVase_3`) true false)
          (`PrimitiveComponent.SetSimulatePhysics` _shatteredvase_4 true)
          (`PrimitiveComponent.SetSimulatePhysics` (`self.ShatteredVase_1`) true)
          (`PrimitiveComponent.SetSimulatePhysics` (`self.ShatteredVase_2`) true)
          (`PrimitiveComponent.SetSimulatePhysics` (`self.vase_LP_Lid`) true)
          (`PrimitiveComponent.SetSimulatePhysics` (`self.ShatteredVase_3`) true)
          (`PrimitiveComponent.AddImpulse` _shatteredvase_4 (* Impulse (`self.ImpuleStrenght`)) "None" false)
          (`PrimitiveComponent.AddImpulse` (`self.ShatteredVase_1`) (* Impulse (`self.ImpuleStrenght`)) "None" false)
          (`PrimitiveComponent.AddImpulse` (`self.ShatteredVase_2`) (* Impulse (`self.ImpuleStrenght`)) "None" false)
          (`PrimitiveComponent.AddImpulse` (`self.vase_LP_Lid`) (* Impulse (`self.ImpuleStrenght`)) "None" false)
          (`PrimitiveComponent.AddImpulse` (`self.ShatteredVase_3`) (* Impulse (`self.ImpuleStrenght`)) "None" false))))
    (:`then_1`
      (`KismetSystemLibrary.Delay` 5.0)
      (`ActorComponent.K2_DestroyComponent` (`self.ShatteredVase_3`))
      (`ActorComponent.K2_DestroyComponent` (`self.ShatteredVase_4`))
      (`ActorComponent.K2_DestroyComponent` (`self.ShatteredVase_1`))
      (`ActorComponent.K2_DestroyComponent` (`self.ShatteredVase_2`))
      (`ActorComponent.K2_DestroyComponent` (`self.vase_LP_Lid`)))))

(fn `UserConstructionScript`)