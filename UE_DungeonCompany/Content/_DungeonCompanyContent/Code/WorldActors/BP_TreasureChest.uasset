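; Treasure chest world actor that plays its opening animation and lights up when a player interacts with it.
; The server interaction event calls Open, which plays the skeletal mesh animation and disables the box collision.
; After a short delay it reveals a shine component with a dynamic material instance.
; A timeline then drives that material's brightness and the point light's intensity together.
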(event `self.ReceiveBeginPlay`)

(event `self.OnInteractedOnServer`
  (`self.Open`))

(event `Open`
  (`SkeletalMeshComponent.PlayAnimation` (`self.SK_treasureChest`) "/Game/_DungeonCompanyContent/Assets/WorldActors/TreasureChest/SK_treasureChest_Open_Anim.SK_treasureChest_Open_Anim" false)
  (`self.ShineUp`))

(event `ShineUp`
  (`PrimitiveComponent.SetCollisionEnabled` (`self.Box`) "NoCollision")
  (`KismetSystemLibrary.Delay` 0.5)
  (`SceneComponent.SetVisibility` (`self.TreasureChestShine`) true false)
  (bind _returnvalue (`KismetMaterialLibrary.CreateDynamicMaterialInstance` "/Game/_DungeonCompanyContent/Assets/WorldActors/TreasureChest/Shine/M_TreasureShine.M_TreasureShine"))
  (`PrimitiveComponent.SetMaterial` (`self.TreasureChestShine`) 0 _returnvalue)
  (bind (_direction _010) (`Timeline|Timeline` :!via `PlayFromStart`)
    (:`Update`
      (`MaterialInstanceDynamic.SetScalarParameterValue` _returnvalue "Brightness" _010)
      (`LightComponent.SetIntensity` (`self.PointLight`) (* _010 5000.0)))))

(fn `UserConstructionScript`)