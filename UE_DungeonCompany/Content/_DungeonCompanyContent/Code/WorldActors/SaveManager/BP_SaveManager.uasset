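; Server-side save manager that persists and restores world state: item spawners, treasure chests, loose world items and breakable props.
; SaveGame gathers each category on separate ticks into BP_DC_SaveGame, skipping spawner-originated items, held items and backpacks, then writes the slot.
; LoadSave async-loads the game instance's current slot and restores one element per tick via the IterateOverTime macro, counting progress for the loading screen.
; Without an existing save, it creates and saves one first.
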(event `LoadingDone`
  (`Widget.RemoveFromParent` (`self.Loading Screen`)))

(event `LoadSave` :!signature `self.SavingDone`
  (params (`Loading Screen` :type "/Game/_DungeonCompanyContent/Code/UI/WBP_LoadingScreen Object Reference"))
  ;[0.9279 1 0.2531] Load
  (set `self.Loading Screen` `Loading Screen`)
  (`/Engine/EditorBlueprintResources/ActorMacros.Switch Has Authority`
    (:`Authority`
      (bind _asbp_dc_gi (cast `/Game/_DungeonCompanyContent/Code/DCGame/BP_DC_GI` (`GameplayStatics.GetGameInstance`))
        (:`then`
          (bind _output_get (set `self.Current Save GameName` (`/Game/_DungeonCompanyContent/Code/DCGame/BP_DC_GI.CurrentSaveGame` _asbp_dc_gi)))
          (bind _savegame (`AsyncActionHandleSaveGame.AsyncLoadGameFromSlot` _output_get)
            (:`Completed`
              (bind _asbp_dc_save_game (cast `/Game/_DungeonCompanyContent/Code/SaveSystem/BP_DC_SaveGame` _savegame)
                (:`then`
                  (set `self.Save Game Object` _asbp_dc_save_game)
                  (`|ExecutionSequence`
                    (:`then_0`
                      (set `/Game/_DungeonCompanyContent/Code/UI/WBP_LoadingScreen.ActionsToLoad` (`/Game/_DungeonCompanyContent/Code/SaveSystem/BP_DC_SaveGame.ActionsToLoad` (`self.Save Game Object`)) (`self.Loading Screen`)))
                    (:`then_1`
                      ;;[1 1 1] Load Item Spawners
                      (for _array_element (`/Game/_DungeonCompanyContent/Code/SaveSystem/BP_DC_SaveGame.ItemSpawners` (`self.Save Game Object`))
                        (bind (_spawner _itempickedup) (break `/Game/_DungeonCompanyContent/Code/SaveSystem/ItemSpawners_SaveData` _array_element))
                        (set `/Game/_DungeonCompanyContent/Code/WorldActors/BP_ItemSpawner.ItemPickedUp` _itempickedup _spawner))
                      (bind _outactors (`GameplayStatics.GetAllActorsOfClass` "/Game/_DungeonCompanyContent/Code/WorldActors/BP_ItemSpawner.BP_ItemSpawner_C"))
                      (bind _item (`self.IterateOverTime` _outactors)
                        (:`Execute`
                          (`/Game/_DungeonCompanyContent/Code/WorldActors/BP_ItemSpawner.SpawnMyItem` _item)
                          (`/Engine/EditorBlueprintResources/StandardMacros.IncrementInt` (`self.ActionsLoaded`)))
                        (:`End`
                          ;;[1 1 1] Load Chests
                          (bind _item_2 (`self.IterateOverTime` (`/Game/_DungeonCompanyContent/Code/SaveSystem/BP_DC_SaveGame.Chests` (`self.Save Game Object`)))
                            (:`Execute`
                              (`/Engine/EditorBlueprintResources/StandardMacros.IncrementInt` (`self.ActionsLoaded`)
                                (:`  `
                                  (bind (_chest _used) (break `/Game/_DungeonCompanyContent/Code/SaveSystem/Chests_SaveData` _item_2))
                                  (bind _output_get_2 (set `/Game/_DungeonCompanyContent/Code/WorldActors/TreasureChest/BP_TreasureChest.Used` _used _chest))
                                  (if _output_get_2
                                    (`/Game/_DungeonCompanyContent/Code/WorldActors/TreasureChest/BP_TreasureChest.DeactivateOnStart` _chest)))))
                            (:`End`
                              ;;[1 1 1] Load World Iems
                              (bind _item_3 (`self.IterateOverTime` (`/Game/_DungeonCompanyContent/Code/SaveSystem/BP_DC_SaveGame.WorldItems` (`self.Save Game Object`)))
                                (:`Execute`
                                  (bind (_worlditem _transform _stringdata) (break `/Game/_DungeonCompanyContent/Code/SaveSystem/WorldItems_SaveData` _item_3))
                                  (`self.SpawnWorldItem` _worlditem _transform _stringdata)
                                  (`/Engine/EditorBlueprintResources/StandardMacros.IncrementInt` (`self.ActionsLoaded`)))
                                (:`End`
                                  ;;[1 1 1] Load Breakables
                                  (bind _item_4 (`self.IterateOverTime` (`/Game/_DungeonCompanyContent/Code/SaveSystem/BP_DC_SaveGame.Breakables` (`self.Save Game Object`)))
                                    (:`Execute`
                                      (bind _output_get_3 (set `BreakableProp.bIsBroken` (`.Broken_7_8A84946C4BE5F50D5A08949F42BA1D30` (break `/Game/_DungeonCompanyContent/Code/SaveSystem/Breakables_SaveData` _item_4)) (break `/Game/_DungeonCompanyContent/Code/SaveSystem/Breakables_SaveData` _item_4)))
                                      (`/Engine/EditorBlueprintResources/StandardMacros.IncrementInt` (`self.ActionsLoaded`)
                                        (:`  `
                                          (if _output_get_3
                                            (`BreakableProp.SetBrokenState` (break `/Game/_DungeonCompanyContent/Code/SaveSystem/Breakables_SaveData` _item_4))))))
                                    (:`End`
                                      (`self.LoadingDone`))))))))))))
                (:`CastFailed`
                  (bind _returnvalue (`GameplayStatics.CreateSaveGameObject` "/Game/_DungeonCompanyContent/Code/SaveSystem/BP_DC_SaveGame.BP_DC_SaveGame_C")) ; saves once because otherwise items will not be spawned
                  (set `self.Save Game Object` _returnvalue)
                  (`self.SaveGame`)
                  (add `self.SavingDone` (`|CreateDelegate` :!event `LoadSave`)))))))
        (:`CastFailed`
          (`KismetSystemLibrary.PrintString` "wrong game instance \nExpected: BP_DC_GI"))))))

(event `SaveGame`
  ;[0.4352 0.486 1] Save
  (set `self.ActionsSaved` 0)
  (`self.SaveItemSpawners`)
  (`KismetSystemLibrary.DelayUntilNextTick`)
  (`self.SaveChests`)
  (`KismetSystemLibrary.DelayUntilNextTick`)
  (`self.SaveItems`)
  (`KismetSystemLibrary.DelayUntilNextTick`)
  (`self.SaveBreakables`)
  (`KismetSystemLibrary.DelayUntilNextTick`)
  (`self.FinalizeSave`))

(event `FinalizeSave`
  ;[0.4352 0.486 1] Save
  (`KismetSystemLibrary.PrintString` "Finalizing Save")
  (set `/Game/_DungeonCompanyContent/Code/SaveSystem/BP_DC_SaveGame.ActionsToLoad` (`self.ActionsSaved`) (`self.Save Game Object`))
  (bind _returnvalue (`GameplayStatics.SaveGameToSlot` (`self.Save Game Object`) (`self.Current Save GameName`)))
  (if _returnvalue
    (`self.SavingDone` (`self.Loading Screen`))
    (clear `self.SavingDone`)
    (else
      (`KismetSystemLibrary.PrintString` "ErrorWhileSaving"))))

(fn `SaveBreakables`
  (`KismetSystemLibrary.PrintString` "Saving breakables")
  (`KismetArrayLibrary.Array_Clear` (`/Game/_DungeonCompanyContent/Code/SaveSystem/BP_DC_SaveGame.Breakables` (`self.Save Game Object`)))
  (bind _outactors (`GameplayStatics.GetAllActorsOfClass` "/Script/UE_DungeonCompany.BreakableProp"))
  (for _array_element _outactors
    (`KismetArrayLibrary.Array_Add` (`/Game/_DungeonCompanyContent/Code/SaveSystem/BP_DC_SaveGame.Breakables` (`self.Save Game Object`)) (make `/Game/_DungeonCompanyContent/Code/SaveSystem/Breakables_SaveData` _array_element (`BreakableProp.bIsBroken` _array_element)))
    (`/Engine/EditorBlueprintResources/StandardMacros.IncrementInt` (`self.ActionsSaved`))))

(fn `SaveChests`
  (`KismetSystemLibrary.PrintString` "Saving Chests")
  (`KismetArrayLibrary.Array_Clear` (`/Game/_DungeonCompanyContent/Code/SaveSystem/BP_DC_SaveGame.Chests` (`self.Save Game Object`)))
  (bind _outactors (`GameplayStatics.GetAllActorsOfClass` "/Game/_DungeonCompanyContent/Code/WorldActors/TreasureChest/BP_TreasureChest.BP_TreasureChest_C"))
  (for _array_element _outactors
    (`KismetArrayLibrary.Array_Add` (`/Game/_DungeonCompanyContent/Code/SaveSystem/BP_DC_SaveGame.Chests` (`self.Save Game Object`)) (make `/Game/_DungeonCompanyContent/Code/SaveSystem/Chests_SaveData` _array_element (`/Game/_DungeonCompanyContent/Code/WorldActors/TreasureChest/BP_TreasureChest.Used` _array_element)))
    (`/Engine/EditorBlueprintResources/StandardMacros.IncrementInt` (`self.ActionsSaved`))))

(fn `SaveItems`
  (`KismetSystemLibrary.PrintString` "Saving Items")
  (`KismetArrayLibrary.Array_Clear` (`/Game/_DungeonCompanyContent/Code/SaveSystem/BP_DC_SaveGame.WorldItems` (`self.Save Game Object`)))
  (bind _outactors (`GameplayStatics.GetAllActorsOfClass` "/Script/UE_DungeonCompany.WorldItem"))
  (for _array_element _outactors
    (if (and (not (`WorldItem.bCameFromItemSpawner` _array_element)) (not (`GameplayStatics.ObjectIsA` _array_element "/Game/_DungeonCompanyContent/Code/Items/BackPack/BP_Backpack_World.BP_Backpack_World_C")) (not (`WorldItem.bIsHeldByPlayer` _array_element)))
      (`KismetArrayLibrary.Array_Add` (`/Game/_DungeonCompanyContent/Code/SaveSystem/BP_DC_SaveGame.WorldItems` (`self.Save Game Object`)) (make `/Game/_DungeonCompanyContent/Code/SaveSystem/WorldItems_SaveData` (`GameplayStatics.GetObjectClass` _array_element) (`self.GetTransform` _array_element) (`ItemData.SerializeMyData` (`WorldItem.MyData` _array_element))))
      (`/Engine/EditorBlueprintResources/StandardMacros.IncrementInt` (`self.ActionsSaved`)))))

(fn `SaveItemSpawners`
  (`KismetSystemLibrary.PrintString` "Saving Item Spawners")
  (`KismetArrayLibrary.Array_Clear` (`/Game/_DungeonCompanyContent/Code/SaveSystem/BP_DC_SaveGame.ItemSpawners` (`self.Save Game Object`)))
  (bind _outactors (`GameplayStatics.GetAllActorsOfClass` "/Game/_DungeonCompanyContent/Code/WorldActors/BP_ItemSpawner.BP_ItemSpawner_C"))
  (for _array_element _outactors
    (`KismetArrayLibrary.Array_Add` (`/Game/_DungeonCompanyContent/Code/SaveSystem/BP_DC_SaveGame.ItemSpawners` (`self.Save Game Object`)) (make `/Game/_DungeonCompanyContent/Code/SaveSystem/ItemSpawners_SaveData` _array_element (`/Game/_DungeonCompanyContent/Code/WorldActors/BP_ItemSpawner.ItemPickedUp` _array_element)))
    (`/Engine/EditorBlueprintResources/StandardMacros.IncrementInt` (`self.ActionsSaved`))))

(fn `UserConstructionScript`)