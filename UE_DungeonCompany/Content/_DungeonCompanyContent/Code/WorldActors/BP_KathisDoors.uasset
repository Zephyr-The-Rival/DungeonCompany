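; Two-lever puzzle door actor that opens a pair of doors when both externally assigned levers are set.
; On BeginPlay it binds to each lever's button-press event; each press stores that lever's state, triggers its feedback and runs a shared check.
; Solving instantly shifts the doors vertically in opposite directions, and a failed check after solving reverses the shift.
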(event `CustomEvent_1`
  (params (InteractingPawn :type "Pawn Object Reference"))
  (bind _doorleft (`self.DoorLeft`))
  (bind _doorright (`self.DoorRight`))
  (bind _lever2 (`self.Lever2`))
  (bind _doorleft_2 (`self.DoorLeft`))
  (bind _doorright_2 (`self.DoorRight`))
  (bind (_returnvalue_x _returnvalue_y _returnvalue_z) (`KismetMathLibrary.BreakVector` (`SceneComponent.K2_GetComponentLocation` _doorright_2)))
  (bind (_returnvalue_x_2 _returnvalue_y_2 _returnvalue_z_2) (`KismetMathLibrary.BreakVector` (`SceneComponent.K2_GetComponentLocation` _doorright)))
  (bind (_returnvalue_x_3 _returnvalue_y_3 _returnvalue_z_3) (`KismetMathLibrary.BreakVector` (`SceneComponent.K2_GetComponentLocation` _doorleft_2)))
  (bind (_returnvalue_x_4 _returnvalue_y_4 _returnvalue_z_4) (`KismetMathLibrary.BreakVector` (`SceneComponent.K2_GetComponentLocation` _doorleft)))
  (bind _ispressed (`/Game/_DungeonCompanyContent/Code/WorldActors/BP_KathisLever.LeverSet` _lever2))
  (`/Game/_DungeonCompanyContent/Code/WorldActors/BP_KathisLever.Lever Feedback` _lever2)
  (if (and (stale `CustomEvent` _ispressed) _ispressed) :!label _label
    (`KismetSystemLibrary.PrintString` "Puzzle Solved!")
    (set `self.PuzzleSolved` true)
    (`|ExecutionSequence`
      (:`then_0`
        (`SceneComponent.K2_SetWorldTransform` _doorleft_2 (`KismetMathLibrary.MakeTransform` (`KismetMathLibrary.MakeVector` _returnvalue_x_3 _returnvalue_y_3 (- _returnvalue_z_3 400.0)) (`SceneComponent.K2_GetComponentRotation` _doorleft_2) (`SceneComponent.K2_GetComponentScale` _doorleft_2)) false false))
      (:`then_1`
        (`SceneComponent.K2_SetWorldTransform` _doorright_2 (`KismetMathLibrary.MakeTransform` (`KismetMathLibrary.MakeVector` _returnvalue_x _returnvalue_y (+ _returnvalue_z 400.0)) (`SceneComponent.K2_GetComponentRotation` _doorright_2) (`SceneComponent.K2_GetComponentScale` _doorright_2)) false false)))
    (elif (`self.PuzzleSolved`)
      (`KismetSystemLibrary.PrintString` "Doors Closing")
      (`|ExecutionSequence`
        (:`then_0`
          (`SceneComponent.K2_SetWorldTransform` _doorleft (`KismetMathLibrary.MakeTransform` (`KismetMathLibrary.MakeVector` _returnvalue_x_4 _returnvalue_y_4 (+ _returnvalue_z_4 400.0)) (`SceneComponent.K2_GetComponentRotation` _doorleft) (`SceneComponent.K2_GetComponentScale` _doorleft)) false false))
        (:`then_1`
          (`SceneComponent.K2_SetWorldTransform` _doorright (`KismetMathLibrary.MakeTransform` (`KismetMathLibrary.MakeVector` _returnvalue_x_2 _returnvalue_y_2 (- _returnvalue_z_2 400.0)) (`SceneComponent.K2_GetComponentRotation` _doorright) (`SceneComponent.K2_GetComponentScale` _doorright)) false false))
        (:`then_2`
          (set `self.PuzzleSolved` false))))))

(event `CustomEvent`
  (params (InteractingPawn :type "Pawn Object Reference"))
  (bind _lever1 (`self.Lever1`))
  (`|ExecutionSequence`
    (:`then_0`
      (bind _ispressed (`/Game/_DungeonCompanyContent/Code/WorldActors/BP_KathisLever.LeverSet` _lever1))
      (`/Game/_DungeonCompanyContent/Code/WorldActors/BP_KathisLever.Lever Feedback` _lever1))
    (:`then_1`
      (goto _label))))

(event `self.ReceiveBeginPlay`
  (`/Engine/EditorBlueprintResources/StandardMacros.IsValid` (`self.Lever1`)
    (:`Is Valid`
      (`/Engine/EditorBlueprintResources/StandardMacros.IsValid` (`self.Lever2`)
        (:`Is Valid`
          (add `BasicButton.OnButtonPressed` (`self.Lever2`) (delegate `CustomEvent_1`))
          (add `BasicButton.OnButtonPressed` (`self.Lever1`) (delegate `CustomEvent`)))
        (:`Is Not Valid`
          (`KismetSystemLibrary.PrintString` "Lever 2 was not valid \nBind in Outliner"))))
    (:`Is Not Valid`
      (`KismetSystemLibrary.PrintString` "Lever 1 was not valid \nBind in Outliner"))))

(fn `UserConstructionScript`)