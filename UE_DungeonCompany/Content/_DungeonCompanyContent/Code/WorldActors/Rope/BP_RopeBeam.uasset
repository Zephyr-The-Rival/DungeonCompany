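; BP_RopeBeam is a world actor that draws a vertical rope as a stretched plane up to a linked rope end actor.
; GenerateRope runs in construction and every tick, scaling the plane's Z by the height difference to MyRopeEnd, compensated for root scale.
; It then yaws the plane from the local player's first-person camera direction, billboarding it around the vertical axis.
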(event `self.ReceiveTick`
  (params (DeltaSeconds :type "Float (single-precision)"))
  (`self.GenerateRope`))

(event `GenerateRope`
  (bind _plane (`self.Plane`))
  (bind (_returnvalue_roll _returnvalue_pitch) (`KismetMathLibrary.BreakRotator` (`SceneComponent.K2_GetComponentRotation` _plane)))
  (bind (_returnvalue_x _returnvalue_y _returnvalue_z) (`KismetMathLibrary.BreakVector` (`SceneComponent.K2_GetComponentScale` (`self.DefaultSceneRoot`))))
  (`/Engine/EditorBlueprintResources/StandardMacros.IsValid` (`self.MyRopeEnd`)
    (:`Is Valid`
      (bind _output_get (set `self.RopeLenght` (- (.z (`SceneComponent.K2_GetComponentLocation` (`/Game/_DungeonCompanyContent/Code/WorldActors/Rope/BP_RopeEnd.DefaultSceneRoot` (`self.MyRopeEnd`)))) (.z (`SceneComponent.K2_GetComponentLocation` (`self.DefaultSceneRoot`))))))
      (`SceneComponent.SetRelativeScale3D` (`self.Plane`) (`KismetMathLibrary.MakeVector` 1.0 1.0 (/ (* _output_get (/ 1.0 _returnvalue_z)) 100.0)))
      (bind _asplayer_character (cast `PlayerCharacter` (`Controller.K2_GetPawn` (`GameplayStatics.GetPlayerController` 0))))
      (bind (_returnvalue_roll_2 _returnvalue_pitch_2 _returnvalue_yaw) (`KismetMathLibrary.BreakRotator` (`KismetMathLibrary.FindLookAtRotation` (`SceneComponent.K2_GetComponentLocation` (`PlayerCharacter.FirstPersonCamera` _asplayer_character)) (`SceneComponent.K2_GetComponentLocation` (`self.Plane`)))))
      (`SceneComponent.K2_SetWorldRotation` _plane (`KismetMathLibrary.MakeRotator` _returnvalue_roll _returnvalue_pitch _returnvalue_yaw) false false))))

(fn `UserConstructionScript`
  (`/Engine/EditorBlueprintResources/StandardMacros.IsValid` (`self.MyRopeEnd`)
    (:`Is Valid`
      (`self.GenerateRope`))))