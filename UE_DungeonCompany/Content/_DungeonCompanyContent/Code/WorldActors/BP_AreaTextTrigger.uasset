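; BP_AreaTextTrigger is a world trigger that announces an area name on the player's HUD when a player character enters it.
; On overlap it reaches the player's BP_PlayerHud and calls AnnounceNewArea, skipping the call if the HUD's area text already shows that name.
; The construction script writes AreaName into a text render component and resets its world scale to one, so the label stays unscaled.
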(event `self.ReceiveActorBeginOverlap`
  (params (OtherActor :type "Actor Object Reference"))
  (bind _asplayer_character (cast `PlayerCharacter` OtherActor))
  (bind _asbp_player_hud (cast `/Game/_DungeonCompanyContent/Code/UI/PlayerHud/BP_PlayerHud` (`PlayerCharacter.GetMyHud` _asplayer_character)))
  (if (not (`KismetStringLibrary.EqualEqual_StrStr` (`KismetTextLibrary.Conv_TextToString` (`TextBlock.Text` (`/Game/_DungeonCompanyContent/Code/UI/PlayerHud/BP_PlayerHud.AreaNameText` _asbp_player_hud))) (`self.AreaName`)))
    (`/Game/_DungeonCompanyContent/Code/UI/PlayerHud/BP_PlayerHud.AnnounceNewArea` _asbp_player_hud (`self.AreaName`))))

(fn `UserConstructionScript`
  (bind _textrender (`self.TextRender`))
  (`TextRenderComponent.K2_SetText` _textrender (`KismetTextLibrary.Conv_StringToText` (`self.AreaName`)))
  (`SceneComponent.SetWorldScale3D` _textrender (1.0 1.0 1.0)))