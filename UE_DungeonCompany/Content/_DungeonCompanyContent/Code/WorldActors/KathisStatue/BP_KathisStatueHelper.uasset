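; Helper actor that drives the Kathi statue's reaction to button presses.
; On BeginPlay it binds to the referenced Statue's button-pressed event, or prints a warning if none is assigned in the level.
; The first press makes the statue stand up and sets a one-shot flag; later presses only print a placeholder "add crystal" message.
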(event `CustomEvent_1`
  (params (InteractingPawn :type "Pawn Object Reference"))
  (if (`self.DidPress`)
    (`KismetSystemLibrary.PrintString` "add crystal")
    (else
      (`/Game/_DungeonCompanyContent/Code/WorldActors/KathisStatue/BP_KathisStatue.Stand Up` (`self.Statue`))
      (set `self.DidPress` true))))

(event `self.ReceiveBeginPlay`
  (`/Engine/EditorBlueprintResources/StandardMacros.IsValid` (`self.Statue`)
    (:`Is Valid`
      (add `BasicButton.OnButtonPressed` (`self.Statue`) (delegate `CustomEvent_1`)))
    (:`Is Not Valid`
      (`KismetSystemLibrary.PrintString` "Statue was not valid \nBind in Outliner"))))

(fn `UserConstructionScript`)