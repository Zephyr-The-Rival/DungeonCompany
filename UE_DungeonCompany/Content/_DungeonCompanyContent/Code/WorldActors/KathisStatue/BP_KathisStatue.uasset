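; BP_KathisStatue is a statue world actor that can be switched to an upright pose through its Stand Up function.
; Stand Up applies fixed offsets to the StaticMesh's current relative roll, pitch and location in one instant step, with no interpolation.
; Each call stacks on the last, as nothing guards against repeats.
; The event graph and construction script are empty, so the file itself never calls the function.
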(fn `Stand Up`
  (locals (NewLocalVar :type "Array of Float (single-precision)"))
  (bind _staticmesh (`self.StaticMesh`))
  (bind (_relativelocation_x _relativelocation_y _relativelocation_z) (`KismetMathLibrary.BreakVector` (`SceneComponent.RelativeLocation` _staticmesh)))
  (bind (_relativerotation_roll _relativerotation_pitch _relativerotation_yaw) (`KismetMathLibrary.BreakRotator` (`SceneComponent.RelativeRotation` _staticmesh)))
  (`|ExecutionSequence`
    (:`then_0`
      (`SceneComponent.K2_SetRelativeRotation` _staticmesh (`KismetMathLibrary.MakeRotator` (- _relativerotation_roll 25.0) (- _relativerotation_pitch 95.0) _relativerotation_yaw) false false))
    (:`then_1`
      (`SceneComponent.K2_SetRelativeLocation` _staticmesh (`KismetMathLibrary.MakeVector` (- _relativelocation_x 50.0) (- _relativelocation_y 80.0) (+ _relativelocation_z 150.0)) false false))))

(fn `UserConstructionScript`)