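; Floor puzzle actor for Kathi's statue: a statue is stood up to unlock an item socket, and the floor can move as a platform.
; Pressing the standup button snaps Statue4 into a new pose, destroys the button and enables query collision on the socket's child actor.
; MovePlatform, not called here, reveals a crystal and light, destroys pillars, plays platform-down audio and adds a timeline-driven Z offset each update.
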(event `self.ReceiveBeginPlay`
  (add `BasicButton.OnButtonPressed` (`self.StatueStandupButton`) (delegate `StandupStatue`)))

(event `StandupStatue`
  (params (InteractingPawn :type "Pawn Object Reference"))
  (bind _statue4 (`self.Statue4`))
  (bind (_returnvalue_x _returnvalue_y _returnvalue_z) (`KismetMathLibrary.BreakVector` (`SceneComponent.K2_GetComponentLocation` _statue4)))
  (bind (_relativerotation_roll _relativerotation_pitch _relativerotation_yaw) (`KismetMathLibrary.BreakRotator` (`SceneComponent.RelativeRotation` _statue4)))
  (`|ExecutionSequence`
    (:`then_0`
      (`|ExecutionSequence`
        (:`then_0`
          (`SceneComponent.K2_SetWorldRotation` (`self.Statue4`) (`KismetMathLibrary.MakeRotator` 0.0 (- _relativerotation_pitch 20.0) (- _relativerotation_yaw 5.0)) false false))
        (:`then_1`
          (`SceneComponent.K2_SetWorldLocation` (`self.Statue4`) (`KismetMathLibrary.MakeVector` _returnvalue_x (+ _returnvalue_y 140.0) (- _returnvalue_z 75.0)) false false))))
    (:`then_1`
      (`self.K2_DestroyActor` (`self.StatueStandupButton`))
      (bind _asbp_item_socket_interact (cast `/Game/_DungeonCompanyContent/Code/WorldActors/KathisStatue/BP_ItemSocketInteract` (`ChildActorComponent.ChildActor` (`self.ItemSocket`))))
      (`PrimitiveComponent.SetCollisionEnabled` (`/Game/_DungeonCompanyContent/Code/WorldActors/KathisStatue/BP_ItemSocketInteract.BoxCollision` _asbp_item_socket_interact) "QueryOnly"))))

(event `MovePlatform`
  (`|ExecutionSequence`
    (:`then_0`
      (`SceneComponent.SetVisibility` (`self.PointLight3`) true false)
      (`SceneComponent.SetVisibility` (`self.Crystal4`) true false))
    (:`then_1`
      (`self.K2_DestroyActor` (`self.PillarsToDelete`)))
    (:`then_2`
      (bind (_direction _newtrack_0) (`Timeline|Timeline`)
        (:`Update`
          (`SceneComponent.K2_AddWorldOffset` (`self.FloorMesh`) (`KismetMathLibrary.MakeVector` 0.0 0.0 _newtrack_0) false false))))
    (:`then_3`
      (`AudioComponent.Play` (`self.MS_PlatformDown`) 0.0))))

(fn `UserConstructionScript`)