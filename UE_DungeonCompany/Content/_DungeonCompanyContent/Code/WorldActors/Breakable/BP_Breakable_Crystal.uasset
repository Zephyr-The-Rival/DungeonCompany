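; Breakable mana crystal node that only shatters when hit with a pickaxe; other tools just print a message.
; A server hit marks it broken, multicasts Shatter for sound and Niagara effects, and spawns mana crystal pickups launched by a random upward impulse.
; The SetBrokenState override swaps to the mined mesh while a timeline fades the point light and dynamic material glow.
; LocalReset restores the intact crystal and light on dungeon reset.
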(event `self.ReceiveBeginPlay`
  (`parent.ReceiveBeginPlay`)
  (`|ExecutionSequence`
    (:`then_0`
      (bind _object (`|LoadAsset` "/Game/_DungeonCompanyContent/Audio/WorldActors/HitNodeWithPickaxe.HitNodeWithPickaxe")
        (:`Completed`
          (bind _assound_base (cast `SoundBase` _object))
          (set `self.ShatterSound` _assound_base))))
    (:`then_1`
      (bind _returnvalue (`KismetMaterialLibrary.CreateDynamicMaterialInstance` "/Game/_DungeonCompanyContent/Assets/MKMine/Crystal_Node/MI_CrystalNodeBroken.MI_CrystalNodeBroken"))
      (bind _output_get (set `self.BrokenMaterial` _returnvalue))
      (`PrimitiveComponent.SetMaterial` (`self.Mined`) 0 _output_get)
      (set `self.LightOriginalIntensity` (`LightComponentBase.Intensity` (`self.PointLight`))))))

(event `self.Hit`
  (params (ImpulseDirection :type "Vector Structure") (WeaponClass :type "Weapon Class Reference"))
  (bind _returnvalue (`KismetMathLibrary.RandomFloatInRange` 0.0 1.0))
  ;[1 0.4192 0] OnServer
  ; Hit
  (if (== WeaponClass "/Game/_DungeonCompanyContent/Code/Items/Weapons/Pickaxe/BP_Pickaxe_World.BP_Pickaxe_World_C")
    (`self.Shatter` ImpulseDirection)
    (set `self.bIsBroken` true :!pinned true) ; DONT FORGET ME!!!!
    (for _ (range 2)
      (bind _returnvalue_2 (`|SpawnActorFromClass` "/Game/_DungeonCompanyContent/Code/Items/ManaCrystal/BP_ManaCrystal_World.BP_ManaCrystal_World_C" (`KismetMathLibrary.MakeTransform` (+ (`SceneComponent.K2_GetComponentLocation` (`self.Mined`)) (0.0 0.0 45.0)) (`KismetMathLibrary.RandomRotator` true)) "Undefined" "MultiplyWithRoot" null null))
      (`PrimitiveComponent.AddImpulse` (`/Game/_DungeonCompanyContent/Code/Items/ManaCrystal/BP_ManaCrystal_World.Mesh` _returnvalue_2) (* (`KismetMathLibrary.MakeVector` _returnvalue _returnvalue 2.0) (`self.ImpulseStrenght`)) "None" false))
    (else
      (`KismetSystemLibrary.PrintString` "DING! Wrong Tool"))))

(event `Shatter`
  (params (Impulse :type "Vector Structure"))
  ;[0.6869 0.2143 1] Multicast
  ; Shatter
  (`GameplayStatics.PlaySoundAtLocation` (`self.ShatterSound`) (`SceneComponent.K2_GetComponentLocation` (`self.DefaultSceneRoot`)) (struct) 1.0 1.0 0.0 null null null null)
  (`ActorComponent.Activate` (`self.Niagara`) true)
  (`self.SetBrokenState`))

(event `self.SetBrokenState`
  (bind _mined (`self.Mined`))
  (bind _crystal (`self.Crystal`))
  ;[0.2275 1 0.4275] Set Broken State override
  (`|ExecutionSequence`
    (:`then_0`
      (`SceneComponent.SetVisibility` _crystal false false)
      (`PrimitiveComponent.SetCollisionEnabled` _crystal "NoCollision"))
    (:`then_1`
      (`SceneComponent.SetVisibility` _mined true false)
      (`PrimitiveComponent.SetCollisionEnabled` _mined "QueryAndPhysics"))
    (:`then_2`
      (bind (_direction _1_to_0) (`Timeline|Timeline` :!via `PlayFromStart`)
        (:`Update`
          (`LightComponent.SetIntensity` (`self.PointLight`) (* (`self.LightOriginalIntensity`) _1_to_0))
          (`MaterialInstanceDynamic.SetScalarParameterValue` (`self.BrokenMaterial`) "Emissive brightness" (+ _1_to_0 0.1)))
        (:`Finished`
          (`SceneComponent.SetVisibility` (`self.PointLight`) false false))))))

(event `/Game/_DungeonCompanyContent/Code/WorldActors/DungeonReset/BP_Resettable.LocalReset`
  (bind _crystal (`self.Crystal`))
  (bind _mined (`self.Mined`))
  ;[1 1 1] On Dungeon Reset
  (`|ExecutionSequence`
    (:`then_0`
      (`SceneComponent.SetVisibility` _crystal true false)
      (`SceneComponent.SetVisibility` (`self.PointLight`) true false)
      (`PrimitiveComponent.SetCollisionEnabled` _crystal "QueryAndPhysics")
      (`LightComponent.SetIntensity` (`self.PointLight`) (`self.LightOriginalIntensity`)))
    (:`then_1`
      (`SceneComponent.SetVisibility` _mined false false)
      (`PrimitiveComponent.SetCollisionEnabled` _mined "NoCollision"))
    (:`then_2`
      (set `self.bIsBroken` false :!pinned true) ; DONT FORGET ME!!!!
    )))

(fn `UserConstructionScript`)