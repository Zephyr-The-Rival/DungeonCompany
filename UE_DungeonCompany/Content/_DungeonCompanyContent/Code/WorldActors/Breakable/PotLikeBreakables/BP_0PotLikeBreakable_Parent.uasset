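; Parent Blueprint for breakable pot-like props that shatter when hit and can drop loot.
; On the server, Hit sets IsBroken, spawns zero to five pickups from tiered coin-chance thresholds, and calls multicast Shatter.
; Shatter swaps the whole mesh for impulsed physics shards with sound and Niagara burst, hiding them after a delay.
; Overrides restore broken or intact state, while the construction script optionally snaps the pot to the surface normal.
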(event `self.ReceiveBeginPlay`)

(event `ServerSpawnLoot`
  (bind _returnvalue (`KismetMathLibrary.RandomFloatInRange` -5.0 5.0))
  ;[1 1 1] SpawnLoot
  (bind _coinamount (`self.DropChanceCalculation`))
  (for _ (range 1 (+ _coinamount 1))
    (`|SpawnActorFromClass` "/Game/_DungeonCompanyContent/Code/Items/WorldCurrency/Coin/BP_Coin_World.BP_Coin_World_C" (`KismetMathLibrary.MakeTransform` (+ (`SceneComponent.K2_GetComponentLocation` (`self.DefaultSceneRoot`)) (0.0 0.0 20.0) (`KismetMathLibrary.MakeVector` _returnvalue _returnvalue _returnvalue)) (`KismetMathLibrary.RandomRotator` true)) "Undefined" "MultiplyWithRoot" null null)))

(event `self.Hit`
  (params (ImpulseDirection :type "Vector Structure") (WeaponClass :type "Weapon Class Reference"))
  ;[1 0.5049 0] On Server
  (`self.Shatter` ImpulseDirection)
  (set `self.bIsBroken` true :!pinned true) ; DONT FORGET ME!!!!
  (`self.ServerSpawnLoot`))

(event `Shatter`
  (params (Impulse :type "Vector Structure"))
  (bind _shattered_meshes (`self.Shattered Meshes`))
  (bind _wholemesh (`self.WholeMesh`))
  (bind _shattered_meshes_2 (`self.Shattered Meshes`))
  ;[1 0.09837 0.845] Multicast
  (`|ExecutionSequence`
    (:`then_0`
      (`|ExecutionSequence`
        (:`then_0`
          (`SceneComponent.SetVisibility` _wholemesh false false)
          (`PrimitiveComponent.SetCollisionEnabled` _wholemesh "NoCollision"))
        (:`then_1`
          (`SceneComponent.SetVisibility` _shattered_meshes true false)
          (`PrimitiveComponent.SetSimulatePhysics` _shattered_meshes true)
          (`PrimitiveComponent.SetCollisionEnabled` _shattered_meshes "PhysicsOnly")
          (`PrimitiveComponent.AddImpulse` _shattered_meshes (* Impulse (`self.ImpuleStrenght`)) "None" false))
        (:`then_2`
          (`GameplayStatics.SpawnSoundAtLocation` (`self.ShatterSound`) (`SceneComponent.K2_GetComponentLocation` (`self.DefaultSceneRoot`)) (struct) 1.0 1.0 0.0 null null))
        (:`then_3`
          (`NiagaraFunctionLibrary.SpawnSystemAtLocation` "/Game/_DungeonCompanyContent/Assets/VFX/NiagaraSystem/NS_VaseBrust.NS_VaseBrust" (+ (`SceneComponent.K2_GetComponentLocation` (`self.DefaultSceneRoot`)) (0.0 0.0 50.0))))))
    (:`then_1`
      (`KismetSystemLibrary.Delay` 5.0)
      (`SceneComponent.SetVisibility` _shattered_meshes_2 false false)
      (`PrimitiveComponent.SetSimulatePhysics` _shattered_meshes_2 false)
      (`PrimitiveComponent.SetCollisionEnabled` _shattered_meshes_2 "NoCollision"))))

(event `self.SetBrokenState`
  (bind _shattered_meshes (`self.Shattered Meshes`))
  (bind _wholemesh (`self.WholeMesh`))
  ;[0.2275 1 0.4275] SetBrokenState override
  (`|ExecutionSequence`
    (:`then_0`
      (`SceneComponent.SetVisibility` _wholemesh false false)
      (`PrimitiveComponent.SetSimulatePhysics` _wholemesh false)
      (`PrimitiveComponent.SetCollisionEnabled` _wholemesh "NoCollision"))
    (:`then_1`
      (`SceneComponent.SetVisibility` _shattered_meshes false false)
      (`PrimitiveComponent.SetSimulatePhysics` _shattered_meshes false)
      (`PrimitiveComponent.SetCollisionEnabled` _shattered_meshes "NoCollision"))))

(event `self.LocalReset`
  (bind _shattered_meshes (`self.Shattered Meshes`))
  (bind _wholemesh (`self.WholeMesh`))
  (if (`self.Resets`)
    (`|ExecutionSequence`
      (:`then_0`
        (set `self.bIsBroken` false :!pinned true) ; DONT FORGET ME!!!!
      )
      (:`then_1`
        (`SceneComponent.ResetRelativeTransform` _shattered_meshes)
        (`SceneComponent.SetVisibility` _shattered_meshes false false)
        (`PrimitiveComponent.SetSimulatePhysics` _shattered_meshes false)
        (`PrimitiveComponent.SetCollisionEnabled` _shattered_meshes "NoCollision"))
      (:`then_2`
        (`SceneComponent.SetVisibility` _wholemesh true false)
        (`PrimitiveComponent.SetCollisionEnabled` _wholemesh "QueryAndPhysics")))))

(fn `DefineParts`
  (params (ShatteredMeshes :type "Array of StaticMeshComponent Object Reference"))
  (bind _output_get (set `self.Shattered Meshes` ShatteredMeshes))
  (for _array_element _output_get
    (`PrimitiveComponent.SetCollisionProfileName` _array_element "BreakableShards" true)
    (`SceneComponent.SetVisibility` _array_element false false)))

(fn `DropChanceCalculation`
  (returns (CoinAmount :type Integer))
  (locals (LuckyNumber :type "Float (double-precision)" :default 0.0))
  (set `local.LuckyNumber` (`KismetMathLibrary.RandomFloatInRange` 0.0 100.0))
  (if (< (`local.LuckyNumber`) (`self.ChanceFor1Coin`))
    (if (< (`local.LuckyNumber`) (`self.ChanceFor2Coin`))
      (if (< (`local.LuckyNumber`) (`self.ChanceFor3Coin`))
        (if (< (`local.LuckyNumber`) (`self.ChanceFor4Coin`))
          (if (< (`local.LuckyNumber`) (`self.ChanceFor5Coin`))
            (return 5)
            (else
              (return 4)))
          (else
            (return 3)))
        (else
          (return 2)))
      (else
        (return 1)))
    (else
      (return 0))))

(fn `UserConstructionScript`
  (bind _returnvalue (`SceneComponent.K2_GetComponentLocation` (`self.DefaultSceneRoot`)))
  (bind (_returnvalue_roll _returnvalue_pitch _returnvalue_yaw) (`KismetMathLibrary.BreakRotator` (`SceneComponent.K2_GetComponentRotation` (`self.WholeMesh`))))
  (if (`self.AlignWithNormal`)
    (bind (_outhit _returnvalue_2) (`KismetSystemLibrary.LineTraceSingle` (+ _returnvalue (0.0 0.0 20.0)) (- _returnvalue (0.0 0.0 20.0)) "TraceTypeQuery1" false (`|MakeArray` self :!type "Actor Object Reference") "ForOneFrame"))
    (if _returnvalue_2
      (bind (_bblockinghit _binitialoverlap _time _distance _location _impactpoint _normal) (`GameplayStatics.BreakHitResult` _outhit))
      (`SceneComponent.K2_SetWorldLocation` (`self.DefaultSceneRoot`) _location false false)
      (bind (_returnvalue_roll_2 _returnvalue_pitch_2) (`KismetMathLibrary.BreakRotator` (`KismetMathLibrary.MakeRotFromZ` _normal)))
      (`SceneComponent.K2_SetWorldRotation` (`self.DefaultSceneRoot`) (`KismetMathLibrary.MakeRotator` _returnvalue_roll_2 _returnvalue_pitch_2 _returnvalue_yaw) false false))))