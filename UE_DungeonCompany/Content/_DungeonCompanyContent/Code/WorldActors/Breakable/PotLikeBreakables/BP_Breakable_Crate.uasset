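; Breakable crate world actor that drops random loot, built on a parent breakable class.
; On BeginPlay it registers its pre-fractured mesh pieces, lid included, with the parent through DefineParts.
; Its ServerSpawnLoot override rolls each LootTable entry independently against its percentage chance, so several items can drop at once.
; Winning items spawn slightly above the crate root with small positional jitter and random rotation.
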(event `self.ReceiveBeginPlay`
  (`parent.ReceiveBeginPlay`)
  (`self.DefineParts` (`|MakeArray` (`self.FracturedCrate_Crate_Fractured10`) (`self.FracturedCrate_Crate_Fractured11`) (`self.FracturedCrate_Crate_Fractured12`) (`self.FracturedCrate_Crate_Fractured13`) (`self.FracturedCrate_Crate_Fractured15`) (`self.FracturedCrate_Crate_Fractured14`) (`self.FracturedCrate_Crate_Fractured16`) (`self.FracturedCrate_Crate_Fractured17`) (`self.FracturedCrate_Crate_Fractured18`) (`self.FracturedCrate_Lid`) (`self.FracturedCrate_Crate_Fractured8`) (`self.FracturedCrate_Crate_Fractured9`) (`self.FracturedCrate_Crate_Fractured1`) (`self.FracturedCrate_Crate_Fractured2`) (`self.FracturedCrate_Crate_Fractured7`) (`self.FracturedCrate_Crate_Fractured3`) (`self.FracturedCrate_Crate_Fractured4`) (`self.FracturedCrate_Crate_Fractured5`) (`self.FracturedCrate_Crate_Fractured6`))))

(event `self.ServerSpawnLoot`
  (bind _returnvalue (`KismetMathLibrary.RandomFloatInRange` -5.0 5.0))
  (for _array_element (`self.LootTable`)
    (bind (_itemtospawn _spawnprobability) (break `/Game/_DungeonCompanyContent/Code/WorldActors/TreasureChest/LootTableEntry` _array_element))
    (if (< (`KismetMathLibrary.RandomFloatInRange` 0.0 100.0) _spawnprobability)
      (`|SpawnActorFromClass` _itemtospawn (`KismetMathLibrary.MakeTransform` (+ (`SceneComponent.K2_GetComponentLocation` (`self.DefaultSceneRoot`)) (0.0 0.0 20.0) (`KismetMathLibrary.MakeVector` _returnvalue _returnvalue _returnvalue)) (`KismetMathLibrary.RandomRotator` true)) "Undefined" "MultiplyWithRoot" null null))))

(fn `UserConstructionScript`
  (`parent.UserConstructionScript`))