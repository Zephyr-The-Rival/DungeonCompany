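; Breakable vase world actor that shatters into physics pieces when hit and rolls a coin drop count.
; The server-side Hit event calls a multicast Shatter, which swaps the intact mesh and capsule for pre-placed shards, applies impulse, plays a sound and removes pieces after a delay.
; DropChanceCalculation checks one random roll against nested thresholds to return zero to five coins, but Hit leaves the result unused.
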(event `self.ReceiveTick`
  (params (DeltaSeconds :type "Float (single-precision)")))

(event `self.ReceiveBeginPlay`)

(event `self.Hit`
  (params (ImpulseDirection :type "Vector Structure") (WeaponClass :type "Weapon Class Reference"))
  ;[1 0.5049 0] On Server
  (`self.Shatter` ImpulseDirection)
  (`self.DropChanceCalculation`))

(event `Shatter`
  (params (Impulse :type "Vector Structure"))
  (bind _shatteredvase_4 (`self.ShatteredVase_4`))
  ;[1 0.09837 0.845] Multicast
  (`|ExecutionSequence`
    (:`then_0`
      (`|ExecutionSequence`
        (:`then_0`
          (`ActorComponent.K2_DestroyComponent` (`self.vase_LP`))
          (`ActorComponent.K2_DestroyComponent` (`self.Capsule`)))
        (:`then_1`
          (`SceneComponent.SetVisibility` (`self.ShatteredVase_1`) true false)
          (`SceneComponent.SetVisibility` _shatteredvase_4 true false)
          (`SceneComponent.SetVisibility` (`self.ShatteredVase_2`) true false)
          (`SceneComponent.SetVisibility` (`self.vase_LP_Lid`) true false)
          (`SceneComponent.SetVisibility` (`self.ShatteredVase_3`) true false)
          (`PrimitiveComponent.SetSimulatePhysics` _shatteredvase_4 true)
          (`PrimitiveComponent.SetSimulatePhysics` (`self.ShatteredVase_1`) true)
          (`PrimitiveComponent.SetSimulatePhysics` (`self.ShatteredVase_2`) true)
          (`PrimitiveComponent.SetSimulatePhysics` (`self.vase_LP_Lid`) true)
          (`PrimitiveComponent.SetSimulatePhysics` (`self.ShatteredVase_3`) true)
          (`PrimitiveComponent.AddImpulse` _shatteredvase_4 (* Impulse (`self.ImpuleStrenght`)) "None" false)
          (`PrimitiveComponent.AddImpulse` (`self.ShatteredVase_1`) (* Impulse (`self.ImpuleStrenght`)) "None" false)
          (`PrimitiveComponent.AddImpulse` (`self.ShatteredVase_2`) (* Impulse (`self.ImpuleStrenght`)) "None" false)
          (`PrimitiveComponent.AddImpulse` (`self.vase_LP_Lid`) (* Impulse (`self.ImpuleStrenght`)) "None" false)
          (`PrimitiveComponent.AddImpulse` (`self.ShatteredVase_3`) (* Impulse (`self.ImpuleStrenght`)) "None" false))
        (:`then_2`
          (`GameplayStatics.SpawnSoundAtLocation` (`self.ShatterSound`) (`SceneComponent.K2_GetComponentLocation` (`self.DefaultSceneRoot`)) (struct) 1.0 1.0 0.0 null null))))
    (:`then_1`
      (`KismetSystemLibrary.Delay` 5.0)
      (`ActorComponent.K2_DestroyComponent` (`self.ShatteredVase_3`))
      (`ActorComponent.K2_DestroyComponent` (`self.ShatteredVase_4`))
      (`ActorComponent.K2_DestroyComponent` (`self.ShatteredVase_1`))
      (`ActorComponent.K2_DestroyComponent` (`self.ShatteredVase_2`))
      (`ActorComponent.K2_DestroyComponent` (`self.vase_LP_Lid`)))))

(fn `DropChanceCalculation`
  (returns (CoinAmount :type Integer))
  (locals (LuckyNumber :type "Float (double-precision)" :default 0.0))
  (set `local.LuckyNumber` (`KismetMathLibrary.RandomFloatInRange` 0.0 100.0))
  (if (< (`local.LuckyNumber`) (`self.ChanceFor1Coin`))
    (if (< (`local.LuckyNumber`) (`self.ChanceFor2Coin`))
      (if (< (`local.LuckyNumber`) (`self.ChanceFor3Coin`))
        (if (< (`local.LuckyNumber`) (`self.ChanceFor4Coin`))
          (if (< (`local.LuckyNumber`) (`self.ChanceFor5Coin`))
            (return 5)
            (else
              (return 4)))
          (else
            (return 3)))
        (else
          (return 2)))
      (else
        (return 1)))
    (else
      (return 0))))

(fn `UserConstructionScript`)