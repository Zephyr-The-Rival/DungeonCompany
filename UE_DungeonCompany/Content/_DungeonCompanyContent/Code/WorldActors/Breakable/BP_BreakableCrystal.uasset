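; BP_BreakableCrystal is a world crystal that can be mined with a pickaxe for mana crystals.
; A server Hit event checks the weapon class, printing a debug message for any other tool.
; A pickaxe hit calls multicast Shatter, which destroys the crystal component and enables the mined remnant's visibility and collision.
; The server then spawns two mana crystal pickups above the remnant and tosses them with randomized upward impulses.
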(event `self.Hit`
  (params (ImpulseDirection :type "Vector Structure") (WeaponClass :type "Weapon Class Reference"))
  (bind _returnvalue (`KismetMathLibrary.RandomFloatInRange` 0.0 1.0))
  ;[1 0.4192 0] OnServer
  ; Hit
  (if (== WeaponClass "/Game/_DungeonCompanyContent/Code/Items/Weapons/Pickaxe/BP_Pickaxe_World.BP_Pickaxe_World_C")
    (`self.Shatter` ImpulseDirection)
    (for _ (range 2)
      (bind _returnvalue_2 (`|SpawnActorFromClass` "/Game/_DungeonCompanyContent/Code/Items/ManaCrystal/BP_ManaCrystal_World.BP_ManaCrystal_World_C" (`KismetMathLibrary.MakeTransform` (+ (`SceneComponent.K2_GetComponentLocation` (`self.Mined`)) (0.0 0.0 45.0)) (`KismetMathLibrary.RandomRotator` true)) "Undefined" "MultiplyWithRoot" null null))
      (`PrimitiveComponent.AddImpulse` (`/Game/_DungeonCompanyContent/Code/Items/ManaCrystal/BP_ManaCrystal_World.Mesh` _returnvalue_2) (* (`KismetMathLibrary.MakeVector` _returnvalue _returnvalue 2.0) (`self.ImpulseStrenght`)) "None" false))
    (else
      (`KismetSystemLibrary.PrintString` "DING! Wrong Tool"))))

(event `Shatter`
  (params (Impulse :type "Vector Structure"))
  (bind _mined (`self.Mined`))
  ;[0.6869 0.2143 1] Multicast
  ; Shatter
  (`|ExecutionSequence`
    (:`then_0`
      (`ActorComponent.K2_DestroyComponent` (`self.Crystal`)))
    (:`then_1`
      (`SceneComponent.SetVisibility` _mined true false)
      (`PrimitiveComponent.SetCollisionEnabled` _mined "QueryAndPhysics"))))

(fn `UserConstructionScript`)