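; Breakable pot world actor that shatters when hit and may drop up to five coin pickups.
; Server-side Hit multicasts Shatter, marks the pot broken and spawns coins from a single random roll against nested chance thresholds.
; Shatter swaps the intact mesh for physics-driven pieces with impulse and sound, hiding them after a delay; SetBrokenState hides everything immediately.
; The construction script can snap the pot to the surface below via line trace.
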(event `self.ReceiveBeginPlay`)

(event `self.Hit`
  (params (ImpulseDirection :type "Vector Structure") (WeaponClass :type "Weapon Class Reference"))
  (bind _returnvalue (`KismetMathLibrary.RandomFloatInRange` -5.0 5.0))
  ;[1 0.5049 0] On Server
  (`self.Shatter` ImpulseDirection)
  (set `self.bIsBroken` true :!pinned true) ; DONT FORGET ME!!!!
  (bind _coinamount (`self.DropChanceCalculation`))
  (for _ (range 1 (+ _coinamount 1))
    (`|SpawnActorFromClass` "/Game/_DungeonCompanyContent/Code/Items/WorldCurrency/Coin/BP_Coin_World.BP_Coin_World_C" (`KismetMathLibrary.MakeTransform` (+ (`SceneComponent.K2_GetComponentLocation` (`self.DefaultSceneRoot`)) (0.0 0.0 20.0) (`KismetMathLibrary.MakeVector` _returnvalue _returnvalue _returnvalue)) (`KismetMathLibrary.RandomRotator` true)) "Undefined" "MultiplyWithRoot" null null)))

(event `Shatter`
  (params (Impulse :type "Vector Structure"))
  (bind _vase_lp (`self.vase_LP`))
  (bind _shatteredvase_4 (`self.ShatteredVase_4`))
  (bind _shatteredvase_3 (`self.ShatteredVase_3`))
  ;[1 0.09837 0.845] Multicast
  (`|ExecutionSequence`
    (:`then_0`
      (`|ExecutionSequence`
        (:`then_0`
          (`SceneComponent.SetVisibility` _vase_lp false false)
          (`PrimitiveComponent.SetCollisionEnabled` _vase_lp "NoCollision"))
        (:`then_1`
          (`SceneComponent.SetVisibility` (`self.ShatteredVase_1`) true false)
          (`SceneComponent.SetVisibility` _shatteredvase_4 true false)
          (`SceneComponent.SetVisibility` (`self.ShatteredVase_2`) true false)
          (`SceneComponent.SetVisibility` (`self.vase_LP_Lid`) true false)
          (`SceneComponent.SetVisibility` (`self.ShatteredVase_3`) true false)
          (`PrimitiveComponent.SetSimulatePhysics` _shatteredvase_4 true)
          (`PrimitiveComponent.SetSimulatePhysics` (`self.ShatteredVase_1`) true)
          (`PrimitiveComponent.SetSimulatePhysics` (`self.ShatteredVase_2`) true)
          (`PrimitiveComponent.SetSimulatePhysics` (`self.vase_LP_Lid`) true)
          (`PrimitiveComponent.SetSimulatePhysics` (`self.ShatteredVase_3`) true)
          (`PrimitiveComponent.AddImpulse` _shatteredvase_4 (* Impulse (`self.ImpuleStrenght`)) "None" false)
          (`PrimitiveComponent.AddImpulse` (`self.ShatteredVase_1`) (* Impulse (`self.ImpuleStrenght`)) "None" false)
          (`PrimitiveComponent.AddImpulse` (`self.ShatteredVase_2`) (* Impulse (`self.ImpuleStrenght`)) "None" false)
          (`PrimitiveComponent.AddImpulse` (`self.vase_LP_Lid`) (* Impulse (`self.ImpuleStrenght`)) "None" false)
          (`PrimitiveComponent.AddImpulse` (`self.ShatteredVase_3`) (* Impulse (`self.ImpuleStrenght`)) "None" false))
        (:`then_2`
          (`GameplayStatics.SpawnSoundAtLocation` (`self.ShatterSound`) (`SceneComponent.K2_GetComponentLocation` (`self.DefaultSceneRoot`)) (struct) 1.0 1.0 0.0 null null))))
    (:`then_1`
      (`KismetSystemLibrary.Delay` 5.0)
      (`SceneComponent.SetVisibility` _shatteredvase_3 false false)
      (`SceneComponent.SetVisibility` (`self.ShatteredVase_4`) false false)
      (`SceneComponent.SetVisibility` (`self.ShatteredVase_1`) false false)
      (`SceneComponent.SetVisibility` (`self.ShatteredVase_2`) false false)
      (`SceneComponent.SetVisibility` (`self.vase_LP_Lid`) false false)
      (`PrimitiveComponent.SetSimulatePhysics` _shatteredvase_3 false)
      (`PrimitiveComponent.SetSimulatePhysics` (`self.ShatteredVase_1`) false)
      (`PrimitiveComponent.SetSimulatePhysics` (`self.ShatteredVase_2`) false)
      (`PrimitiveComponent.SetSimulatePhysics` (`self.vase_LP_Lid`) false)
      (`PrimitiveComponent.SetSimulatePhysics` (`self.ShatteredVase_4`) false)
      (`PrimitiveComponent.SetCollisionEnabled` _shatteredvase_3 "NoCollision")
      (`PrimitiveComponent.SetCollisionEnabled` (`self.ShatteredVase_4`) "NoCollision")
      (`PrimitiveComponent.SetCollisionEnabled` (`self.ShatteredVase_1`) "NoCollision")
      (`PrimitiveComponent.SetCollisionEnabled` (`self.ShatteredVase_2`) "NoCollision")
      (`PrimitiveComponent.SetCollisionEnabled` (`self.vase_LP_Lid`) "NoCollision"))))

(event `self.SetBrokenState`
  (bind _shatteredvase_3 (`self.ShatteredVase_3`))
  ;[0.2275 1 0.4275] SetBrokenState override
  (`SceneComponent.SetVisibility` _shatteredvase_3 false false)
  (`SceneComponent.SetVisibility` (`self.ShatteredVase_4`) false false)
  (`SceneComponent.SetVisibility` (`self.ShatteredVase_1`) false false)
  (`SceneComponent.SetVisibility` (`self.ShatteredVase_2`) false false)
  (`SceneComponent.SetVisibility` (`self.vase_LP_Lid`) false false)
  (`SceneComponent.SetVisibility` (`self.vase_LP`) false false)
  (`PrimitiveComponent.SetSimulatePhysics` _shatteredvase_3 false)
  (`PrimitiveComponent.SetSimulatePhysics` (`self.ShatteredVase_1`) false)
  (`PrimitiveComponent.SetSimulatePhysics` (`self.ShatteredVase_2`) false)
  (`PrimitiveComponent.SetSimulatePhysics` (`self.vase_LP_Lid`) false)
  (`PrimitiveComponent.SetSimulatePhysics` (`self.ShatteredVase_4`) false)
  (`PrimitiveComponent.SetSimulatePhysics` (`self.vase_LP`) false)
  (`PrimitiveComponent.SetCollisionEnabled` _shatteredvase_3 "NoCollision")
  (`PrimitiveComponent.SetCollisionEnabled` (`self.ShatteredVase_4`) "NoCollision")
  (`PrimitiveComponent.SetCollisionEnabled` (`self.ShatteredVase_1`) "NoCollision")
  (`PrimitiveComponent.SetCollisionEnabled` (`self.ShatteredVase_2`) "NoCollision")
  (`PrimitiveComponent.SetCollisionEnabled` (`self.vase_LP_Lid`) "NoCollision")
  (`PrimitiveComponent.SetCollisionEnabled` (`self.vase_LP`) "NoCollision"))

(fn `DropChanceCalculation`
  (returns (CoinAmount :type Integer))
  (locals (LuckyNumber :type "Float (double-precision)" :default 0.0))
  (set `local.LuckyNumber` (`KismetMathLibrary.RandomFloatInRange` 0.0 100.0))
  (if (< (`local.LuckyNumber`) (`self.ChanceFor1Coin`))
    (if (< (`local.LuckyNumber`) (`self.ChanceFor2Coin`))
      (if (< (`local.LuckyNumber`) (`self.ChanceFor3Coin`))
        (if (< (`local.LuckyNumber`) (`self.ChanceFor4Coin`))
          (if (< (`local.LuckyNumber`) (`self.ChanceFor5Coin`))
            (return 5)
            (else
              (return 4)))
          (else
            (return 3)))
        (else
          (return 2)))
      (else
        (return 1)))
    (else
      (return 0))))

(fn `UserConstructionScript`
  (bind _returnvalue (`SceneComponent.K2_GetComponentLocation` (`self.DefaultSceneRoot`)))
  (if (`self.AlignWithNormal`)
    (bind (_outhit _returnvalue_2) (`KismetSystemLibrary.LineTraceSingle` (+ _returnvalue (0.0 0.0 20.0)) (- _returnvalue (0.0 0.0 20.0)) "TraceTypeQuery1" false (`|MakeArray` self :!type "Actor Object Reference") "ForOneFrame"))
    (if _returnvalue_2
      (bind (_bblockinghit _binitialoverlap _time _distance _location _impactpoint _normal) (`GameplayStatics.BreakHitResult` _outhit))
      (`SceneComponent.K2_SetWorldLocation` (`self.DefaultSceneRoot`) _location false false)
      (`SceneComponent.K2_SetWorldRotation` (`self.DefaultSceneRoot`) (`KismetMathLibrary.MakeRotFromZ` _normal) false false))))