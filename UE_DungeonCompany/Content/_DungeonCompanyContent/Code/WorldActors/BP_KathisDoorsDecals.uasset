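; Double sliding door puzzle actor that opens when two linked decal levers, assigned per instance, are both set.
; BeginPlay binds each decal's button-pressed event, which refreshes that lever's state, triggers its eye feedback and checks both states.
; Timelines slide the left and right doors along X with sound, closing them again if a press breaks the solved combination.
; An IsMoving flag blocks presses during movement, and debug strings report state and missing references.
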(event `CustomEvent_1`
  (params (InteractingPawn :type "Pawn Object Reference"))
  (bind _doorright (`self.DoorRight`))
  (bind _decal2 (`self.Decal2`))
  (bind _doorright_2 (`self.DoorRight`))
  (bind _doorleft (`self.DoorLeft`))
  (bind _doorleft_2 (`self.DoorLeft`))
  (bind (_relativelocation_x _relativelocation_y _relativelocation_z) (`KismetMathLibrary.BreakVector` (`SceneComponent.RelativeLocation` _doorright_2)))
  (bind (_relativelocation_x_2 _relativelocation_y_2 _relativelocation_z_2) (`KismetMathLibrary.BreakVector` (`SceneComponent.RelativeLocation` _doorright)))
  (bind (_relativelocation_x_3 _relativelocation_y_3 _relativelocation_z_3) (`KismetMathLibrary.BreakVector` (`SceneComponent.RelativeLocation` _doorleft)))
  (bind (_relativelocation_x_4 _relativelocation_y_4 _relativelocation_z_4) (`KismetMathLibrary.BreakVector` (`SceneComponent.RelativeLocation` _doorleft_2)))
  (if (`self.isMoving`)
    (`KismetSystemLibrary.PrintString` "movement blocked")
    (else
      (bind _ispressed (`/Game/_DungeonCompanyContent/Code/WorldActors/BP_KathisDecal.LeverSet` _decal2))
      (`/Game/_DungeonCompanyContent/Code/WorldActors/BP_KathisDecal.EyeFeedback` _decal2)
      (if (and (stale `CustomEvent` _ispressed) _ispressed) :!label _label
        (`KismetSystemLibrary.PrintString` "Puzzle Solved!")
        (set `self.PuzzleSolved` true)
        (`|ExecutionSequence`
          (:`then_0`
            (`AudioComponent.Play` (`self.MS_DoorSlide`) 0.0))
          (:`then_1`
            (set `self.isMoving` true))
          (:`then_2`
            (bind (_direction _floattrack) (`Timeline|Timeline` :!via `PlayFromStart`)
              (:`Update`
                (`SceneComponent.K2_SetRelativeLocation` _doorleft_2 (`KismetMathLibrary.MakeVector` _floattrack _relativelocation_y_4 _relativelocation_z_4) false false))
              (:`Finished`
                (set `self.isMoving` false))))
          (:`then_3`
            (bind (_direction_2 _floattrack_2) (`Timeline|Timeline_0` :!via `PlayFromStart`)
              (:`Update`
                (`SceneComponent.K2_SetRelativeLocation` _doorright_2 (`KismetMathLibrary.MakeVector` _floattrack_2 _relativelocation_y _relativelocation_z) false false))
              (:`Finished`
                (set `self.isMoving` false)))))
        (elif (`self.PuzzleSolved`)
          (`KismetSystemLibrary.PrintString` "Doors Closing")
          (`|ExecutionSequence`
            (:`then_0`
              (`AudioComponent.Play` (`self.MS_DoorSlide`) 0.0))
            (:`then_1`
              (set `self.isMoving` true))
            (:`then_2`
              (bind (_direction_3 _floattrack_3) (`Timeline|Timeline_1` :!via `PlayFromStart`)
                (:`Update`
                  (`SceneComponent.K2_SetRelativeLocation` _doorleft (`KismetMathLibrary.MakeVector` _floattrack_3 _relativelocation_y_3 _relativelocation_z_3) false false))
                (:`Finished`
                  (set `self.isMoving` false))))
            (:`then_3`
              (bind (_direction_4 _floattrack_4) (`Timeline|Timeline_2` :!via `PlayFromStart`)
                (:`Update`
                  (`SceneComponent.K2_SetRelativeLocation` _doorright (`KismetMathLibrary.MakeVector` _floattrack_4 _relativelocation_y_2 _relativelocation_z_2) false false))
                (:`Finished`
                  (set `self.isMoving` false))))
            (:`then_4`
              (set `self.PuzzleSolved` false))))))))

(event `CustomEvent`
  (params (InteractingPawn :type "Pawn Object Reference"))
  (bind _decal1 (`self.Decal1`))
  (if (`self.isMoving`)
    (`KismetSystemLibrary.PrintString` "movement blocked")
    (else
      (`|ExecutionSequence`
        (:`then_0`
          (bind _ispressed (`/Game/_DungeonCompanyContent/Code/WorldActors/BP_KathisDecal.LeverSet` _decal1))
          (`/Game/_DungeonCompanyContent/Code/WorldActors/BP_KathisDecal.EyeFeedback` _decal1))
        (:`then_1`
          (goto _label))))))

(event `self.ReceiveBeginPlay`
  (`/Engine/EditorBlueprintResources/StandardMacros.IsValid` (`self.Decal1`)
    (:`Is Valid`
      (`/Engine/EditorBlueprintResources/StandardMacros.IsValid` (`self.Decal2`)
        (:`Is Valid`
          (add `BasicButton.OnButtonPressed` (`self.Decal2`) (delegate `CustomEvent_1`))
          (add `BasicButton.OnButtonPressed` (`self.Decal1`) (delegate `CustomEvent`)))
        (:`Is Not Valid`
          (`KismetSystemLibrary.PrintString` "Lever 2 was not valid \nBind in Outliner"))))
    (:`Is Not Valid`
      (`KismetSystemLibrary.PrintString` "Lever 1 was not valid \nBind in Outliner"))))

(fn `UserConstructionScript`)