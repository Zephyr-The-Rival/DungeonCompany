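; Wall generator actor that fills the X/Z span to a linked WallGeneratorEnd marker with a grid of brick mesh components.
; The construction script rebinds the marker's drag event and runs GenerateStuff, which clears and rebuilds the bricks using configurable gaps.
; Options add staggered rows, cube fillers at row ends, random flips and yaw jitter.
; RasterBricks hands the components to SpawnBricks; the Y-depth loop is disconnected.
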(event `Generate Stuff`
  (bind _blocktransform (`self.BlockTransform`))
  (bind _blocktransform_2 (`self.BlockTransform`))
  (bind _dalta_location_x (`KismetMathLibrary.BreakVector` (`self.Dalta location`)))
  (bind _blocktransform_3 (`self.BlockTransform`))
  (bind _blocktransform_4 (`self.BlockTransform`))
  (bind _bricks (`self.Bricks`))
  (bind (_dalta_location_x_2 _dalta_location_y _dalta_location_z) (`KismetMathLibrary.BreakVector` (`self.Dalta location`)))
  (bind _currentx (`self.CurrentX`))
  (bind _textrender (`/Game/_DungeonCompanyContent/Code/WorldActors/WallGenerator/BP_WallGeneratorEnd.TextRender` (`self.WallGeneratorEnd`)))
  (bind (_relativelocation_x _relativelocation_y _relativelocation_z) (`KismetMathLibrary.BreakVector` (`SceneComponent.RelativeLocation` _textrender)))
  (bind _returnvalue (`KismetMathLibrary.FTrunc` (/ _dalta_location_x (+ (`self.GapX`) 100.0))))
  (bind _returnvalue_2 (`KismetMathLibrary.FTrunc` (/ _dalta_location_z (+ (`self.GapZ`) 50.0))))
  (`|ExecutionSequence`
    (:`then_0`
      (for _array_element _bricks
        (`ActorComponent.K2_DestroyComponent` _array_element))
      (`KismetArrayLibrary.Array_Clear` _bricks))
    (:`then_1`
      (`|ExecutionSequence`
        (:`then_0`
          (`self.K2_AttachToComponent` (`self.WallGeneratorEnd`) (`self.DefaultSceneRoot`) "None" "KeepWorld" "KeepWorld" "KeepRelative" true)
          (`SceneComponent.K2_SetRelativeLocation` _textrender (`KismetMathLibrary.MakeVector` _relativelocation_x 0.0 _relativelocation_z) false false))
        (:`then_1`
          (set `self.Dalta location` (`SceneComponent.RelativeLocation` (`/Game/_DungeonCompanyContent/Code/WorldActors/WallGenerator/BP_WallGeneratorEnd.TextRender` (`self.WallGeneratorEnd`))))
          ;[1 1 1] Z
          (bind _output_get (set `self.LastZ` (`KismetMathLibrary.Abs_Int` _returnvalue_2)))
          (for _index (range (+ _output_get 1))
            (bind _output_get_2 (set `self.CurrentZ` _index))
            (if (> _returnvalue_2 0)
              (bind _returnvalue_3 (* _output_get_2 (+ 50.0 (`self.GapZ`))))
              (`KismetMathLibrary.Vector_Set` _blocktransform (.x _blocktransform) (.y _blocktransform) _returnvalue_3)
              (else
                (`KismetMathLibrary.Vector_Set` _blocktransform_2 (.x _blocktransform_2) (.y _blocktransform_2) (* _returnvalue_3 -1.0))))
            ;[1 1 1] X
            (bind _output_get_3 (set `self.LastX` (`KismetMathLibrary.Abs_Int` _returnvalue)))
            (for _index_2 (range (+ _output_get_3 1))
              (bind _output_get_4 (set `self.CurrentX` _index_2))
              (if (> _returnvalue 0)
                (bind _returnvalue_4 (* _output_get_4 (+ 100.0 (`self.GapX`))))
                (`KismetMathLibrary.Vector_Set` _blocktransform_4 _returnvalue_4 (.y _blocktransform_4) (.z _blocktransform_4))
                (else
                  (`KismetMathLibrary.Vector_Set` _blocktransform_3 (* _returnvalue_4 -1.0) (.y _blocktransform_3) (.z _blocktransform_3))))
              (if (and (`self.Offset`) (== (`KismetMathLibrary.FMod` (`KismetMathLibrary.Conv_IntToDouble` (`self.CurrentZ`)) 2.0) 0.0))
                (set `self.BlockTransform` (+ (`self.BlockTransform`) (50.0 0.0 0.0))))
              (if false
                (set `self.BlockTransform` (+ (`self.BlockTransform`) (50.0 0.0 0.0))))
              (if (not (`self.Offset`))
                (bind _returnvalue_5 (`AddComponent|NODE_AddStaticMeshComponent-1` :`RelativeTransform` (`KismetMathLibrary.MakeTransform` (`self.BlockTransform`) (`self.Get Rotation With Variations`)))) ; regular brick
                (`KismetArrayLibrary.Array_Add` (`self.Bricks`) _returnvalue_5)
                (elif (and (== (`KismetMathLibrary.FMod` (`KismetMathLibrary.Conv_IntToDouble` (`self.CurrentZ`)) 2.0) 0.0) (or (== _currentx 0) (== _currentx (`self.LastX`))))
                  (if (== (`self.CurrentX`) 0)
                    (bind _returnvalue_6 (`AddComponent|NODE_AddStaticMeshComponent-5` :`RelativeTransform` (`KismetMathLibrary.MakeTransform` (`self.BlockTransform`) (`self.Get Rotation With Variations`)))) ; regular brick
                    (`KismetArrayLibrary.Array_Add` (`self.Bricks`) _returnvalue_6)
                    (if (`self.FillerBricks`)
                      (bind _returnvalue_7 (`AddComponent|NODE_AddStaticMeshComponent-6` :`RelativeTransform` (`KismetMathLibrary.MakeTransform` (+ (`self.BlockTransform`) (-75.0 0.0 0.0)) (`self.Get Rotation With Variations`)))) ; cube brick
                      (`KismetArrayLibrary.Array_Add` (`self.Bricks`) _returnvalue_7))
                    (elif (`self.FillerBricks`)
                      (bind _returnvalue_8 (`AddComponent|NODE_AddStaticMeshComponent-4` :`RelativeTransform` (`KismetMathLibrary.MakeTransform` (- (`self.BlockTransform`) (25.0 0.0 0.0)) (`self.Get Rotation With Variations`)))) ; cube brick
                      (`KismetArrayLibrary.Array_Add` (`self.Bricks`) _returnvalue_8)))
                  (else
                    (bind _returnvalue_9 (`AddComponent|NODE_AddStaticMeshComponent-2` :`RelativeTransform` (`KismetMathLibrary.MakeTransform` (`self.BlockTransform`) (`self.Get Rotation With Variations`)))) ; regular brick
                    (`KismetArrayLibrary.Array_Add` (`self.Bricks`) _returnvalue_9)))))))))))

(event `RasterBricks`
  (`self.SpawnBricks` (`self.Bricks`) (`self.NameSuffix`)))

(fn `Get Rotation With Variations`
  (returns (NewParam :type "Rotator Structure"))
  (locals (RotToReturn :type "Rotator Structure"))
  (bind _microorientationamount (`self.MicroOrientationAmount`))
  (bind (_rottoreturn_roll _rottoreturn_pitch _rottoreturn_yaw) (`KismetMathLibrary.BreakRotator` (`local.RotToReturn`)))
  (`|ExecutionSequence`
    (:`then_0`
      (if (`self.RandomOrientation`)
        (if (`KismetMathLibrary.RandomBool`)
          (set `local.RotToReturn` (struct))
          (else
            (set `local.RotToReturn` (struct :`Yaw` 180.0))))))
    (:`then_1`
      (if (!= (`self.MicroOrientationAmount`) 0.0)
        (set `local.RotToReturn` (`KismetMathLibrary.MakeRotator` _rottoreturn_roll _rottoreturn_pitch (+ _rottoreturn_yaw (`KismetMathLibrary.RandomFloatInRange` (* _microorientationamount -1.0) _microorientationamount))))))
    (:`then_2`
      (return (`local.RotToReturn`)))))

(fn `UserConstructionScript`
  (bind _wallgeneratorend (`self.WallGeneratorEnd`))
  (`/Engine/EditorBlueprintResources/StandardMacros.IsValid` (`self.WallGeneratorEnd`)
    (:`Is Valid`
      (clear `/Game/_DungeonCompanyContent/Code/WorldActors/WallGenerator/BP_WallGeneratorEnd.IsBeeingDragged` _wallgeneratorend)
      (add `/Game/_DungeonCompanyContent/Code/WorldActors/WallGenerator/BP_WallGeneratorEnd.IsBeeingDragged` _wallgeneratorend (`|CreateDelegate` :!event `Generate Stuff`))
      (`self.Generate Stuff`))))