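; World actor that switches the level between a ray-traced setup for light baking and normal settings.
; SetSettingsToLightbake sets the first PostProcessVolume found to brute-force ray tracing and turns on the project's ray-traced shadows setting.
; ResetSettings sets those methods to None and turns the shadow setting off, printing status along the way.
; BeginPlay runs the same reset, so the bake settings do not carry into gameplay.
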(event `SetSettingsToLightbake`
  (bind _returnvalue (`GameplayStatics.GetActorOfClass` "/Script/Engine.PostProcessVolume"))
  (`/Engine/EditorBlueprintResources/StandardMacros.IsValid` _returnvalue
    (:`Is Valid`
      (bind _structout (setmembers `PostProcessSettings` :`StructRef` (`PostProcessVolume.Settings` _returnvalue) :`DynamicGlobalIlluminationMethod` "RayTraced" :`RayTracingGIType` "BruteForce" :`RayTracingGIMaxBounces` 4 :`RayTracingGISamplesPerPixel` 8 :`ReflectionMethod` "RayTraced"))
      (set `PostProcessVolume.Settings` _structout _returnvalue)
      (`KismetSystemLibrary.PrintString` "PostProcess settings set")
      (`self.SetShadowProjectSettings` true)
      (`KismetSystemLibrary.PrintString` "Project setting Ray traced shadows set to true"))
    (:`Is Not Valid`
      (`KismetSystemLibrary.PrintString` "no post process volume found"))))

(event `ResetSettings`
  (bind _returnvalue (`GameplayStatics.GetActorOfClass` "/Script/Engine.PostProcessVolume" :!label _label))
  (`/Engine/EditorBlueprintResources/StandardMacros.IsValid` _returnvalue
    (:`Is Valid`
      (bind _structout (setmembers `PostProcessSettings` :`StructRef` (`PostProcessVolume.Settings` _returnvalue) :`DynamicGlobalIlluminationMethod` "None" :`RayTracingGIType` "Disabled" :`RayTracingGIMaxBounces` 4 :`RayTracingGISamplesPerPixel` 8 :`ReflectionMethod` "None"))
      (set `PostProcessVolume.Settings` _structout _returnvalue)
      (`KismetSystemLibrary.PrintString` "PostProcess settings set")
      (`self.SetShadowProjectSettings` false)
      (`KismetSystemLibrary.PrintString` "Project setting Ray traced shadows set to false"))))

(event `self.ReceiveBeginPlay`
  (goto _label))

(fn `UserConstructionScript`)