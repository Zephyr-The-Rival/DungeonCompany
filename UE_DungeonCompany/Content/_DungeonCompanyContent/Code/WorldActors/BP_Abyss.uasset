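; BP_Abyss is a world actor that renders an abyss using a decal and a black floor, set up entirely in the construction script.
; It creates a dynamic material instance for the decal and feeds it the root's world height, vertical scale and a strength value.
; The black floor is moved below the root by a distance proportional to the root's Z scale, so actor scale controls depth.
; It has no runtime logic.
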(fn `UserConstructionScript`
  (bind _defaultsceneroot (`self.DefaultSceneRoot`))
  (bind _defaultsceneroot_2 (`self.DefaultSceneRoot`))
  (bind (_returnvalue_x _returnvalue_y _returnvalue_z) (`KismetMathLibrary.BreakVector` (`SceneComponent.K2_GetComponentScale` _defaultsceneroot_2)))
  (bind (_returnvalue_x_2 _returnvalue_y_2 _returnvalue_z_2) (`KismetMathLibrary.BreakVector` (`SceneComponent.K2_GetComponentLocation` _defaultsceneroot_2)))
  (bind (_returnvalue_x_3 _returnvalue_y_3 _returnvalue_z_3) (`KismetMathLibrary.BreakVector` (`SceneComponent.K2_GetComponentScale` _defaultsceneroot)))
  (`|ExecutionSequence`
    (:`then_0`
      (bind _returnvalue (`KismetMaterialLibrary.CreateDynamicMaterialInstance` "/Game/_DungeonCompanyContent/Assets/Materials/AbyssMaterial.AbyssMaterial"))
      (`DecalComponent.SetDecalMaterial` (`self.Decal`) _returnvalue)
      (`MaterialInstanceDynamic.SetScalarParameterValue` _returnvalue "Height" _returnvalue_z_2)
      (`MaterialInstanceDynamic.SetScalarParameterValue` _returnvalue "VerticalScale" _returnvalue_z)
      (`MaterialInstanceDynamic.SetScalarParameterValue` _returnvalue "Strenght" (`self.Strenght`)))
    (:`then_1`
      (`SceneComponent.K2_SetWorldLocation` (`self.BlackFloor`) (- (`SceneComponent.K2_GetComponentLocation` _defaultsceneroot) (`KismetMathLibrary.MakeVector` 0.0 0.0 (* _returnvalue_z_3 100.0))) false false))))