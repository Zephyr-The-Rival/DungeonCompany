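; Dungeon elevator that toggles up or down on a bell-rope pull, using timelines, rumble audio and local camera fades.
; At the top, the server teleports riders to BP_Elevator_Village's points, starts that elevator rising and calls LeftBehind on players outside.
; During descent, a kill box kills overlapping entities that are not falling.
; The construction script links and generates both rope beams.
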(event `self.ReceiveBeginPlay`
  (add `/Game/_DungeonCompanyContent/Code/WorldActors/Elevator/BP_ElevatorCall_Button.RopePulled` (`self.MyRopeButton`) (delegate `OnRopePulled`))
  (set `self.TeleportPoints` (`|MakeArray` (`self.TeleportPoint`) (`self.TeleportPoint1`) (`self.TeleportPoint2`) (`self.TeleportPoint3`))))

(event `OnRopePulled`
  (`AudioComponent.Play` (`self.BellSound`) 0.0)
  (if (not (`self.IsMoving`))
    (`KismetSystemLibrary.Delay` 1.5)
    (if (`self.IsDown`)
      (`self.MoveUp`)
      (else
        (`self.MoveDown`)))))

(event `StartSound`)

(event `MoveDown`
  ;[1 1 1] Move down
  (`self.FadeFromBlack`)
  (`AudioComponent.Play` (`self.ElevatorRumble`) 5.0)
  (set `self.IsMoving` true)
  (bind (_direction _newtrack_0) (`Timeline|Timeline` :!via `PlayFromStart`)
    (:`Update`
      (`SceneComponent.K2_SetRelativeLocation` (`self.SM_Elevator`) _newtrack_0 false false))
    (:`Finished`
      (`AudioComponent.Stop` (`self.ElevatorRumble`))
      (set `self.IsMoving` false)
      (set `self.IsDown` true)
      (set `self.bAlwaysRelevant` false))))

(event `MoveUp`
  ;[1 1 1] MoveUP
  (`|ExecutionSequence`
    (:`then_0`
      (`AudioComponent.Play` (`self.ElevatorRumble`) 5.0)
      (set `self.IsMoving` true)
      (bind (_direction _newtrack_0) (`Timeline|Timeline_1` :!via `PlayFromStart`)
        (:`Update`
          (`SceneComponent.K2_SetRelativeLocation` (`self.SM_Elevator`) _newtrack_0 false false))
        (:`Finished`
          (`AudioComponent.Stop` (`self.ElevatorRumble`))
          (set `self.IsMoving` false)
          (set `self.IsDown` false)
          (`SceneComponent.SetVisibility` (`SkyLight.LightComponent` (`self.SkyLightToTurnBackOn`)) true false)
          (`/Engine/EditorBlueprintResources/ActorMacros.Switch Has Authority`
            (:`Authority`
              (`self.ElevatorArrivedOnTop`))))))
    (:`then_1`
      (`KismetSystemLibrary.Delay` 8.0)
      (`self.FadeToWhite`))))

(event `self.KillBox.OnComponentBeginOverlap`
  (params (OverlappedComponent :type "PrimitiveComponent Object Reference") (OtherActor :type "Actor Object Reference") (OtherComp :type "PrimitiveComponent Object Reference") (OtherBodyIndex :type Integer) (bFromSweep :type Boolean) (SweepResult :type "HitResult Structure (by ref)"))
  (bind _asdc_entity (cast `DC_Entity` OtherActor))
  (if (and (not (`NavMovementComponent.IsFalling` (`Character.CharacterMovement` _asdc_entity))) (`self.IsMoving`) (not (`self.IsDown`)))
    (`DC_Entity.OnDeath` _asdc_entity)))

(fn `ElevatorArrivedOnTop`
  (locals (PlayersInElevator :type "Array of Actor Object Reference"))
  (bind _output_get (set `local.PlayersInElevator` (`PrimitiveComponent.GetOverlappingActors` (`self.Box`) "/Game/_DungeonCompanyContent/Code/PlayerCharacter/BP_PlayerCharacter.BP_PlayerCharacter_C")))
  (if (not (`KismetArrayLibrary.Array_IsEmpty` _output_get))
    (`|ExecutionSequence`
      (:`then_0`
        (bind _outactors (`GameplayStatics.GetAllActorsOfClass` "/Game/_DungeonCompanyContent/Code/PlayerCharacter/BP_PlayerCharacter.BP_PlayerCharacter_C"))
        (for (_array_element _array_index) _outactors
          (if (`KismetArrayLibrary.Array_Contains` (`local.PlayersInElevator`) _array_element)
            (bind _returnvalue (`GameplayStatics.GetActorOfClass` "/Game/_DungeonCompanyContent/Code/WorldActors/Elevator/BP_Elevator_Village.BP_Elevator_Village_C"))
            (`SceneComponent.K2_SetWorldTransform` (`Character.CapsuleComponent` _array_element) (`SceneComponent.K2_GetComponentToWorld` (`|GetArrayItem` (`/Game/_DungeonCompanyContent/Code/WorldActors/Elevator/BP_Elevator_Village.TeleportPoints` _returnvalue) _array_index)) false true)
            (`/Engine/EditorBlueprintResources/StandardMacros.DoOnce` false
              (:`Completed`
                (`/Game/_DungeonCompanyContent/Code/WorldActors/Elevator/BP_Elevator_Village.MoveUp` _returnvalue)))
            (else
              (`PlayerCharacter.LeftBehind` _array_element)))))
      (:`then_1`
        (bind _returnvalue_2 (`GameplayStatics.GetActorOfClass` "/Game/_DungeonCompanyContent/Code/WorldActors/Elevator/BP_Elevator_Village.BP_Elevator_Village_C"))
        (set `Actor.bAlwaysRelevant` true _returnvalue_2)
        (`/Game/_DungeonCompanyContent/Code/WorldActors/Elevator/BP_Elevator_Village.MoveUp` _returnvalue_2)))))

(fn `FadeFromBlack`
  (bind _returnvalue (`GameplayStatics.GetPlayerController` 0))
  (cast `/Game/_DungeonCompanyContent/Code/PlayerCharacter/BP_PlayerCharacter` (`Controller.K2_GetPawn` _returnvalue))
  (`PlayerCameraManager.StartCameraFade` :`self` (`PlayerController.PlayerCameraManager` _returnvalue) :`FromAlpha` 1.0 :`Duration` 2.0 :`bHoldWhenFinished` true))

(fn `FadeToWhite`
  (bind _returnvalue (`GameplayStatics.GetPlayerController` 0))
  (bind _asbp_player_character (cast `/Game/_DungeonCompanyContent/Code/PlayerCharacter/BP_PlayerCharacter` (`Controller.K2_GetPawn` _returnvalue)))
  (if (`KismetArrayLibrary.Array_Contains` (`PrimitiveComponent.GetOverlappingActors` (`self.Box`) "/Game/_DungeonCompanyContent/Code/PlayerCharacter/BP_PlayerCharacter.BP_PlayerCharacter_C") _asbp_player_character)
    (`PlayerCameraManager.StartCameraFade` (`PlayerController.PlayerCameraManager` _returnvalue) 0.0 1.0 2.0 (struct :`R` 1.0 :`G` 1.0 :`B` 1.0 :`A` 1.0) false true)))

(fn `UserConstructionScript`
  (bind _asbp_rope_beam (cast `/Game/_DungeonCompanyContent/Code/WorldActors/Rope/BP_RopeBeam` (`ChildActorComponent.ChildActor` (`self.RopeRight`))))
  (set `/Game/_DungeonCompanyContent/Code/WorldActors/Rope/BP_RopeBeam.MyRopeEnd` (cast `/Game/_DungeonCompanyContent/Code/WorldActors/Rope/BP_RopeEnd` (`ChildActorComponent.ChildActor` (`self.RopeEndRight`)) :!pure true) _asbp_rope_beam)
  (bind _asbp_rope_beam_2 (cast `/Game/_DungeonCompanyContent/Code/WorldActors/Rope/BP_RopeBeam` (`ChildActorComponent.ChildActor` (`self.RopeLeft`))))
  (set `/Game/_DungeonCompanyContent/Code/WorldActors/Rope/BP_RopeBeam.MyRopeEnd` (cast `/Game/_DungeonCompanyContent/Code/WorldActors/Rope/BP_RopeEnd` (`ChildActorComponent.ChildActor` (`self.RopeEndLeft`)) :!pure true) _asbp_rope_beam_2)
  (`/Game/_DungeonCompanyContent/Code/WorldActors/Rope/BP_RopeBeam.GenerateRope` _asbp_rope_beam_2)
  (`/Game/_DungeonCompanyContent/Code/WorldActors/Rope/BP_RopeBeam.GenerateRope` _asbp_rope_beam))