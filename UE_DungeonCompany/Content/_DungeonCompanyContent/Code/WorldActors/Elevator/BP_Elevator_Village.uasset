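; Village elevator that carries the party to the dungeon once its button is pressed with every living player inside.
; The server binds the button and checks the trigger box against all living player characters.
; A timeline moves the car, then the skylight is hidden and the server starts the linked dungeon elevator, teleporting riders to its teleport points.
; MoveUp animates the return and clears the elevator's always-relevant flag.
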(event `self.ReceiveBeginPlay`
  (set `self.TeleportPoints` (`|MakeArray` (`self.TeleportPoint1`) (`self.TeleportPoint2`) (`self.TeleportPoint3`) (`self.TeleportPoint`)))
  (bind _asbasic_button (cast `BasicButton` (`ChildActorComponent.ChildActor` (`self.Button`))))
  (add `BasicButton.OnButtonPressed` _asbasic_button (delegate `OnButtonPressed_Event`)))

(event `OnButtonPressed_Event`
  (params (InteractingPawn :type "Pawn Object Reference"))
  (bind _allcontained (`self.AreAllAlivePlayersIn` (`PrimitiveComponent.GetOverlappingActors` (`self.Box`) "/Game/_DungeonCompanyContent/Code/PlayerCharacter/BP_PlayerCharacter.BP_PlayerCharacter_C")))
  (if _allcontained
    (`self.Move Down`)))

(event `Move Down`
  (bind _elevatordungeon (`self.ElevatorDungeon`))
  (`AudioComponent.Play` (`self.ElevatorRumble`) 0.0)
  (bind (_direction _0_to__1) (`Timeline|MoveDown` :!via `PlayFromStart`)
    (:`Update`
      (`SceneComponent.K2_SetRelativeLocation` (`self.SM_Elevator`) (`KismetMathLibrary.MakeVector` 0.0 0.0 (* _0_to__1 700.0)) false false))
    (:`Finished`
      (`|ExecutionSequence`
        (:`then_0`
          (bind _returnvalue (`GameplayStatics.GetActorOfClass` "/Script/Engine.SkyLight"))
          (`SceneComponent.SetVisibility` (`SkyLight.LightComponent` _returnvalue) false false)
          (`AudioComponent.Stop` (`self.ElevatorRumble`)))
        (:`then_1`
          (`/Engine/EditorBlueprintResources/ActorMacros.Switch Has Authority`
            (:`Authority`
              (set `Actor.bAlwaysRelevant` true _elevatordungeon)
              (`/Game/_DungeonCompanyContent/Code/WorldActors/Elevator/BP_Elevator_Dungeon.MoveDown` _elevatordungeon)
              (`KismetSystemLibrary.DelayUntilNextTick`)
              (bind _output_get (set `self.Overlapping Actors` (`PrimitiveComponent.GetOverlappingActors` (`self.Box`) "/Game/_DungeonCompanyContent/Code/PlayerCharacter/BP_PlayerCharacter.BP_PlayerCharacter_C")))
              (for (_array_element _array_index) _output_get
                (bind _asbp_player_character (cast `/Game/_DungeonCompanyContent/Code/PlayerCharacter/BP_PlayerCharacter` _array_element))
                (`SceneComponent.K2_SetWorldTransform` (`Character.CapsuleComponent` _asbp_player_character) (`SceneComponent.K2_GetComponentToWorld` (`|GetArrayItem` (`/Game/_DungeonCompanyContent/Code/WorldActors/Elevator/BP_Elevator_Dungeon.TeleportPoints` (`self.ElevatorDungeon`)) _array_index)) false true)))))))))

(event `MoveUp`
  (`AudioComponent.Play` (`self.ElevatorRumble`) 0.0)
  (bind (_direction __1_to_0) (`Timeline|Timeline` :!via `PlayFromStart`)
    (:`Update`
      (`SceneComponent.K2_SetRelativeLocation` (`self.SM_Elevator`) (`KismetMathLibrary.MakeVector` 0.0 0.0 (* __1_to_0 700.0)) false false))
    (:`Finished`
      (set `self.bAlwaysRelevant` false)
      (`AudioComponent.Stop` (`self.ElevatorRumble`)))))

(fn `AreAllAlivePlayersIn`
  (params (Actors :type "Array of Actor Object Reference"))
  (returns (AllContained :type Boolean))
  (bind _outactors (`GameplayStatics.GetAllActorsOfClass` "/Game/_DungeonCompanyContent/Code/PlayerCharacter/BP_PlayerCharacter.BP_PlayerCharacter_C"))
  (for _array_element _outactors
    (if (and (not (`DC_Entity.IsDead` _array_element)) (not (`KismetArrayLibrary.Array_Contains` Actors _array_element)))
      (return false)))
  (return true))

(fn `UserConstructionScript`)