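; BP_ElevatorCall_Button is an interactable elevator call button that behaves as a pull rope.
; A press plays a timeline that animates the static mesh's relative height.
; When the timeline finishes, only the authority fires RopePulled.
; BeginPlay binds the press event and stores Pulled and Hangin transforms, which the graph never reads.
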(event `self.ReceiveBeginPlay`
  (bind (_returnvalue_location _returnvalue_rotation _returnvalue_scale) (`KismetMathLibrary.BreakTransform` (`SceneComponent.GetRelativeTransform` (`self.StaticMesh`))))
  (`|ExecutionSequence`
    (:`then_0`
      (set `self.Pulled` (`KismetMathLibrary.MakeTransform` _returnvalue_location _returnvalue_rotation _returnvalue_scale))
      (set `self.Hangin` (`KismetMathLibrary.MakeTransform` (- _returnvalue_scale (0.0 0.0 -30.0)) _returnvalue_rotation _returnvalue_scale)))
    (:`then_1`
      (add `BasicButton.OnButtonPressed` (delegate `Interacted`)))))

(event `Interacted`
  (params (InteractingPawn :type "Pawn Object Reference"))
  (`self.MoveRope`))

(event `MoveRope`
  (bind (_direction _height) (`Timeline|Timeline` :!via `PlayFromStart`)
    (:`Update`
      (`SceneComponent.K2_SetRelativeLocation` (`self.StaticMesh`) (`KismetMathLibrary.MakeVector` 0.0 0.0 _height) false false))
    (:`Finished`
      (`/Engine/EditorBlueprintResources/ActorMacros.Switch Has Authority`
        (:`Authority`
          (`self.RopePulled`))))))

(fn `UserConstructionScript`)