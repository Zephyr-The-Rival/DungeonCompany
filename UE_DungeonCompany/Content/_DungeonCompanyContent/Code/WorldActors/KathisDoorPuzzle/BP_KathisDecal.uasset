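; BP_KathisDecal is a decal actor for Kathi's door puzzle that gives glowing eye feedback.
; The construction script gives the decal a dynamic material instance at a default emissive amount.
; EyeFeedback alternates on each call between playing a sound with a timeline that animates the emissive, and stopping the timeline to restore the default glow.
; A separate LeverSet function toggles and returns a pressed flag.
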(event `EyeFeedback`
  (bind _dynamicmat (`self.DynamicMat`))
  (if (`self.DidSwitch`)
    (`|ExecutionSequence`
      (:`then_0`
        (bind (_direction _track_01) (`Timeline|Timeline` :!via `Stop` :!label _label)
          (:`Update`
            (`MaterialInstanceDynamic.SetScalarParameterValue` _dynamicmat "EmissiveAmount" _track_01))))
      (:`then_1`
        (`MaterialInstanceDynamic.SetScalarParameterValue` _dynamicmat "EmissiveAmount" (`self.DefaultEmissiveAmount`))
        (set `self.DidSwitch` false)))
    (else
      (set `self.DidSwitch` true)
      (`AudioComponent.Play` (`self.MS_EyeDoorFeedback`) 0.0)
      (goto _label :!via `PlayFromStart`))))

(fn `LeverSet`
  (returns (IsPressed :type Boolean))
  (if (`self.isPressed`)
    (bind _output_get (set `self.isPressed` false))
    (return _output_get)
    (else
      (bind _output_get_2 (set `self.isPressed` true))
      (return _output_get_2))))

(fn `UserConstructionScript`
  (`|ExecutionSequence`
    (:`then_0`
      (bind _returnvalue (`KismetMaterialLibrary.CreateDynamicMaterialInstance` (`DecalComponent.GetDecalMaterial` (`self.Decal`))))
      (bind _output_get (set `self.DynamicMat` _returnvalue))
      (`MaterialInstanceDynamic.SetScalarParameterValue` _output_get "EmissiveAmount" (`self.DefaultEmissiveAmount`))
      (`DecalComponent.SetDecalMaterial` (`self.Decal`) (`self.DynamicMat`)))))