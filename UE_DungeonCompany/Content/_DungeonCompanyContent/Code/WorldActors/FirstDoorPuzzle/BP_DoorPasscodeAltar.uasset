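; Passcode altar for the first door puzzle that, once a crystal is placed, shows the door code as a sequence of glowing orb flashes.
; The server draws four non-repeating values and replicates DoorCode, whose RepNotify starts the flashes through a timeline driving orb materials and a light.
; The code regenerates after a set number of cycles, and CheckPasscode compares attempts against it.
; Opening the door bursts the crystal and marks the altar used.
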(event `self.ReceiveBeginPlay`
  (bind _crystal (`self.Crystal`))
  (`SceneComponent.SetHiddenInGame` _crystal true false)
  (`PrimitiveComponent.SetCollisionEnabled` _crystal "NoCollision")
  (for _array_element (`|MakeArray` (`self.Orb1`) (`self.Orb2`) (`self.Orb3`) (`self.Orb4`))
    (bind _returnvalue (`PrimitiveComponent.CreateDynamicMaterialInstance` _array_element 0 (`PrimitiveComponent.GetMaterial` _array_element 0) "None"))
    (`KismetArrayLibrary.Array_Add` (`self.Materials`) _returnvalue)
    (`MaterialInstanceDynamic.SetScalarParameterValue` _returnvalue "Brightness" 0.0)))

(event `MulticastOnPlaced`
  ;[1 0 0.5656] Multicast OnPlaced
  (`GameplayStatics.SpawnSoundAtLocation` "/Game/_DungeonCompanyContent/Audio/WorldActors/DoorPuzzle/PlaceCrystal.PlaceCrystal" (`SceneComponent.K2_GetComponentLocation` (`self.ItemAltar`)) (struct) 1.0 1.0 0.0 null null)
  (`SceneComponent.SetHiddenInGame` (`self.CrystalLight`) false false)
  (`SceneComponent.SetHiddenInGame` (`self.Crystal`) false false))

(event `self.OnItemPlaced`
  ;[1 0.6108 0.007893] ItemPlaced
  (`self.MulticastOnPlaced`)
  (`self.GenerateNewDoorCode`))

(event `OnDoorCodeGenerated`
  ;[1 1 1] OnDoor code Generated
  (set `self.NumOfCodeFlashes` 0)
  (set `self.CodeFlashIterator` 0)
  (`self.FlashRoomCode`))

(event `GenerateNewDoorCode`
  ;[1 1 1] Generate Door code
  (`/Engine/EditorBlueprintResources/ActorMacros.Switch Has Authority`
    (:`Authority`
      (`KismetSystemLibrary.PrintString` "New Door code is beeing generated")
      (bind _code (`self.GenerateCode`))
      (set `self.DoorCode` _code) ; multicasts
    )))

(event `FlashRoomCode`
  ;[1 1 1] FlashDoor Code
  (if (not (`self.Used`))
    (bind (_direction _0_1_0) (`Timeline|RuneFlash` :!via `PlayFromStart`)
      (:`Update`
        (`MaterialInstanceDynamic.SetScalarParameterValue` (`|GetArrayItem` (`self.Materials`) (- (`|GetArrayItem` (`self.DoorCode`) (`self.CodeFlashIterator`)) 1)) "Brightness" (* _0_1_0 30.0))
        (`LightComponent.SetIntensity` (`self.Headight`) (* _0_1_0 60.0)))
      (:`Finished`
        (`/Engine/EditorBlueprintResources/StandardMacros.IncrementInt` (`self.CodeFlashIterator`)
          (:`  `
            (if (`self.ContinueFlashing`)
              (if (not (>= (`self.CodeFlashIterator`) (`KismetArrayLibrary.Array_Length` (`self.DoorCode`))))
                (`self.FlashRoomCode`)
                (else
                  (`self.CodeCycleCompleted`))))))))))

(event `CodeCycleCompleted`
  ;[1 1 1] FlashDoor Code
  (`/Engine/EditorBlueprintResources/StandardMacros.IncrementInt` (`self.NumOfCodeFlashes`)
    (:`  `
      (`KismetSystemLibrary.Delay` 2.0)
      (if (>= (`self.NumOfCodeFlashes`) (`self.NumOfCodeFlashesBeforeChange`))
        (`self.GenerateNewDoorCode`)
        (else
          (set `self.CodeFlashIterator` 0)
          (`self.FlashRoomCode`))))))

(event `OnDoorOpened`
  (bind _crystal (`self.Crystal`))
  ;[1 1 1] On Door opened
  (`SceneComponent.SetHiddenInGame` _crystal true false)
  (`PrimitiveComponent.SetCollisionEnabled` _crystal "NoCollision")
  (set `self.Used` true)
  (`GameplayStatics.PlaySoundAtLocation` "/Game/_DungeonCompanyContent/Audio/WorldActors/DoorPuzzle/CrystalBurst.CrystalBurst" (`SceneComponent.K2_GetComponentLocation` (`self.Crystal`)) (struct) 1.0 1.0 0.0 null null null null)
  (`SceneComponent.SetHiddenInGame` (`self.CrystalLight`) true false))

(event `/Game/_DungeonCompanyContent/Code/WorldActors/DungeonReset/BP_Resettable.LocalReset`
  (bind _crystal (`self.Crystal`))
  ;[1 1 1] Reset
  (`SceneComponent.SetHiddenInGame` _crystal true false)
  (`PrimitiveComponent.SetCollisionEnabled` _crystal "NoCollision")
  (set `self.ContinueFlashing` false)
  (`SceneComponent.SetHiddenInGame` (`self.CrystalLight`) true false))

(fn `CheckPasscode`
  (params (Code :type "Array of Integer (by ref)"))
  (returns (Correct :type Boolean))
  (return (`KismetArrayLibrary.Array_Identical` Code (`self.DoorCode`))))

(fn `GenerateCode`
  (returns (Code :type "Array of Integer"))
  (locals (Bag :type "Array of Integer") (Random :type Integer) (CodeToReturn :type "Array of Integer"))
  (`|ExecutionSequence`
    (:`then_0`
      (for _ (range 4)
        (set `local.Random` (`KismetMathLibrary.RandomIntegerInRange` 0 (- (`KismetArrayLibrary.Array_Length` (`local.Bag`)) 1)))
        (`KismetArrayLibrary.Array_Add` (`local.CodeToReturn`) (`|GetArrayItem` (`local.Bag`) (`local.Random`)))
        (`KismetArrayLibrary.Array_Remove` (`local.Bag`) (`local.Random`))))
    (:`then_1`
      (return (`local.CodeToReturn`)))))

(fn `OnRep_DoorCode`
  (`self.OnDoorCodeGenerated`))

(fn `UserConstructionScript`)