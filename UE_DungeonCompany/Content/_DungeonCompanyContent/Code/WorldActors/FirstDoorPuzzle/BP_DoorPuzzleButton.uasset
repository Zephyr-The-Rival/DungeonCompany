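; Numbered button for the first door puzzle that lights up when pressed.
; The construction script picks one of four dynamic materials from ButtonNumber.
; A press while off sets On and calls ButtonTurnedOn with its number; the button never turns itself off.
; OnRep_On drives the Glow timeline forward or in reverse, animating material brightness and point light intensity.
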(event `self.ReceiveBeginPlay`
  (`parent.ReceiveBeginPlay`)
  (add `BasicButton.OnButtonPressed` (delegate `OnPressed`)))

(event `OnPressed`
  (params (InteractingPawn :type "Pawn Object Reference"))
  (if (not (`self.On`))
    (set `self.On` true)
    (`self.ButtonTurnedOn` (`self.ButtonNumber`))))

(event `TurnOn/Off`
  (params (On :type Boolean))
  (if On
    (bind (_direction _0_to_1) (`Timeline|Glow` :!via `PlayFromStart` :!label _label)
      (:`Update`
        (`MaterialInstanceDynamic.SetScalarParameterValue` (`self.ButtonMaterial`) "Brightness" (* _0_to_1 10.0))
        (`LightComponent.SetIntensity` (`self.PointLight`) (* _0_to_1 30.0))))
    (else
      (goto _label :!via `ReverseFromEnd`))))

(fn `OnRep_On`
  (`self.TurnOn/Off` (`self.On`)))

(fn `UserConstructionScript`
  (`parent.UserConstructionScript`)
  (switch `int` (`self.ButtonNumber`)
    (:`1`
      (bind _returnvalue (`PrimitiveComponent.CreateDynamicMaterialInstance` (`self.StaticMesh`) 0 "/Game/_DungeonCompanyContent/Assets/0_Placeholder/Materials/DoorButtons/MI_DoorButton_1.MI_DoorButton_1" "None"))
      (set `self.ButtonMaterial` _returnvalue))
    (:`2`
      (bind _returnvalue_2 (`PrimitiveComponent.CreateDynamicMaterialInstance` (`self.StaticMesh`) 0 "/Game/_DungeonCompanyContent/Assets/0_Placeholder/Materials/DoorButtons/MI_DoorButton_2.MI_DoorButton_2" "None"))
      (set `self.ButtonMaterial` _returnvalue_2))
    (:`3`
      (bind _returnvalue_3 (`PrimitiveComponent.CreateDynamicMaterialInstance` (`self.StaticMesh`) 0 "/Game/_DungeonCompanyContent/Assets/0_Placeholder/Materials/DoorButtons/MI_DoorButton_3.MI_DoorButton_3" "None"))
      (set `self.ButtonMaterial` _returnvalue_3))
    (:`4`
      (bind _returnvalue_4 (`PrimitiveComponent.CreateDynamicMaterialInstance` (`self.StaticMesh`) 0 "/Game/_DungeonCompanyContent/Assets/0_Placeholder/Materials/DoorButtons/MI_DoorButton_4.MI_DoorButton_4" "None"))
      (set `self.ButtonMaterial` _returnvalue_4))))