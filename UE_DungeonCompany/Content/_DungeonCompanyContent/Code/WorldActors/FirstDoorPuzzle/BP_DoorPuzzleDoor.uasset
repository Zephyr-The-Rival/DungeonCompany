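; Puzzle door that opens when players enter the correct four-press code on its directional buttons.
; Four child-actor buttons feed presses into an entered code, which MyAltar validates; a wrong code clears it and switches the buttons off.
; Success notifies the altar, then raises the mesh by timeline with sound and Niagara effects.
; Non-authority instances replay the opening on BeginPlay if already open, and a sound plays whenever the altar generates a new code.
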(event `self.ReceiveBeginPlay`
  (`|ExecutionSequence`
    (:`then_0`
      (bind _output_get (set `self.Buttons` (`|MakeArray` (`self.BP_DoorPuzzleButton_Up`) (`self.BP_DoorPuzzleButton_Right`) (`self.BP_DoorPuzzleButton_Down`) (`self.BP_DoorPuzzleButton_Left`))))
      (for _array_element _output_get
        (bind _asbp_door_puzzle_button (cast `/Game/_DungeonCompanyContent/Code/WorldActors/FirstDoorPuzzle/BP_DoorPuzzleButton` (`ChildActorComponent.ChildActor` _array_element)))
        (add `/Game/_DungeonCompanyContent/Code/WorldActors/FirstDoorPuzzle/BP_DoorPuzzleButton.ButtonTurnedOn` _asbp_door_puzzle_button (`|CreateDelegate` :!event `Button Pressed`))))
    (:`then_1`
      ;[1 1 1] for loading
      (if (and (`self.IsOpen`) (not (`self.HasAuthority`)))
        (`self.DoorOpen`) ; will only execute locally
      ))
    (:`then_2`
      (add `/Game/_DungeonCompanyContent/Code/WorldActors/FirstDoorPuzzle/BP_DoorPasscodeAltar.OnGeneratingNewDoorCode` (`self.MyAltar`) (delegate `DoorCodeChangeSound`)))))

(event `Button Pressed`
  (params (buttonNumber :type Integer))
  (`KismetArrayLibrary.Array_Add` (`self.EnterdCode`) buttonNumber)
  (if (== (`KismetArrayLibrary.Array_Length` (`self.EnterdCode`)) 4)
    (bind _correct (`/Game/_DungeonCompanyContent/Code/WorldActors/FirstDoorPuzzle/BP_DoorPasscodeAltar.CheckPasscode` (`self.MyAltar`) (`self.EnterdCode`)))
    (if _correct
      (`KismetSystemLibrary.Delay` 1.0)
      (`self.DoorOpen`)
      (else
        (`KismetSystemLibrary.Delay` 1.0)
        (`KismetArrayLibrary.Array_Clear` (`self.EnterdCode`))
        (for _array_element (`self.Buttons`)
          (bind _asbp_door_puzzle_button (cast `/Game/_DungeonCompanyContent/Code/WorldActors/FirstDoorPuzzle/BP_DoorPuzzleButton` (`ChildActorComponent.ChildActor` _array_element)))
          (set `/Game/_DungeonCompanyContent/Code/WorldActors/FirstDoorPuzzle/BP_DoorPuzzleButton.On` false _asbp_door_puzzle_button))))))

(event `DoorCodeChangeSound`
  (`GameplayStatics.PlaySoundAtLocation` "/Game/_DungeonCompanyContent/Audio/WorldActors/Door/DoorCodeChangedCue.DoorCodeChangedCue" (`SceneComponent.K2_GetComponentLocation` (`self.StaticMesh`)) (struct) 1.0 1.0 0.0 null null null null))

(event `DoorOpen`
  (bind _niagara (`self.Niagara`))
  (`|ExecutionSequence`
    (:`then_0`
      (`/Game/_DungeonCompanyContent/Code/WorldActors/FirstDoorPuzzle/BP_DoorPasscodeAltar.OnDoorOpened` (`self.MyAltar`))
      (set `self.IsOpen` true))
    (:`then_1`
      (`KismetSystemLibrary.Delay` 2.0)
      (`|ExecutionSequence`
        (:`then_0`
          (bind (_direction _height) (`Timeline|DoorOpening` :!via `PlayFromStart`)
            (:`Update`
              (`SceneComponent.K2_SetRelativeLocation` (`self.StaticMesh`) (`KismetMathLibrary.MakeVector` 0.0 0.0 _height) false false))))
        (:`then_1`
          ;[1 1 1] VFX and SFX
          (`KismetSystemLibrary.Delay` 0.5)
          (`GameplayStatics.PlaySoundAtLocation` "/Game/_DungeonCompanyContent/Audio/WorldActors/Door/dooropen_Cue.dooropen_Cue" (`SceneComponent.K2_GetComponentLocation` (`self.StaticMesh`)) (struct) 1.0 1.0 0.0 null null null null))
        (:`then_2`
          (`ActorComponent.SetAutoActivate` _niagara true)
          (`GameplayStatics.PlaySoundAtLocation` "/Game/_DungeonCompanyContent/Audio/Environment/rock/rocks_Cue.rocks_Cue" (`SceneComponent.K2_GetComponentLocation` (`self.StaticMesh`)) (struct) 1.0 1.0 0.0 null null null null)
          (`ActorComponent.SetActive` _niagara true false)
          (`KismetSystemLibrary.Delay` 4.0)
          (`ActorComponent.SetActive` _niagara false false))))))

(event `/Game/_DungeonCompanyContent/Code/WorldActors/DungeonReset/BP_Resettable.LocalReset`
  (bind _output_get (set `self.Buttons` (`|MakeArray` (`self.BP_DoorPuzzleButton_Up`) (`self.BP_DoorPuzzleButton_Right`) (`self.BP_DoorPuzzleButton_Down`) (`self.BP_DoorPuzzleButton_Left`))))
  (for _array_element _output_get
    (bind _asbp_door_puzzle_button (cast `/Game/_DungeonCompanyContent/Code/WorldActors/FirstDoorPuzzle/BP_DoorPuzzleButton` (`ChildActorComponent.ChildActor` _array_element)))
    (set `/Game/_DungeonCompanyContent/Code/WorldActors/FirstDoorPuzzle/BP_DoorPuzzleButton.On` false _asbp_door_puzzle_button)))

(fn `UserConstructionScript`)