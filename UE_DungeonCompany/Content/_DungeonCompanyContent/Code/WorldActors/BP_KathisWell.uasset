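; BP_KathisWell is a world actor whose point light and Niagara effect are toggled by a button.
; On BeginPlay it binds a custom event to the referenced MyButton's press event, printing a warning if none is set in the Outliner.
; Each press flips the light's visibility and resets the effect's active state to match, then prints the pressing player character's name.
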(event `self.ReceiveBeginPlay`
  (bind _mybutton (`self.MyButton`))
  (`/Engine/EditorBlueprintResources/StandardMacros.IsValid` _mybutton
    (:`Is Valid`
      (add `BasicButton.OnButtonPressed` _mybutton (delegate `CustomEvent`)))
    (:`Is Not Valid`
      (`KismetSystemLibrary.PrintString` "My button was not valid \nBind in Outliner"))))

(event `CustomEvent`
  (params (InteractingPawn :type "Pawn Object Reference"))
  (bind _pointlight (`self.PointLight`))
  (bind _returnvalue (not (`SceneComponent.bVisible` _pointlight)))
  (`|ExecutionSequence`
    (:`then_0`
      (`ActorComponent.SetActive` (`self.Niagara`) _returnvalue true)
      (`SceneComponent.SetVisibility` _pointlight _returnvalue false))
    (:`then_1`
      (bind _asbp_player_character (cast `/Game/_DungeonCompanyContent/Code/PlayerCharacter/BP_PlayerCharacter` InteractingPawn))
      (`KismetSystemLibrary.PrintString` (`KismetStringLibrary.Concat_StrStr` (`KismetSystemLibrary.GetObjectName` _asbp_player_character) " pressed my button")))))

(fn `UserConstructionScript`)