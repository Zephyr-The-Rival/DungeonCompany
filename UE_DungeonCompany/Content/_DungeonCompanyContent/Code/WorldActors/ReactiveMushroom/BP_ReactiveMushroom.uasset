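; BP_ReactiveMushroom is a world prop that glows when a player character walks into its collision sphere.
; The construction script scales the mesh and sphere from variables, creates a dynamic material at a default emissive level and turns the point light off.
; Player overlap plays two timelines from the start, driving emissive brightness and light intensity.
; A delayed re-trigger for a moving, still-overlapping player is present but disconnected, leaving its tracked overlap state and location unused.
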(event `self.ReceiveBeginPlay`
  (bind _collision (`self.Collision`))
  (`|ExecutionSequence`
    (:`then_0`
      (add `PrimitiveComponent.OnComponentBeginOverlap` _collision (delegate `MushroomHit`)))
    (:`then_1`
      (add `PrimitiveComponent.OnComponentEndOverlap` _collision (delegate `EndOverlap`)))))

(event `MushroomFeedback`
  (`|ExecutionSequence`
    (:`then_0`
      (bind (_direction _emissiveamount) (`Timeline|Timeline` :!via `PlayFromStart`)
        (:`Update`
          (`MaterialInstanceDynamic.SetScalarParameterValue` (`self.DynamicMat`) "Emissive brightness" _emissiveamount))))
    (:`then_1`
      (bind (_direction_2 _emissiveamount_2) (`Timeline|Timeline_0` :!via `PlayFromStart`)
        (:`Update`
          (`LightComponent.SetIntensity` (`self.PointLight`) _emissiveamount_2))))))

(event `MushroomHit`
  (params (OverlappedComponent :type "PrimitiveComponent Object Reference") (OtherActor :type "Actor Object Reference") (OtherComp :type "PrimitiveComponent Object Reference") (OtherBodyIndex :type Integer) (bFromSweep :type Boolean) (SweepResult :type "HitResult Structure (by ref)"))
  (bind _asplayer_character (cast `PlayerCharacter` OtherActor))
  (`|ExecutionSequence`
    (:`then_0`
      (set `self.PlayerOverlapping` true)
      (`self.MushroomFeedback`))
    (:`then_1`
      (set `self.OldLocation` (`self.K2_GetActorLocation` _asplayer_character)))))

(event `EndOverlap`
  (params (OverlappedComponent :type "PrimitiveComponent Object Reference") (OtherActor :type "Actor Object Reference") (OtherComp :type "PrimitiveComponent Object Reference") (OtherBodyIndex :type Integer))
  (cast `PlayerCharacter` OtherActor)
  (set `self.PlayerOverlapping` false))

(event `self.ReceiveTick`
  (params (DeltaSeconds :type "Float (single-precision)")))

(fn `UserConstructionScript`
  (bind _staticmesh (`self.StaticMesh`))
  (bind _mushroomscale (`self.MushroomScale`))
  (bind _collisionspherescale (`self.CollisionSphereScale`))
  (`|ExecutionSequence`
    (:`then_0`
      (`SceneComponent.SetWorldScale3D` (`self.StaticMesh`) (`KismetMathLibrary.MakeVector` _mushroomscale _mushroomscale _mushroomscale)))
    (:`then_1`
      (`SceneComponent.SetWorldScale3D` (`self.Collision`) (`KismetMathLibrary.MakeVector` _collisionspherescale _collisionspherescale _collisionspherescale)))
    (:`then_2`
      (bind _returnvalue (`PrimitiveComponent.CreateDynamicMaterialInstance` _staticmesh 0 (`PrimitiveComponent.GetMaterial` _staticmesh 0) "None"))
      (bind _output_get (set `self.DynamicMat` _returnvalue))
      (`MaterialInstanceDynamic.SetScalarParameterValue` _output_get "Emissive brightness" (`self.DefaultEmissiveAmount`)))
    (:`then_3`
      (`LightComponent.SetIntensity` (`self.PointLight`) 0.0))))