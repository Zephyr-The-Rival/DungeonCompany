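; Placeable item spawner that spawns an actor of the configured item class at its own transform.
; The construction script shows the item as a child actor preview, or a warning text if no class is set, and BeginPlay destroys the preview.
; SpawnMyItem runs only with authority, flags the item as coming from a spawner and binds its pickup event.
; Once an item is picked up, further spawns are blocked.
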(event `self.ReceiveBeginPlay`
  (`ActorComponent.K2_DestroyComponent` (`self.PreviewItem`)))

(event `SpawnMyItem`
  (`/Engine/EditorBlueprintResources/ActorMacros.Switch Has Authority`
    (:`Authority`
      (if (not (`self.ItemPickedUp`))
        (bind _returnvalue (`|SpawnActorFromClass` (`self.ItemClass`) (`SceneComponent.K2_GetComponentToWorld` (`self.DefaultSceneRoot`)) "Undefined" "MultiplyWithRoot" null null))
        (add `WorldItem.OnPickedUp` _returnvalue (delegate `OnItemPickedUp`))
        (set `WorldItem.bCameFromItemSpawner` true _returnvalue)))))

(event `OnItemPickedUp`
  (set `self.ItemPickedUp` true))

(fn `UserConstructionScript`
  (`ActorComponent.K2_DestroyComponent` (`self.PreviewItem`))
  (if (`KismetSystemLibrary.IsValidClass` (`self.ItemClass`))
    (bind _returnvalue (`AddComponent|NODE_AddChildActorComponent-0`))
    (bind _output_get (set `self.PreviewItem` _returnvalue))
    (`ChildActorComponent.SetChildActorClass` _output_get (`self.ItemClass`))
    (else
      (`TextRenderComponent.K2_SetText` (`self.text`) "Fill out class"))))