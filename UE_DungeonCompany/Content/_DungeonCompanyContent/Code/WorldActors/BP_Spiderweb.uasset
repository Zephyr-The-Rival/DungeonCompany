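; BP_Spiderweb is a world actor that shows a spiderweb on a plane mesh, with a selectable visual variant.
; The construction script switches on Version to set the plane's material to the base web or a corner, ceiling or horizontal instance.
; Versions 1 and 2 both use the same corner material, MI_SpiderwebCorner2.
; The event graph has no active logic.
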(fn `UserConstructionScript`
  (switch `int` (`self.Version`)
    (:`0`
      (`PrimitiveComponent.SetMaterial` (`self.Plane`) 0 "/Game/_DungeonCompanyContent/Assets/0_Placeholder/Spierwebs/M_Spiderweb.M_Spiderweb"))
    (:`1`
      (`PrimitiveComponent.SetMaterial` (`self.Plane`) 0 "/Game/_DungeonCompanyContent/Assets/0_Placeholder/Spierwebs/MI_SpiderwebCorner2.MI_SpiderwebCorner2"))
    (:`2`
      (`PrimitiveComponent.SetMaterial` (`self.Plane`) 0 "/Game/_DungeonCompanyContent/Assets/0_Placeholder/Spierwebs/MI_SpiderwebCorner2.MI_SpiderwebCorner2"))
    (:`3`
      (`PrimitiveComponent.SetMaterial` (`self.Plane`) 0 "/Game/_DungeonCompanyContent/Assets/0_Placeholder/Spierwebs/MI_SpiderwebCeling.MI_SpiderwebCeling"))
    (:`4`
      (`PrimitiveComponent.SetMaterial` (`self.Plane`) 0 "/Game/_DungeonCompanyContent/Assets/0_Placeholder/Spierwebs/MI_SpiderwebHorizontal.MI_SpiderwebHorizontal"))))