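; Audio-reactive actor in the AudioReactivePlant folder that makes a mesh's emissive respond to the loudness of its own sound.
; BeginPlay puts a dynamic MI_PlantReactor material on the Cube and starts the PickUpCoin01 audio component after a short delay.
; Playback percent callbacks read the sound's cooked envelope data and write it straight to the material's Emissive parameter, with no Tick.
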(event `self.ReceiveBeginPlay`
  (add `AudioComponent.OnAudioPlaybackPercent` (`self.PickUpCoin_01`) (delegate `NoiseMade`))
  (bind _returnvalue (`KismetMaterialLibrary.CreateDynamicMaterialInstance` "/Game/_DungeonCompanyContent/Code/AudioReactivePlant/MI_PlantReactor.MI_PlantReactor"))
  (set `self.DynamicMat` _returnvalue)
  (`PrimitiveComponent.SetMaterial` (`self.Cube`) 0 (`self.DynamicMat`))
  (`KismetSystemLibrary.Delay` 1.0)
  (`AudioComponent.Play` (`self.PickUpCoin_01`) 0.0))

(event `NoiseMade`
  (params (PlayingSoundWave :type "SoundWave Object Reference") (PlaybackPercent :type "Float (single-precision)"))
  (bind _outenvelopedata (`AudioComponent.GetCookedEnvelopeData` (`self.PickUpCoin_01`)))
  (`MaterialInstanceDynamic.SetScalarParameterValue` (`self.DynamicMat`) "Emissive" _outenvelopedata))

(fn `UserConstructionScript`)