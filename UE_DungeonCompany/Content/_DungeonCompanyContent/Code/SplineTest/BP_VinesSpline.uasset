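; BP_VinesSpline is a construction-script spline actor that builds vines from deforming spline mesh segments along its spline.
; It derives segment length from Mesh1's X bounds, then adds collision-enabled segments along the spline, using Mesh2 for the first and Mesh1 for the rest.
; Each segment gets random start and end roll for variation, with tangents clamped to the segment length.
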(fn `UserConstructionScript`
  (bind _returnvalue (`KismetMathLibrary.RandomFloatInRange` 0.0 360.0))
  (bind _spline (`self.Spline`))
  (bind _spline_2 (`self.Spline`))
  (bind _xlength (`self.XLength`))
  (bind (_returnvalue_min _returnvalue_max) (break `Box` (`StaticMesh.GetBoundingBox` (`self.Mesh1`))))
  (bind _returnvalue_x (`KismetMathLibrary.BreakVector` (+ (`KismetMathLibrary.Vector_GetAbs` _returnvalue_min) (`KismetMathLibrary.Vector_GetAbs` _returnvalue_max))))
  (bind _output_get (set `self.XLength` _returnvalue_x))
  (for _index (range (+ (`KismetMathLibrary.FTrunc` (/ (`SplineComponent.GetSplineLength` (`self.Spline`)) _output_get)) 1))
    (bind _returnvalue_2 (`AddComponent|NODE_AddSplineMeshComponent-0`))
    (`PrimitiveComponent.SetCollisionEnabled` _returnvalue_2 "QueryAndPhysics")
    (`SplineMeshComponent.SetForwardAxis` _returnvalue_2 "X" true)
    ;[1 1 1] First Spline Component is Mesh 2
    (if (== _index 0)
      (`StaticMeshComponent.SetStaticMesh` _returnvalue_2 (`self.Mesh2`))
      (else
        (`StaticMeshComponent.SetStaticMesh` _returnvalue_2 (`self.Mesh1`))))
    ;[1 1 1] Random Rotation
    (`SplineMeshComponent.SetStartRollDegrees` _returnvalue_2 _returnvalue true)
    (`SplineMeshComponent.SetEndRollDegrees` _returnvalue_2 _returnvalue true)
    (bind _returnvalue_3 (* _index (`self.XLength`)))
    (bind _returnvalue_4 (* (+ _index 1) (`self.XLength`)))
    (`SplineMeshComponent.SetStartAndEnd` _returnvalue_2 (`SplineComponent.GetLocationAtDistanceAlongSpline` _spline_2 _returnvalue_3 "Local") (`KismetMathLibrary.ClampVectorSize` (`SplineComponent.GetTangentAtDistanceAlongSpline` _spline_2 _returnvalue_3 "Local") 0.0 _xlength) (`SplineComponent.GetLocationAtDistanceAlongSpline` _spline _returnvalue_4 "Local") (`KismetMathLibrary.ClampVectorSize` (`SplineComponent.GetTangentAtDistanceAlongSpline` _spline _returnvalue_4 "Local") 0.0 _xlength) true)))