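; Player character Blueprint that adds local-only feedback and item hooks on top of its parent class.
; On begin play it sets view light and mesh shadow by local control and gives the local player starter items.
; Events drive a repeating blur yawn, damage, left-behind and sending-stone widgets, delayed death when left behind, and potion and climbing-hook endings.
; Tick refreshes held items through a one-second Delay; coal decal spawning is marked unused.
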(event `self.ReceiveBeginPlay`
  (bind _returnvalue (`self.IsLocallyControlled`))
  (`parent.ReceiveBeginPlay`)
  (`KismetSystemLibrary.DelayUntilNextTick`)
  (`|ExecutionSequence`
    (:`then_0`
      (`SceneComponent.SetVisibility` (`self.ViewLight`) _returnvalue false)
      (`PrimitiveComponent.SetCastShadow` (`self.Mesh`) (not _returnvalue)))
    (:`then_1`
      (if _returnvalue
        (for _array_element (`self.StarterItems`)
          (bind _returnvalue_2 (`|GenericCreateObject` (`|ConvertAsset` _array_element)))
          (`self.AddItemToInventory` _returnvalue_2))))))

(event `self.BP_Yawn`
  ;[1 1 1] Yawn
  (set `self.KeepYawning` true)
  (if (`self.IsLocallyControlled`)
    (`GameplayStatics.PlaySound2D` (`self.YawnSound`) 1.0 1.0 0.0 null null)
    (bind _returnvalue (`|CreateWidget` "/Game/_DungeonCompanyContent/Assets/VFX/PostProcessing/Blurr.Blurr_C"))
    (`UserWidget.AddToViewport` _returnvalue 0)
    (bind (_direction _010) (`Timeline|Yawn 4s` :!via `PlayFromStart`)
      (:`Update`
        (`BackgroundBlur.SetBlurStrength` (`/Game/_DungeonCompanyContent/Assets/VFX/PostProcessing/Blurr.BackgroundBlur_228` _returnvalue) (* _010 20.0)))
      (:`Finished`
        (`Widget.RemoveFromParent` _returnvalue)
        (if (`self.KeepYawning`)
          (`KismetSystemLibrary.Delay` (`KismetMathLibrary.RandomFloatInRange` 10.0 60.0))
          (if (`self.KeepYawning`)
            (`self.BP_Yawn`)))))))

(event `self.ShowHudDamageIndicator`
  ;[1 1 1] Hud damage indicator
  (`self.OnClientShowHudDamage`))

(event `OnClientShowHudDamage`
  ;[1 1 1] Hud damage indicator
  (if (`self.IsLocallyControlled`)
    (bind _returnvalue (`|CreateWidget` "/Game/_DungeonCompanyContent/Code/UI/PlayerHud/BP_DamageInicator.BP_DamageInicator_C"))
    (`UserWidget.AddToViewport` _returnvalue 0)))

(event `self.BP_StopYawn`
  ;[1 1 1] Yawn
  (set `self.KeepYawning` false))

(event `self.LeftBehind`
  ;[1 1 1] Left behind
  (`self.LocalLeftBehind`)
  (`KismetSystemLibrary.Delay` 3.0)
  (`self.DamageEntity` 100000.0))

(event `LocalLeftBehind`
  ;[1 1 1] Left behind
  (bind _returnvalue (`|CreateWidget` "/Game/_DungeonCompanyContent/Code/UI/LeftBehind.LeftBehind_C"))
  (`UserWidget.AddToViewport` _returnvalue 0)
  (`KismetSystemLibrary.Delay` 3.0)
  (`Widget.RemoveFromParent` _returnvalue))

(event `CoalSpawnDecal`
  (bind _firstpersoncamera (`self.FirstPersonCamera`))
  (bind _returnvalue (`SceneComponent.K2_GetComponentLocation` _firstpersoncamera))
  ;[1 1 1] Coal decal not in use
  (bind (_outhit _returnvalue_2) (`KismetSystemLibrary.LineTraceSingle` _returnvalue (+ _returnvalue (* (`SceneComponent.GetForwardVector` _firstpersoncamera) (300.0 300.0 300.0))) "TraceTypeQuery4"))
  (if _returnvalue_2
    (bind (_bblockinghit _binitialoverlap _time _distance _location _impactpoint _normal) (`GameplayStatics.BreakHitResult` _outhit))
    (`self.Server_SpawnDecal` _location (`KismetMathLibrary.MakeRotFromX` _normal))))

(event `self.ReceiveTick`
  (params (DeltaSeconds :type "Float (single-precision)"))
  ;[1 1 1] updated held items for on death
  (if (`self.IsLocallyControlled`)
    (`KismetSystemLibrary.Delay` 1.0)
    (`self.UpdateHeldItems`)))

(event `Server_SpawnDecal`
  (params (Location :type "Vector Structure") (Rotation :type "Rotator Structure"))
  ;[1 1 1] Coal decal not in use
  (`self.Multicast_SpawnCoalDecal` Location Rotation))

(event `EndDrinkingPotion`
  ;[1 1 1] Stop drinking potion
  (`KismetSystemLibrary.DelayUntilNextTick`)
  (`self.StopDrinkingPotion`))

(event `Multicast_SpawnCoalDecal`
  (params (Location :type "Vector Structure") (Rotation :type "Rotator Structure"))
  ;[1 1 1] Coal decal not in use
  (`GameplayStatics.SpawnDecalAtLocation` "/Game/_DungeonCompanyContent/Assets/0_Placeholder/M_CoalDecal.M_CoalDecal" (5.0 5.0 5.0) Location Rotation))

(event `StopThrowHook`
  ;[1 1 1] Stop throwing hook
  (`KismetSystemLibrary.DelayUntilNextTick`)
  (bind _asbp_climbing_hook_world (cast `/Game/_DungeonCompanyContent/Code/Items/ClimbingHook/BP_ClimbingHook_World` (`self.GetCurrentlyHeldWorldItem`)))
  (`Hook.OnHookThrown` _asbp_climbing_hook_world self))

(event `FlashSendingStoneNotification`
  (params (Signal :type "ESendingStoneAnimatoinState Enum" :default "Neutral"))
  (`GameplayStatics.PlaySound2D` "/Game/_DungeonCompanyContent/Audio/SendingStoneSounds/CrystalLightUpSound.CrystalLightUpSound" 1.0 1.0 0.0 null null)
  (bind _returnvalue (`|CreateWidget` "/Game/_DungeonCompanyContent/Code/Items/SendingStone/BP_SendingStoneNotification.BP_SendingStoneNotification_C" null Signal))
  (`UserWidget.AddToViewport` _returnvalue 0))

(fn `UserConstructionScript`)